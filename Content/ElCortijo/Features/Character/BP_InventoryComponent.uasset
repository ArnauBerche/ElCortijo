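; Single-slot inventory component that lets a character hold one pickable item actor and drop it again.
; PickUpActor saves scale, disables physics and interaction, and moves the real actor into a preview room using its ItemData pose, isolated in a SceneCapture show-only list.
; DropActor places it ahead of the given camera transform, restoring scale, physics and interaction.
; EmptyInventoryRef only clears the reference; ClearItem is an empty stub.
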(fn `ClearItem`)

(fn `DropActor`
  (params (CameraTransform :type "Transform Structure"))
  (returns (Dropped :type Boolean))
  (locals (TempRef :type "/Game/ElCortijo/Features/Interaction/Pickable/BP_Pickable Object Reference"))
  (bind _rotation (.rotation CameraTransform))
  (bind _tempref (`local.TempRef`))
  (bind _empty (`self.IsEmpty`))
  (if _empty
    (return false)
    (else
      (set `local.TempRef` (`self.CurrentItemActor`))
      (set `self.CurrentItemActor` null)
      (`Actor.K2_DetachFromActor` _tempref "KeepWorld" "KeepWorld" "KeepWorld")
      (`Actor.K2_SetActorTransform` _tempref (`KismetMathLibrary.MakeTransform` (+ (.location CameraTransform) (* (`KismetMathLibrary.GetForwardVector` _rotation) (`self.DropOffset`))) _rotation (`self.SavedScale`)) false true)
      (`/Game/ElCortijo/Features/Interaction/Pickable/BP_Pickable.SetPhysics` _tempref true)
      (`/Game/ElCortijo/Features/Interaction/Pickable/BP_Pickable.SetInteractable` _tempref true)
      (`SceneCaptureComponent.ClearShowOnlyComponents` (`/Game/ElCortijo/Features/Interaction/Pickable/BP_ItemPreviewRoom.SceneCapture` (`self.PreviewRoomRef`)))
      (return true))))

(fn `EmptyInventoryRef`
  (set `self.CurrentItemActor` null))

(fn `IsEmpty`
  (returns (Empty :type Boolean))
  (return (not (`KismetSystemLibrary.IsValid` (`self.CurrentItemActor`)))))

(fn `PickUpActor`
  (params (Pickable :type "/Game/ElCortijo/Features/Interaction/Pickable/BP_Pickable Object Reference"))
  (returns (Picked :type Boolean))
  (bind _currentitemactor (`self.CurrentItemActor`))
  (bind _currentitemactor_2 (`self.CurrentItemActor`))
  (bind _scenecapture (`/Game/ElCortijo/Features/Interaction/Pickable/BP_ItemPreviewRoom.SceneCapture` (`self.PreviewRoomRef`)))
  (bind (_previewrotator _scale) (break `/Game/ElCortijo/Features/Interaction/Pickable/S_ItemData` (`/Game/ElCortijo/Features/Interaction/Pickable/BP_Pickable.ItemData` _currentitemactor_2)))
  (bind _empty (`self.IsEmpty`))
  (if _empty
    (set `self.CurrentItemActor` Pickable)
    (set `self.SavedScale` (`Actor.GetActorScale3D` Pickable))
    (set `self.SavedRotator` (`Actor.K2_GetActorRotation` Pickable))
    (`/Game/ElCortijo/Features/Interaction/Pickable/BP_Pickable.SetPhysics` _currentitemactor false)
    (`/Game/ElCortijo/Features/Interaction/Pickable/BP_Pickable.SetInteractable` _currentitemactor false)
    (`Actor.K2_AttachToComponent` _currentitemactor (`/Game/ElCortijo/Features/Interaction/Pickable/BP_ItemPreviewRoom.Parent` (`self.PreviewRoomRef`)) "None" "SnapToTarget" "SnapToTarget" "KeepWorld" false)
    (`Actor.K2_SetActorRelativeLocation` _currentitemactor_2 (0.0 0.0 0.0) false true)
    (`Actor.K2_SetActorRelativeRotation` _currentitemactor_2 _previewrotator false false)
    (`Actor.SetActorRelativeScale3D` _currentitemactor_2 _scale)
    (`SceneCaptureComponent.ClearShowOnlyComponents` _scenecapture)
    (`SceneCaptureComponent.ShowOnlyComponent` _scenecapture (`/Game/ElCortijo/Features/Interaction/Pickable/BP_Pickable.Object` (`self.CurrentItemActor`)))
    (return true)
    (else
      (`KismetSystemLibrary.PrintText` "Ocupado")
      (return false))))