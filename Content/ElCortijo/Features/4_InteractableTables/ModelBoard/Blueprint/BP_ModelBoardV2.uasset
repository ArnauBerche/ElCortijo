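; Interactable table holding a scale model whose rooms the player inspects for evidence, with notes shown in a WBP_ModelBoard widget.
; A cursor trace highlights Room-tagged parts with an overlay material; left click animates one to a focus point, where it can be yawed, and right click returns it.
; Evidence actors snap to spots found by Evidence_ID component tags, becoming clickable only while their room is focused.
; Entering and exiting the table toggles the widget and table input mapping.
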(event `self.ReceiveBeginPlay`
  (`|ExecutionSequence`
    (:`then_0`
      (set `self.TType` "NewEnumerator1"))
    (:`then_1`
      (bind _asbp_first_person_character (cast `/Game/ElCortijo/Features/1_MainCharacter/Blueprints/BP_FirstPersonCharacter` (`GameplayStatics.GetPlayerCharacter` 0)))
      (`|ExecutionSequence`
        (:`then_0`
          (add `/Game/ElCortijo/Features/1_MainCharacter/Blueprints/BP_FirstPersonCharacter.OnLeftClickPress` _asbp_first_person_character (delegate `OnLeftClickPress_Handler`)))
        (:`then_1`
          (add `/Game/ElCortijo/Features/1_MainCharacter/Blueprints/BP_FirstPersonCharacter.OnLeftClickRelease` _asbp_first_person_character (delegate `OnLeftClickRelease_Handler`)))
        (:`then_2`
          (add `/Game/ElCortijo/Features/1_MainCharacter/Blueprints/BP_FirstPersonCharacter.OnRightClickPress` _asbp_first_person_character (delegate `OnRightClickPress_Handler`)))
        (:`then_3`
          (add `/Game/ElCortijo/Features/1_MainCharacter/Blueprints/BP_FirstPersonCharacter.OnRightClickRelease` _asbp_first_person_character (delegate `OnRightClickRelease_Handler`)))))
    (:`then_2`
      (bind _returnvalue (`|CreateWidget` "/Game/ElCortijo/Features/4_InteractableTables/ModelBoard/UI/WBP_ModelBoard.WBP_ModelBoard_C" (`self.Controller`) self))
      (set `self.WBP_ModelBoard` _returnvalue))
    (:`then_3`
      (`parent.ReceiveBeginPlay`)
      (`self.GetAllEvidenceSpots`))
    (:`then_4`
      (`KismetSystemLibrary.DelayUntilNextTick`)
      (`self.AddNewOBJEvidence` (`self.BP Evidence`)))))

(event `OnLeftClickPress_Handler`
  (if (`self.PlayerInTable`)
    (if (`self.IsRoomInFocus`)
      (`self.ClickEvidence`)
      (else
        (`self.LeftclickZoomLogic`)))))

(event `OnLeftClickRelease_Handler`)

(event `OnRightClickPress_Handler`
  (if (`self.PlayerInTable`)
    (if (`self.IsRoomInFocus`)
      (set `self.DescriptinObject` null)
      (`self.RightclickZoomLogic`)
      (`/Game/ElCortijo/Features/4_InteractableTables/ModelBoard/UI/WBP_ModelBoard.ForceClose` (`self.WBP_ModelBoard`)))))

(event `OnRightClickRelease_Handler`)

(event `self.ReceiveTick`
  (params (DeltaSeconds :type "Float (single-precision)"))
  (bind (_returnvalue_roll _returnvalue_pitch _returnvalue_yaw) (`KismetMathLibrary.BreakRotator` (`SceneComponent.K2_GetComponentRotation` (`self.FocusPoint`))))
  (`parent.ReceiveTick` DeltaSeconds)
  (if (`self.PlayerInTable`)
    (if (`self.IsRoomInFocus`)
      (if (`self.IsRoomAnimating`)
        (if (`self.NeedsFocus`)
          (bind (_direction _newtrack_0) (`Timeline|Room Animation` :!label _label)
            (:`Update`
              (`SceneComponent.K2_SetWorldTransform` (`self.HoveredRoom`) (`KismetMathLibrary.TLerp` (`self.FocusRoomLastTransform`) (`SceneComponent.K2_GetComponentToWorld` (`self.FocusPoint`)) _newtrack_0 "EulerInterp") false false))
            (:`Finished`
              (set `self.IsRoomAnimating` false)
              (set `self.Value` _returnvalue_yaw)
              (if (not (`self.NeedsFocus`))
                (set `self.IsRoomInFocus` false))))
          (else
            (goto _label :!via `Reverse`))))
      (else
        (`self.RoomHover`)))))

(event `self.EnterTable`
  (bind _wbp_modelboard (`self.WBP_ModelBoard`))
  (`parent.EnterTable`)
  (`UserWidget.AddToViewport` _wbp_modelboard 0)
  (bind _asbp_game_instance (cast `/Game/ElCortijo/Features/0_Unsorted/GameInstance/BP_GameInstance` (`GameplayStatics.GetGameInstance`)))
  (set `self.GI_Ref` _asbp_game_instance)
  (`/Game/ElCortijo/Features/4_InteractableTables/ModelBoard/UI/WBP_ModelBoard.OnNotesUpdated_Handler_L` _wbp_modelboard)
  (`/Game/ElCortijo/Features/4_InteractableTables/ModelBoard/UI/WBP_ModelBoard.OnNotesUpdated_Handler_R` _wbp_modelboard)
  (`EnhancedInputSubsystemInterface.AddMappingContext` (pcsubsystem `EnhancedInputLocalPlayerSubsystem` (`self.Controller`)) "/Game/ElCortijo/Features/1_MainCharacter/Input/IMC_Table.IMC_Table" 100 (struct))
  (add `/Game/ElCortijo/Features/1_MainCharacter/Blueprints/BP_FirstPersonCharacter.OnCameraHPress` (`self.Character`) (delegate `TurnOBJ`)))

(event `TurnOBJ`
  (params (Value :type "Float (double-precision)"))
  (if (and (!= (`self.HoveredRoom`) null) (`self.IsRoomInFocus`))
    (bind _output_get (set `self.Value` (+ (* (* (`self.HorizontalSpeed`) Value) (`GameplayStatics.GetWorldDeltaSeconds`)) (`self.Value`))))
    (`SceneComponent.K2_SetWorldRotation` (`self.HoveredRoom`) (`KismetMathLibrary.MakeRotator` 0.0 0.0 _output_get) false false)
    (`SceneComponent.K2_SetWorldRotation` (`self.FocusPoint`) (`KismetMathLibrary.MakeRotator` 0.0 0.0 _output_get) false false)))

(event `self.ExitTable`
  (bind _character (`self.Character`))
  (bind _hoveredroom (`self.HoveredRoom`))
  (if (not (`self.IsRoomInFocus`))
    (`Widget.RemoveFromParent` (`self.WBP_ModelBoard`))
    (`EnhancedInputSubsystemInterface.RemoveMappingContext` (pcsubsystem `EnhancedInputLocalPlayerSubsystem` (`self.Controller`)) "/Game/ElCortijo/Features/1_MainCharacter/Input/IMC_Table.IMC_Table" (struct))
    (clear `/Game/ElCortijo/Features/1_MainCharacter/Blueprints/BP_FirstPersonCharacter.OnCameraHPress` _character)
    (clear `/Game/ElCortijo/Features/1_MainCharacter/Blueprints/BP_FirstPersonCharacter.OnCameraVPress` _character)
    (`parent.ExitTable`)
    (`KismetSystemLibrary.Delay` (`self.AnimBlendTime`))
    (`self.ClearHover` _hoveredroom)
    (set `self.HoveredRoom` _hoveredroom)))

(fn `AddNewOBJEvidence`
  (params (BP_Evidence :type "/Game/ElCortijo/Features/3_InteractableElements/1_IObjects/Evidence/BP_Evidence Object Reference"))
  (bind _asbp_object_evidence_v2 (cast `/Game/ElCortijo/Features/3_InteractableElements/1_IObjects/Evidence/BP_ObjectEvidenceV2` BP_Evidence))
  (bind _slotindex (`/Game/ElCortijo/Features/3_InteractableElements/1_IObjects/Evidence/BP_Evidence.SlotIndex` _asbp_object_evidence_v2))
  (bind (_value _returnvalue) (`BlueprintMapLibrary.Map_Find` (`self.EvidenceSpots`) _slotindex))
  (if _returnvalue
    (`BlueprintMapLibrary.Map_Add` (`self.EvidenceInTable`) _slotindex _asbp_object_evidence_v2)
    (`self.K2_AttachToComponent` BP_Evidence _value "None" "SnapToTarget" "SnapToTarget" "KeepRelative" true)
    (bind (_returnvalue_x _returnvalue_y _returnvalue_z) (`KismetMathLibrary.BreakVector` (`SceneComponent.K2_GetComponentLocation` (`/Game/ElCortijo/Features/2_InteractionSystem/Pickable/BP_Pickable.Collision` _asbp_object_evidence_v2))))
    (`self.K2_SetActorLocation` BP_Evidence (`KismetMathLibrary.MakeVector` _returnvalue_x _returnvalue_y (+ _returnvalue_z (`/Game/ElCortijo/Features/3_InteractableElements/1_IObjects/Evidence/BP_ObjectEvidenceV2.Offset` _asbp_object_evidence_v2))) false false)
    (`/Game/ElCortijo/Features/2_InteractionSystem/Pickable/BP_Pickable.SetPhysics` BP_Evidence false)
    (`/Game/ElCortijo/Features/2_InteractionSystem/Pickable/BP_Pickable.SetInteractable` BP_Evidence false)
    (`/Game/ElCortijo/Features/3_InteractableElements/1_IObjects/Evidence/BP_Evidence.SetTable` BP_Evidence self)
    (return)
    (else
      (`KismetSystemLibrary.PrintString` "NoSlot"))))

(fn `BuildHover`
  (params (Target :type "SceneComponent Object Reference"))
  (for _array_element (`SceneComponent.GetChildrenComponents` Target true)
    (bind _asprimitive_component (cast `PrimitiveComponent` _array_element))
    (`KismetArrayLibrary.Array_Add` (`self.HoveredRoomComponents`) _asprimitive_component))
  (for _array_element_2 (`self.HoveredRoomComponents`)
    (bind _asmesh_component (cast `MeshComponent` _array_element_2))
    (`MeshComponent.SetOverlayMaterial` _asmesh_component (`self.HoverMaterial`))))

(fn `ChechForEvidence`
  (params (Room :type "SceneComponent Object Reference") (EnableClick :type Boolean))
  (for _array_element (`SceneComponent.GetChildrenComponents` Room true)
    (bind (_id _isevidence) (`self.CheckEvidenceTag` _array_element))
    (if _isevidence
      (bind (_value _returnvalue) (`BlueprintMapLibrary.Map_Find` (`self.EvidenceInTable`) (`KismetStringLibrary.Conv_StringToInt` _id)))
      (if _returnvalue
        (`/Game/ElCortijo/Features/3_InteractableElements/1_IObjects/Evidence/BP_Evidence.SetClickable` _value EnableClick)
        (if EnableClick
          (bind _rootcomponent (`Actor.RootComponent` _value))
          (`self.BuildHover` _rootcomponent)
          (else
            (`self.ClearHover` _rootcomponent)))))))

(fn `CheckEvidenceTag`
  (params (Evidence :type "SceneComponent Object Reference"))
  (returns (ID :type String) (IsEvidence :type Boolean))
  (bind _componenttags (`ActorComponent.ComponentTags` Evidence))
  (bind _returnvalue (`KismetStringLibrary.ParseIntoArray` (`KismetStringLibrary.Conv_NameToString` (`|GetArrayItem` _componenttags)) "_" false))
  (if (`KismetArrayLibrary.Array_IsNotEmpty` _componenttags)
    (return (`|GetArrayItem` _returnvalue 1) (== (`|GetArrayItem` _returnvalue) "Evidence"))))

(fn `ClearHover`
  (params (Target :type "SceneComponent Object Reference"))
  (locals (Holder :type "Array of PrimitiveComponent Object Reference"))
  (set `local.Holder` (`self.HoveredRoomComponents`))
  (for _array_element (`SceneComponent.GetChildrenComponents` Target true)
    (bind _asmesh_component (cast `MeshComponent` _array_element))
    (`MeshComponent.SetOverlayMaterial` _asmesh_component null)
    (bind _asprimitive_component (cast `PrimitiveComponent` _array_element))
    (`KismetArrayLibrary.Array_RemoveItem` (`local.Holder`) _asprimitive_component))
  (set `self.HoveredRoomComponents` (`local.Holder`)))

(fn `ClickEvidence`
  (bind (_bblockinghit _binitialoverlap _time _distance _location _impactpoint _normal _impactnormal _physmat _hitactor) (`GameplayStatics.BreakHitResult` (`PlayerController.GetHitResultUnderCursorByChannel` (`self.Controller`) "TraceTypeQuery5" true)))
  (if (`KismetSystemLibrary.DoesImplementInterface` _hitactor "/Game/ElCortijo/Features/2_InteractionSystem/BPI_Clickable.BPI_Clickable_C")
    (bind _asbp_evidence (cast `/Game/ElCortijo/Features/3_InteractableElements/1_IObjects/Evidence/BP_Evidence` _hitactor))
    (set `self.DescriptinObject` _asbp_evidence)
    (`self.SetDescriptonOnScreen`)))

(fn `GetAllEvidenceSpots`
  (bind _evidencespots (`self.EvidenceSpots`))
  (for _array_element (`SceneComponent.GetChildrenComponents` (`self.BP_Maqueta`) true)
    (bind (_id _isevidence) (`self.CheckEvidenceTag` _array_element))
    (if _isevidence
      (bind _returnvalue (`KismetStringLibrary.Conv_StringToInt` _id))
      (if (not (`BlueprintMapLibrary.Map_Contains` _evidencespots _returnvalue))
        (`BlueprintMapLibrary.Map_Add` _evidencespots _returnvalue _array_element)))))

(fn `LeftclickZoomLogic`
  (bind _hoveredroom (`self.HoveredRoom`))
  (if (not (`self.IsRoomAnimating`))
    (if (!= _hoveredroom null)
      (set `self.FocusRoomLastTransform` (`SceneComponent.K2_GetComponentToWorld` _hoveredroom))
      (set `self.IsRoomAnimating` true)
      (set `self.IsRoomInFocus` true)
      (set `self.NeedsFocus` true)
      (`self.ClearHover` (`self.HoveredRoom`))
      (`self.ChechForEvidence` (`self.HoveredRoom`) true))))

(fn `RightclickZoomLogic`
  (if (`self.IsRoomInFocus`)
    (if (not (`self.IsRoomAnimating`))
      (if (!= (`self.HoveredRoom`) null)
        (set `self.IsRoomAnimating` true)
        (set `self.NeedsFocus` false)
        (`self.BuildHover` (`self.HoveredRoom`))
        (`self.ChechForEvidence` (`self.HoveredRoom`))))))

(fn `RoomHover`
  (locals (NeedsClear :type Boolean) (Valid :type Boolean) (NewLocalVar :type "SceneComponent Object Reference"))
  (bind (_bblockinghit _binitialoverlap _time _distance _location _impactpoint _normal _impactnormal _physmat _hitactor _hitcomponent) (`GameplayStatics.BreakHitResult` (`PlayerController.GetHitResultUnderCursorByChannel` (`self.Controller`) "TraceTypeQuery5" true)))
  (bind _output (`|GetArrayItem` (`SceneComponent.GetParentComponents` _hitcomponent)))
  (if (`self.PlayerInTable`)
    ; Check if hitting clickable room, if not clear hover
    (if _bblockinghit
      ; Set Validity
      (set `local.Valid` false)
      (for _array_element (`ActorComponent.ComponentTags` _output)
        (if (== _array_element "Room")
          (set `local.Valid` true)))
      ; Checks
      (if (`local.Valid`)
        (if (!= (`self.HoveredRoom`) _output)
          ; Clear PastObj if needed
          (if (!= (`self.HoveredRoom`) null)
            (for _array_element_2 (`self.HoveredRoomComponents`)
              (bind _asmesh_component (cast `MeshComponent` _array_element_2))
              (`MeshComponent.SetOverlayMaterial` _asmesh_component null))
            (`KismetArrayLibrary.Array_Clear` (`self.HoveredRoomComponents`)))
          ; Add NewObj
          (for _array_element_3 (`SceneComponent.GetChildrenComponents` _output false)
            (bind _asprimitive_component (cast `PrimitiveComponent` _array_element_3))
            (`KismetArrayLibrary.Array_Add` (`self.HoveredRoomComponents`) _asprimitive_component))
          ; Set new material and OBJ
          (for _array_element_4 (`self.HoveredRoomComponents`)
            (bind _asmesh_component_2 (cast `MeshComponent` _array_element_4))
            (`MeshComponent.SetOverlayMaterial` _asmesh_component_2 (`self.HoverMaterial`)))
          (set `self.HoveredRoom` _output)))
      (else
        (for _array_element_5 (`self.HoveredRoomComponents`)
          (bind _asmesh_component_3 (cast `MeshComponent` _array_element_5 :!label _label))
          (`MeshComponent.SetOverlayMaterial` _asmesh_component_3 null))
        (`KismetArrayLibrary.Array_Clear` (`self.HoveredRoomComponents`))
        (set `self.HoveredRoom` null)))
    (else
      (goto _label))))

(fn `SetDescriptonOnScreen`
  (`/Game/ElCortijo/Features/4_InteractableTables/ModelBoard/UI/WBP_ModelBoard.SetEvidenceNotesOnDescription` (`self.WBP_ModelBoard`) (`self.DescriptinObject`)))

(fn `UserConstructionScript`
  (`parent.UserConstructionScript`))