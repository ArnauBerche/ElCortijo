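; BP_Table is an interactable table that the first-person character can enter and exit by interacting with it.
; Interact caches the character and its controller, then toggles between entering and exiting while setting the character's current table.
; Entering blends the view to the table camera, locks look and movement, and shows the cursor; exiting reverses this.
; A CanInteract flag blocks repeat interaction during each timed camera blend.
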(event `EnterTable`
  (bind _controller (`self.Controller`))
  (`Controller.SetIgnoreLookInput` _controller true)
  (`Controller.SetIgnoreMoveInput` _controller true)
  (`PlayerController.SetViewTargetWithBlend` _controller (`ActorComponent.GetOwner` (`self.Camera`)) (`self.AnimBlendTime`) "VTBlend_Linear" 0.0 false)
  (set `PlayerController.bShowMouseCursor` true (`self.Controller`))
  (set `self.CanInteract` false)
  (`WidgetBlueprintLibrary.SetInputMode_GameAndUIEx` (`self.Controller`) null "DoNotLock" false true)
  (`KismetSystemLibrary.Delay` (`self.AnimBlendTime`))
  (set `self.CanInteract` true)
  (bind _output_get (set `self.PlayerInTable` true))
  (set `/Game/ElCortijo/Features/1_MainCharacter/Blueprints/BP_FirstPersonCharacter.BIsInTable` _output_get (`self.Character`)))

(event `ExitTable`
  (bind _controller (`self.Controller`))
  (`PlayerController.SetViewTargetWithBlend` (`self.Controller`) (`self.Character`) (`self.AnimBlendTime`) "VTBlend_Linear" 0.0 false)
  (set `self.CanInteract` false)
  (`KismetSystemLibrary.Delay` (`self.AnimBlendTime`))
  (set `self.CanInteract` true)
  (`Controller.SetIgnoreLookInput` _controller false)
  (`Controller.SetIgnoreMoveInput` _controller false)
  (set `PlayerController.bShowMouseCursor` false _controller)
  (`WidgetBlueprintLibrary.SetInputMode_GameOnly` _controller true)
  (bind _output_get (set `self.PlayerInTable` false))
  (set `/Game/ElCortijo/Features/1_MainCharacter/Blueprints/BP_FirstPersonCharacter.BIsInTable` _output_get (`self.Character`)))

(event `/Game/ElCortijo/Features/2_InteractionSystem/BPI_Interactable.Interact`
  (params (Interactor :type "Actor Object Reference"))
  (`self.OnInteract` Interactor)
  (if (`self.CanInteract`)
    (if (`self.PlayerInTable`)
      (`self.ExitTable`)
      (set `/Game/ElCortijo/Features/1_MainCharacter/Blueprints/BP_FirstPersonCharacter.CurrentTable` null (`self.Character`))
      (else
        (`self.EnterTable`)
        (set `/Game/ElCortijo/Features/1_MainCharacter/Blueprints/BP_FirstPersonCharacter.CurrentTable` self (`self.Character`))))))

(fn `OnInteract`
  (params (Interactor :type "Actor Object Reference"))
  (if (`self.CanInteract`)
    (bind _asbp_first_person_character (cast `/Game/ElCortijo/Features/1_MainCharacter/Blueprints/BP_FirstPersonCharacter` Interactor))
    (set `self.Character` _asbp_first_person_character)
    (bind _asplayer_controller (cast `PlayerController` (`Pawn.GetController` _asbp_first_person_character)))
    (set `self.Controller` _asplayer_controller)))

(fn `UserConstructionScript`)