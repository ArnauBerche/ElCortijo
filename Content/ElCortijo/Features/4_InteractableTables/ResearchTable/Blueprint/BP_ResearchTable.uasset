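; Interactable research table where the player inspects a held clue item up close and clicks clickable spots on it.
; On entry it scales the clue to a target size, isolates its meshes via a show-only SceneCapture2D and separate lighting channel, and adds table UI and input.
; Camera input rotates it, zoom adjusts rotation speed, and cursor traces send BPI_Clickable messages.
; Exiting restores the clue; helpers manage evidence slots and GameInstance notes.
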(event `self.ReceiveBeginPlay`
  (set `self.TType` "NewEnumerator0")
  (bind _asbp_first_person_character (cast `/Game/ElCortijo/Features/1_MainCharacter/Blueprints/BP_FirstPersonCharacter` (`GameplayStatics.GetPlayerCharacter` 0)))
  (`|ExecutionSequence`
    (:`then_0`
      (for _array_element (`SceneComponent.GetChildrenComponents` (`self.ProofPlacement`) true)
        (bind _asstatic_mesh_component (cast `StaticMeshComponent` _array_element))
        (`KismetArrayLibrary.Array_Add` (`self.HintPlacementsRef`) (make `/Game/ElCortijo/Features/4_InteractableTables/S_TablePlacements` _asstatic_mesh_component null))))
    (:`then_1`
      (add `/Game/ElCortijo/Features/1_MainCharacter/Blueprints/BP_FirstPersonCharacter.OnLeftClickPress` _asbp_first_person_character (delegate `OnLeftClick_Handler`))
      (add `/Game/ElCortijo/Features/1_MainCharacter/Blueprints/BP_FirstPersonCharacter.OnResearchPress` _asbp_first_person_character (delegate `OnStartResearch`)))))

(event `OnLeftClick_Handler`
  (`self.LeftClickPress`))

(event `OnStartResearch`
  (params (PlayerRef :type "/Game/ElCortijo/Features/1_MainCharacter/Blueprints/BP_FirstPersonCharacter Object Reference"))
  (`parent.Interact` PlayerRef))

(event `self.EnterTable`
  (bind _character (`self.Character`))
  (bind _output_get (set `self.Inventory Slot` (`/Game/ElCortijo/Features/1_MainCharacter/Blueprints/BP_FirstPersonCharacter.InventorySlot` (`self.Character`))))
  (bind _empty (`/Game/ElCortijo/Features/1_MainCharacter/BP_InventoryComponent.IsEmpty` _output_get))
  (cast `/Game/ElCortijo/Features/3_InteractableElements/1_IObjects/Clues/ClueHotspot/BP_ClueItem` (`/Game/ElCortijo/Features/1_MainCharacter/BP_InventoryComponent.CurrentItemActor` _output_get))
  (if (not _empty)
    (`parent.EnterTable`)
    (`self.CreateResearchableObject` _output_get)
    (bind _returnvalue (`|CreateWidget` "/Game/ElCortijo/Features/4_InteractableTables/ResearchTable/UI/WBP_ResearchTable.WBP_ResearchTable_C"))
    (bind _output_get_2 (set `self.UIResearchTable` _returnvalue))
    (`UserWidget.AddToViewport` _output_get_2 0)
    (`EnhancedInputSubsystemInterface.AddMappingContext` (pcsubsystem `EnhancedInputLocalPlayerSubsystem` (`self.Controller`)) "/Game/ElCortijo/Features/1_MainCharacter/Input/IMC_Table.IMC_Table" 100 (struct))
    (add `/Game/ElCortijo/Features/1_MainCharacter/Blueprints/BP_FirstPersonCharacter.OnCameraHPress` _character (delegate `RotateH`))
    (add `/Game/ElCortijo/Features/1_MainCharacter/Blueprints/BP_FirstPersonCharacter.OnCameraVPress` _character (delegate `RotateV`))
    (add `/Game/ElCortijo/Features/1_MainCharacter/Blueprints/BP_FirstPersonCharacter.OnCameraZoom` _character (delegate `RotateSpeed`))
    (for _array_element (`self.GetAttachedActors` (`self.ResearchableObject`) true true)
      (bind _asbp_bill_board (cast `/Game/ElCortijo/Features/0_Unsorted/BP_BillBoard` _array_element))
      (`SceneComponent.SetVisibility` (`/Game/ElCortijo/Features/0_Unsorted/BP_BillBoard.Scene` _asbp_bill_board) false true))))

(event `RotateH`
  (params (Value :type "Float (double-precision)"))
  (`self.Rotate_H` Value))

(event `RotateV`
  (params (Value :type "Float (double-precision)"))
  (`self.Rotate_V` Value))

(event `RotateSpeed`
  (params (Value :type "Float (double-precision)"))
  (`self.Rotate_Speed` Value))

(event `self.ExitTable`
  (bind _character (`self.Character`))
  (bind _inventory_slot (`self.Inventory Slot`))
  (for _array_element (`self.GetAttachedActors` (`self.ResearchableObject`) true true)
    (bind _asbp_bill_board (cast `/Game/ElCortijo/Features/0_Unsorted/BP_BillBoard` _array_element))
    (`SceneComponent.SetVisibility` (`/Game/ElCortijo/Features/0_Unsorted/BP_BillBoard.Scene` _asbp_bill_board) true true))
  (`self.DestroyReserchableObject` (`self.Character`))
  (`Widget.RemoveFromParent` (`self.UIResearchTable`))
  (`KismetSystemLibrary.CollectGarbage`)
  (bind _asbp_clue_item (cast `/Game/ElCortijo/Features/3_InteractableElements/1_IObjects/Clues/ClueHotspot/BP_ClueItem` (`/Game/ElCortijo/Features/1_MainCharacter/BP_InventoryComponent.CurrentItemActor` _inventory_slot)))
  (`/Game/ElCortijo/Features/1_MainCharacter/BP_InventoryComponent.DropOnExactTransform` _inventory_slot (`/Game/ElCortijo/Features/3_InteractableElements/1_IObjects/Clues/ClueHotspot/BP_ClueItem.GrabSpot` _asbp_clue_item))
  (`EnhancedInputSubsystemInterface.RemoveMappingContext` (pcsubsystem `EnhancedInputLocalPlayerSubsystem` (`self.Controller`)) "/Game/ElCortijo/Features/1_MainCharacter/Input/IMC_Table.IMC_Table" (struct))
  (clear `/Game/ElCortijo/Features/1_MainCharacter/Blueprints/BP_FirstPersonCharacter.OnCameraHPress` _character)
  (clear `/Game/ElCortijo/Features/1_MainCharacter/Blueprints/BP_FirstPersonCharacter.OnCameraVPress` _character)
  (`parent.ExitTable`))

(fn `CreateEvidence`
  (params (Evidence :type "/Game/ElCortijo/Features/3_InteractableElements/1_IObjects/WorldElements/S_Note Structure"))
  (bind _asbp_game_instance (cast `/Game/ElCortijo/Features/0_Unsorted/GameInstance/BP_GameInstance` (`GameplayStatics.GetGameInstance`)))
  (`/Game/ElCortijo/Features/0_Unsorted/GameInstance/BP_GameInstance.AddNote` _asbp_game_instance Evidence))

(fn `CreateResearchableObject`
  (params (InventSlot :type "/Game/ElCortijo/Features/1_MainCharacter/BP_InventoryComponent Object Reference"))
  (locals (TargetSize :type "Vector Structure" :default (30.0 30.0 30.0)))
  (bind _output_get (set `self.Inventory Slot` InventSlot))
  (bind _asbp_clue_item (cast `/Game/ElCortijo/Features/3_InteractableElements/1_IObjects/Clues/ClueHotspot/BP_ClueItem` (`/Game/ElCortijo/Features/1_MainCharacter/BP_InventoryComponent.CurrentItemActor` _output_get)))
  (bind (_smc_ci _collision_ci) (`/Game/ElCortijo/Features/3_InteractableElements/1_IObjects/Clues/ClueHotspot/BP_ClueItem.OnPlacedOnTable` _asbp_clue_item self))
  (set `self.SMC_CI` _smc_ci)
  (set `self.Collision CI` _collision_ci)
  (set `self.ResearchableObject` _asbp_clue_item)
  (`/Game/ElCortijo/Features/1_MainCharacter/BP_InventoryComponent.EmptyInventoryRef` _output_get)
  (bind (_origin _boxextent) (`self.GetActorBounds` _asbp_clue_item true true))
  (`self.SetActorScale3D` _asbp_clue_item (* (`self.GetActorScale3D` _asbp_clue_item) (/ (`local.TargetSize`) (* (`KismetMathLibrary.FMax` (`KismetMathLibrary.FMax` (.x _boxextent) (.y _boxextent)) (.z _boxextent)) 2.0))))
  (`SceneCaptureComponent.ClearShowOnlyComponents` (`self.SceneCaptureComponent2D`))
  (for _array_element (`self.SMC_CI`)
    (bind _asstatic_mesh_component (cast `StaticMeshComponent` _array_element))
    (`PrimitiveComponent.SetVisibleInSceneCaptureOnly` _asstatic_mesh_component true)
    (`SceneCaptureComponent.ShowOnlyComponent` (`self.SceneCaptureComponent2D`) _asstatic_mesh_component)
    (`PrimitiveComponent.SetLightingChannels` _asstatic_mesh_component false true false))
  (`PrimitiveComponent.SetCollisionEnabled` (`self.Collision CI`) "NoCollision")
  (return))

(fn `DestroyReserchableObject`
  (params (Interactor :type "/Game/ElCortijo/Features/1_MainCharacter/Blueprints/BP_FirstPersonCharacter Object Reference"))
  (bind _researchableobject (`self.ResearchableObject`))
  (if (!= _researchableobject null)
    (`/Game/ElCortijo/Features/3_InteractableElements/1_IObjects/Clues/ClueHotspot/BP_ClueItem.SetAllHotspotsActive` _researchableobject false)
    (`/Game/ElCortijo/Features/1_MainCharacter/BP_InventoryComponent.PickUpActor` (`/Game/ElCortijo/Features/1_MainCharacter/Blueprints/BP_FirstPersonCharacter.InventorySlot` Interactor) _researchableobject)
    (for _array_element (`self.SMC_CI`)
      (bind _asstatic_mesh_component (cast `StaticMeshComponent` _array_element))
      (`PrimitiveComponent.SetVisibleInSceneCaptureOnly` _asstatic_mesh_component false)
      (`PrimitiveComponent.SetLightingChannels` _asstatic_mesh_component true false false))
    (`SceneCaptureComponent.ClearShowOnlyComponents` (`self.SceneCaptureComponent2D`))
    (`PrimitiveComponent.SetCollisionEnabled` (`self.Collision CI`) "QueryAndPhysics")
    (`KismetArrayLibrary.Array_Clear` (`self.SMC_CI`))
    (set `self.Collision CI` null)
    (set `self.ResearchableObject` null)
    (return)))

(fn `GetFirstEmptySlot`
  (returns (Slot :type Integer) (IsRoom :type Boolean))
  (locals (TempSlot :type Integer) (TempIsRoom :type Boolean))
  (set `local.TempIsRoom` false)
  (for (_array_element _array_index) (`self.HintPlacementsRef`)
    (if (== (`.Evidence_7_18C52045475546F6D7C545884F8868D5` (break `/Game/ElCortijo/Features/4_InteractableTables/S_TablePlacements` _array_element)) null)
      (set `local.TempIsRoom` true)
      (set `local.TempSlot` _array_index)
      (break)))
  (return (`local.TempSlot`) (`local.TempIsRoom`)))

(fn `LeftClickPress`
  (bind (_bblockinghit _binitialoverlap _time _distance _location _impactpoint _normal _impactnormal _physmat _hitactor) (`GameplayStatics.BreakHitResult` (`PlayerController.GetHitResultUnderCursorByChannel` (`GameplayStatics.GetPlayerController` 0) "TraceTypeQuery5" true)))
  (if (!= (`self.ResearchableObject`) null)
    (if (`self.PlayerInTable`)
      (if (`KismetSystemLibrary.DoesImplementInterface` _hitactor "/Game/ElCortijo/Features/2_InteractionSystem/BPI_Clickable.BPI_Clickable_C")
        (message `/Game/ElCortijo/Features/2_InteractionSystem/BPI_Clickable.Click` _hitactor null)))))

(fn `RemoveEvidence`
  (params (SlotIndex :type Integer))
  (bind _output (`|GetArrayItem` (`self.HintPlacementsRef`) SlotIndex))
  (`|VariableSetRef` _output (make `/Game/ElCortijo/Features/4_InteractableTables/S_TablePlacements` (`.Placement_2_FD44286F48BEEE48D0811A9809672CC7` (break `/Game/ElCortijo/Features/4_InteractableTables/S_TablePlacements` _output)) null)))

(fn `Rotate_H`
  (params (value :type "Float (double-precision)"))
  (`SceneComponent.K2_AddWorldRotation` (`Actor.RootComponent` (`self.ResearchableObject`)) (`KismetMathLibrary.RotatorFromAxisAndAngle` (`SceneComponent.GetUpVector` (`self.Camera`)) (* value (`self.RotSpeed`))) false false))

(fn `Rotate_Speed`
  (params (Value :type "Float (double-precision)"))
  (set `self.RotSpeed` (`KismetMathLibrary.FClamp` (+ (`self.RotSpeed`) (* Value -1.0)) 1.0 4.0)))

(fn `Rotate_V`
  (params (Value :type "Float (double-precision)"))
  (`SceneComponent.K2_AddWorldRotation` (`Actor.RootComponent` (`self.ResearchableObject`)) (`KismetMathLibrary.RotatorFromAxisAndAngle` (`SceneComponent.GetRightVector` (`self.Camera`)) (* Value (`self.RotSpeed`))) false false))

(fn `UserConstructionScript`)