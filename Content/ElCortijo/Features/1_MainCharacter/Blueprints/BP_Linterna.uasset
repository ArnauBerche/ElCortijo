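; Player flashlight actor that toggles its light and plays FMOD on/off sounds.
; On BeginPlay it binds to BP_FirstPersonCharacter's flashlight on/off dispatchers, which show or hide the Proj and Vol components and track the on state.
; A looping three-second timer plays a timeline that drives Proj intensity for a flicker while on; its random check has weight 1.0, so it always passes.
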(event `self.ReceiveTick`
  (params (DeltaSeconds :type "Float (single-precision)")))

(event `TimedFlicker`
  (if (and (`self.IsOn`) (`KismetMathLibrary.RandomBoolWithWeight` 1.0))
    (bind (_direction _intensity) (`Timeline|Flicker` :!via `PlayFromStart`)
      (:`Update`
        (`LightComponent.SetIntensity` (`self.Proj`) _intensity)))))

(event `self.ReceiveBeginPlay`
  (`|ExecutionSequence`
    (:`then_0`
      (`KismetSystemLibrary.K2_SetTimerDelegate` (delegate `TimedFlicker`) 3.0 true))
    (:`then_1`
      (bind _asbp_first_person_character (cast `/Game/ElCortijo/Features/1_MainCharacter/Blueprints/BP_FirstPersonCharacter` (`GameplayStatics.GetPlayerCharacter` 0)))
      (add `/Game/ElCortijo/Features/1_MainCharacter/Blueprints/BP_FirstPersonCharacter.OnFlaslightOn` _asbp_first_person_character (delegate `Open`))
      (add `/Game/ElCortijo/Features/1_MainCharacter/Blueprints/BP_FirstPersonCharacter.OnFlashlightOff` _asbp_first_person_character (delegate `Close`)))))

(event `Open`
  (bind _fmodaudio (`self.FMODAudio`))
  (set `self.IsOn` true)
  (`SceneComponent.SetVisibility` (`self.Proj`) true true)
  (`SceneComponent.SetVisibility` (`self.Vol`) true true)
  (`FMODAudioComponent.SetEvent` _fmodaudio "/Game/FMOD/Events/SFX/Linterna/SFX_18_EncenderLinterna.SFX_18_EncenderLinterna")
  (`FMODAudioComponent.Play` _fmodaudio))

(event `Close`
  (bind _fmodaudio (`self.FMODAudio`))
  (set `self.IsOn` false)
  (`SceneComponent.SetVisibility` (`self.Proj`) false true)
  (`SceneComponent.SetVisibility` (`self.Vol`) false true)
  (`FMODAudioComponent.SetEvent` _fmodaudio "/Game/FMOD/Events/SFX/Linterna/SFX_19_ApagarLinterna.SFX_19_ApagarLinterna")
  (`FMODAudioComponent.Play` _fmodaudio))

(fn `UserConstructionScript`)