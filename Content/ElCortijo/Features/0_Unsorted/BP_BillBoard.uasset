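; Interaction prompt billboard that fades in as the player approaches and turns to face the camera.
; BeginPlay creates a dynamic billboard material on the plane with both opacity layers hidden.
; While the player is within range, Tick rotates it toward the camera and fades in a circle, then an E icon at closer distance, by remapped distance.
; It destroys itself once its owner is no longer valid.
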(event `self.ReceiveBeginPlay`
  (bind _returnvalue (`PrimitiveComponent.CreateDynamicMaterialInstance` (`self.Plane`) 0 "/Game/ElCortijo/Features/0_Unsorted/M_Billboard.M_Billboard" "None"))
  (set `self.DynamicBillboardMat` _returnvalue)
  (`MaterialInstanceDynamic.SetScalarParameterValue` (`self.DynamicBillboardMat`) "OpacityCircle" 0.0)
  (`MaterialInstanceDynamic.SetScalarParameterValue` (`self.DynamicBillboardMat`) "OpacityE" 0.0))

(event `self.ReceiveTick`
  (params (DeltaSeconds :type "Float (single-precision)"))
  (bind _returnvalue (`self.K2_GetActorLocation`))
  (bind _returnvalue_2 (`KismetMathLibrary.Vector_Distance` (`self.K2_GetActorLocation` (`GameplayStatics.GetPlayerPawn` 0)) _returnvalue))
  (if (`KismetSystemLibrary.IsValid` (`self.GetOwner`))
    (if (`KismetMathLibrary.InRange_FloatFloat` _returnvalue_2 0.0 500.0)
      (`self.K2_SetActorRotation` (`KismetMathLibrary.FindLookAtRotation` _returnvalue (`PlayerCameraManager.GetCameraLocation` (`GameplayStatics.GetPlayerCameraManager` 0))))
      (`MaterialInstanceDynamic.SetScalarParameterValue` (`self.DynamicBillboardMat`) "OpacityCircle" (- 1.0 (`KismetMathLibrary.FClamp` (`KismetMathLibrary.NormalizeToRange` _returnvalue_2 50.0 350.0))))
      (`MaterialInstanceDynamic.SetScalarParameterValue` (`self.DynamicBillboardMat`) "OpacityE" (- 1.0 (`KismetMathLibrary.FClamp` (`KismetMathLibrary.NormalizeToRange` _returnvalue_2 50.0 150.0) 0.0 1.0))))
    (else
      (`self.K2_DestroyActor`))))

(fn `UserConstructionScript`)