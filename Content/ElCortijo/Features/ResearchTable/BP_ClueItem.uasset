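; BP_ClueItem is a clue that can be placed on a research table, exposing hotspots while it sits there.
; On BeginPlay it collects its BP_ClueHotspot child actors, sets itself as their owner and deactivates them.
; Placing it snaps it to the table's ProofPlacement and activates every unconsumed hotspot; removal deactivates them and clears the table reference.
; RegisterHotspot is an empty stub.
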(event `self.ReceiveBeginPlay`
  (`parent.ReceiveBeginPlay`)
  (for _array_element (`self.GetAllChildActors` true)
    (bind _asbp_clue_hotspot (cast `/Game/ElCortijo/Features/ResearchTable/BP_ClueHotspot` _array_element))
    (set `/Game/ElCortijo/Features/ResearchTable/BP_ClueHotspot.OwnerClue` self _asbp_clue_hotspot)
    (`KismetSystemLibrary.PrintText` "Hotspot added")
    (`KismetArrayLibrary.Array_Add` (`self.Hotspots`) _asbp_clue_hotspot)
    (`/Game/ElCortijo/Features/ResearchTable/BP_ClueHotspot.SetActive` _asbp_clue_hotspot false)))

(fn `OnPlacedOnTable`
  (params (Table :type "/Game/ElCortijo/Features/ResearchTable/Blueprint/BP_ResearchTable Object Reference"))
  (bind _output_get (set `self.CurrentResearchTable` Table))
  (`self.K2_AttachToComponent` (`/Game/ElCortijo/Features/ResearchTable/Blueprint/BP_ResearchTable.ProofPlacement` _output_get) "None" "SnapToTarget" "SnapToTarget" "KeepWorld")
  (`self.K2_SetActorRelativeLocation` (0.0 0.0 0.0) false true)
  (set `self.bPlacedOnResearchTable` true)
  (`self.SetAllHotspotsActive` true))

(fn `OnRemovedFromTable`
  (`self.SetAllHotspotsActive` false)
  (set `self.CurrentResearchTable` null)
  (set `self.bPlacedOnResearchTable` false))

(fn `RegisterHotspot`
  (params (Hotspot :type "/Game/ElCortijo/Features/ResearchTable/BP_ClueHotspot Object Reference")))

(fn `SetAllHotspotsActive`
  (params (bActive :type Boolean))
  (for _array_element (`self.Hotspots`)
    (if (not (`/Game/ElCortijo/Features/ResearchTable/BP_ClueHotspot.bConsumed` _array_element))
      (`/Game/ElCortijo/Features/ResearchTable/BP_ClueHotspot.SetActive` _array_element bActive))))

(fn `UserConstructionScript`
  (`parent.UserConstructionScript`))