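; BP_ClueHotspot is a clickable hotspot on a clue that creates a piece of evidence on the research table.
; Its owner clue initializes it with evidence data; active, unconsumed hotspots show a decal and enable query-only collision.
; A click calls the table's CreateEvidence if the clue is placed on one, then marks the hotspot consumed, hiding and disabling it.
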(event `/Game/ElCortijo/Features/Interaction/BPI_Clickable.Click`
  (params (Interactor :type "Actor Object Reference"))
  (if (and (`self.bActive`) (not (`self.bConsumed`)))
    (`self.RequestCreateEvidence` (`self.EvidenceData`))))

(fn `Initialize`
  (params (Owner :type "/Game/ElCortijo/Features/ResearchTable/BP_ClueItem Object Reference") (Evidence :type "/Game/ElCortijo/Features/Evidence/BP_Evidence Class Reference"))
  (set `self.OwnerClue` Owner)
  (set `self.EvidenceData` Evidence)
  (`self.SetConsumed` false)
  (`self.SetActive` false))

(fn `RequestCreateEvidence`
  (params (Evidence :type "/Game/ElCortijo/Features/Evidence/BP_Evidence Class Reference"))
  (bind _ownerclue (`self.OwnerClue`))
  (bind _currenttable (`/Game/ElCortijo/Features/ResearchTable/BP_ClueItem.CurrentTable` _ownerclue))
  (if (`self.bConsumed`)
    _
    (elif (and (and (!= _ownerclue null) (`/Game/ElCortijo/Features/ResearchTable/BP_ClueItem.bPlacedOnResearchTable` _ownerclue)) (!= _currenttable null))
      (bind _asbp_research_table (cast `/Game/ElCortijo/Features/ResearchTable/Blueprint/BP_ResearchTable` _currenttable))
      (`/Game/ElCortijo/Features/ResearchTable/Blueprint/BP_ResearchTable.CreateEvidence` _asbp_research_table Evidence)
      (`self.SetConsumed` true))))

(fn `SetActive`
  (params (bActive :type Boolean))
  (bind _collider (`self.Collider`))
  (bind _output_get (set `self.bActive` bActive))
  (bind _returnvalue (and _output_get (not (`self.bConsumed`))))
  (if _returnvalue
    (`PrimitiveComponent.SetCollisionEnabled` _collider "QueryOnly")
    (else
      (`PrimitiveComponent.SetCollisionEnabled` _collider "NoCollision")))
  (`SceneComponent.SetHiddenInGame` (`self.Decal`) (not _returnvalue) false))

(fn `SetConsumed`
  (params (bConsumed :type Boolean))
  (bind _output_get (set `self.bConsumed` bConsumed))
  (if _output_get
    (`self.SetActive` false)))

(fn `UserConstructionScript`)