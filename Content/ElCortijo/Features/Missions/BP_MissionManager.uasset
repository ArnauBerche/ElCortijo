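; Mission manager Blueprint that tracks quest state and updates the HUD's mission name and stage description.
; StartMission looks up a mission row in a data table, skips ones already active or completed, then stores it with stage progress at zero.
; AdvanceMission steps the stage index and calls CompleteMission past the last stage, which moves the mission to completed and clears the HUD.
; Start, advance and completion can optionally play an audio cue.
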(fn `AdvanceMission`
  (params (MissionID :type Name) (PlayAudio :type Boolean))
  (locals (NewIndex :type Integer))
  (bind _missionprogress (`self.MissionProgress`))
  (bind (_value _returnvalue) (`BlueprintMapLibrary.Map_Find` _missionprogress MissionID))
  (bind _value_2 (`BlueprintMapLibrary.Map_Find` (`self.ActiveMissions`) MissionID))
  (if _returnvalue
    (bind _output_get (set `local.NewIndex` (+ _value 1)))
    (`BlueprintMapLibrary.Map_Add` _missionprogress MissionID _output_get)
    (if (< _output_get (`KismetArrayLibrary.Array_Length` (`.Stages_11_C2E03B0A43075B8416D99793B04F26F7` (break `/Game/ElCortijo/Features/Missions/S_Mission` _value_2))))
      (`/Game/ElCortijo/UI/W_HUD.UpdateMissionNameAndDescription` (`self.HUD`) (`.Name_10_7B03D3D94F296D206EA7548E13D4B3DA` (break `/Game/ElCortijo/Features/Missions/S_Mission` _value_2)) (`|GetArrayItem` (`.Stages_11_C2E03B0A43075B8416D99793B04F26F7` (break `/Game/ElCortijo/Features/Missions/S_Mission` _value_2)) (`local.NewIndex`)))
      (if PlayAudio
        (`AudioComponent.Play` (`self.Audio`) 0.2))
      (else
        (`self.CompleteMission` MissionID)))))

(fn `CompleteMission`
  (params (MissionID :type Name) (PlayAudio :type Boolean))
  (`KismetArrayLibrary.Array_Add` (`self.CompletedMissions`) MissionID)
  (`BlueprintMapLibrary.Map_Remove` (`self.ActiveMissions`) MissionID)
  (`/Game/ElCortijo/UI/W_HUD.UpdateMissionNameAndDescription` (`self.HUD`) " " " ")
  (if PlayAudio
    (`AudioComponent.Play` (`self.Audio`) 0.2)))

(fn `StartMission`
  (params (Mission :type Name) (PlaySound :type Boolean :default false))
  (bind _activemissions (`self.ActiveMissions`))
  (bind _returnvalue (`|GetDataTableRow` (`self.MissionTable`) Mission)
    (:`then`
      (if (not (or (`BlueprintMapLibrary.Map_Contains` _activemissions Mission) (`KismetArrayLibrary.Array_Contains` (`self.CompletedMissions`) Mission)))
        (`BlueprintMapLibrary.Map_Add` _activemissions Mission _returnvalue)
        (`BlueprintMapLibrary.Map_Add` (`self.MissionProgress`) Mission)
        (bind (_id _name _stages) (break `/Game/ElCortijo/Features/Missions/S_Mission` _returnvalue))
        (`/Game/ElCortijo/UI/W_HUD.UpdateMissionNameAndDescription` (`self.HUD`) _name (`|GetArrayItem` _stages))
        (if PlaySound
          (`AudioComponent.Play` (`self.Audio`) 0.2))))))

(fn `UserConstructionScript`)