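; File cabinet actor that stores the player's held item, or opens a browsing view when their hands are empty.
; A FlipFlop toggles that view, blending to the cabinet camera, locking movement and showing WBP_FileCabinet.
; Widget events cycle through stored items with wraparound, each previewed as a spawned non-physics BP_Pickable.
; Taking one moves it to the inventory slot and closes the view.
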(event `/Game/ElCortijo/Features/Interaction/BPI_Interactable.Interact`
  (params (Interactor :type "Actor Object Reference"))
  (bind _asbp_first_person_character (cast `/Game/FirstPerson/Blueprints/BP_FirstPersonCharacter` Interactor))
  (set `self.As BP First Person Character` _asbp_first_person_character)
  (bind _asplayer_controller (cast `PlayerController` (`Pawn.GetController` _asbp_first_person_character)))
  (set `self.As Player Controller` _asplayer_controller)
  (set `self.CameraOwner` (`ActorComponent.GetOwner` (`self.Camera`)))
  (if (`self.CanInteract`)
    (bind (_hasobjectinhand _iteminhand) (`self.Check Object InHand` (`self.As BP First Person Character`)))
    (if _hasobjectinhand
      (bind _output_get (set `self.Item in Hand` _iteminhand))
      (`KismetArrayLibrary.Array_Add` (`self.ItemsInCabinet`) _output_get)
      (`/Game/ElCortijo/Features/Character/BP_InventoryComponent.ClearItem` (`self.Inventory Slot`))
      (else
        (`/Engine/EditorBlueprintResources/StandardMacros.FlipFlop` :!label _label
          (:`A`
            (`Controller.SetIgnoreLookInput` (`self.As Player Controller`) true)
            (`Controller.SetIgnoreMoveInput` (`self.As Player Controller`) true)
            (`PlayerController.SetViewTargetWithBlend` (`self.As Player Controller`) (`self.CameraOwner`) (`self.Blend Time`) "VTBlend_Linear" 0.0 false)
            (set `PlayerController.bShowMouseCursor` true (`self.As Player Controller`))
            (set `self.CanInteract` false)
            (`WidgetBlueprintLibrary.SetInputMode_GameAndUIEx` (`self.As Player Controller`) (`self.WBP_FileCabinet`) "DoNotLock" false)
            (`KismetSystemLibrary.Delay` (`self.Blend Time`))
            (set `self.CanInteract` true)
            (set `self.PlayerInTable` true)
            (bind _returnvalue (`|CreateWidget` "/Game/ElCortijo/Features/FileCabinet/WBP_FileCabinet.WBP_FileCabinet_C" (`self.As Player Controller`)))
            (bind _output_get_2 (set `self.WBP_FileCabinet` _returnvalue))
            (`UserWidget.AddToViewport` _output_get_2 0)
            (set `self.ViewID` 0)
            (add `/Game/ElCortijo/Features/FileCabinet/WBP_FileCabinet.ClickGet` (`self.WBP_FileCabinet`) (delegate `Recive Item`))
            (add `/Game/ElCortijo/Features/FileCabinet/WBP_FileCabinet.ClickLast` (`self.WBP_FileCabinet`) (delegate `Previous Item`))
            (add `/Game/ElCortijo/Features/FileCabinet/WBP_FileCabinet.ClickNext` (`self.WBP_FileCabinet`) (delegate `Next Item`))
            (`self.Create Viewing Item` (`self.ViewID`)))
          (:`B`
            (`Widget.RemoveFromParent` (`self.WBP_FileCabinet`))
            (`self.Destroy Viewing Item`)
            (`PlayerController.SetViewTargetWithBlend` (`self.As Player Controller`) (`self.As BP First Person Character`) (`self.Blend Time`) "VTBlend_Linear" 0.0 false)
            (set `self.CanInteract` false)
            (`KismetSystemLibrary.Delay` (`self.Blend Time`))
            (set `self.CanInteract` true)
            (`Controller.SetIgnoreLookInput` (`self.As Player Controller`) false)
            (`Controller.SetIgnoreMoveInput` (`self.As Player Controller`) false)
            (set `PlayerController.bShowMouseCursor` false (`self.As Player Controller`))
            (`WidgetBlueprintLibrary.SetInputMode_GameOnly` (`self.As Player Controller`))
            (set `self.PlayerInTable` false)))))))

(event `Recive Item`
  (`self.Add Object To Hand`)
  (goto _label))

(event `Previous Item`
  (`self.Previous Item Logic`))

(event `Next Item`
  (`self.Next Item Logic`))

(fn `Add Object To Hand`
  (bind _viewid (`self.ViewID`))
  (bind _itemsincabinet (`self.ItemsInCabinet`))
  (`/Game/ElCortijo/Features/Character/BP_InventoryComponent.AddItem` (`self.Inventory Slot`) (`|GetArrayItem` _itemsincabinet _viewid))
  (`KismetArrayLibrary.Array_Remove` _itemsincabinet _viewid))

(fn `Check Object InHand`
  (params (Interactor :type "/Game/FirstPerson/Blueprints/BP_FirstPersonCharacter Object Reference"))
  (returns (HasObjectInHand :type Boolean) (ItemInHand :type "/Game/ElCortijo/Features/Interaction/Pickable/S_ItemData Structure"))
  (bind _inventoryslot (`/Game/FirstPerson/Blueprints/BP_FirstPersonCharacter.InventorySlot` Interactor))
  ; Check if item can be picked up
  (bind _output_get (set `self.Inventory Slot` _inventoryslot))
  (bind _canpickup (`/Game/ElCortijo/Features/Character/BP_InventoryComponent.CanPickup` :`self` _output_get))
  (return (not _canpickup) (`/Game/ElCortijo/Features/Character/BP_InventoryComponent.CurrentItem` _inventoryslot)))

(fn `Create Viewing Item`
  (params (ViewID :type Integer))
  (bind _showobject (`self.ShowObject`))
  (bind (_name _mesh _type _previewrotator _scale _objectoffset _collidersize _canpickup _candrop _isresearched) (break `/Game/ElCortijo/Features/Interaction/Pickable/S_ItemData` (`|GetArrayItem` (`self.ItemsInCabinet`) ViewID)))
  ; Set correct position and spawn Actor
  (bind _returnvalue (`|SpawnActorFromClass` "/Game/ElCortijo/Features/Interaction/Pickable/BP_Pickable.BP_Pickable_C" (`KismetMathLibrary.MakeTransform` (`SceneComponent.K2_GetComponentLocation` _showobject) (`SceneComponent.K2_GetComponentRotation` _showobject) _scale) "AlwaysSpawn" "MultiplyWithRoot" null (make `/Game/ElCortijo/Features/Interaction/Pickable/S_ItemData` _name _mesh _type _previewrotator _scale _objectoffset _collidersize false false _isresearched) true null))
  ; Set collision channel to research
  (`PrimitiveComponent.SetCollisionResponseToChannel` (`/Game/ElCortijo/Features/Interaction/Pickable/BP_Pickable.Collision` _returnvalue) "ECC_GameTraceChannel2" "ECR_Block")
  ; Turn off physics
  (bind _output_get (set `self.ResearchableObject` _returnvalue))
  (`PrimitiveComponent.SetSimulatePhysics` (`/Game/ElCortijo/Features/Interaction/Pickable/BP_Pickable.Collision` _output_get) false))

(fn `Destroy Viewing Item`
  (`self.K2_DestroyActor` (`self.ResearchableObject`))
  (return))

(fn `Next Item Logic`
  (if (> (`KismetArrayLibrary.Array_Length` (`self.ItemsInCabinet`)) 1)
    (`self.Destroy Viewing Item`)
    (if (== (`self.ViewID`) (- (`KismetArrayLibrary.Array_Length` (`self.ItemsInCabinet`)) 1))
      (set `self.ViewID` 0)
      (else
        (set `self.ViewID` (+ (`self.ViewID`) 1))))
    (`self.Create Viewing Item` (`self.ViewID`))))

(fn `Previous Item Logic`
  (if (> (`KismetArrayLibrary.Array_Length` (`self.ItemsInCabinet`)) 1)
    (`self.Destroy Viewing Item`)
    (if (== (`self.ViewID`) 0)
      (set `self.ViewID` (- (`KismetArrayLibrary.Array_Length` (`self.ItemsInCabinet`)) 1))
      (else
        (set `self.ViewID` (- (`self.ViewID`) 1))))
    (`self.Create Viewing Item` (`self.ViewID`))))

(fn `UserConstructionScript`)