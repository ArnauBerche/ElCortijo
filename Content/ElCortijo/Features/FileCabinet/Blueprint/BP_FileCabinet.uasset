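; BP_FileCabinet is an interactable cabinet that stores the player's held items for later browsing and retrieval.
; Interacting with an item in hand places it hidden at ShowObject and adds it to an array.
; Empty-handed interaction toggles a camera-blended viewing mode via FlipFlop, with Begin/End handling input and blocking interaction during blends.
; WBP_FileCabinet's buttons cycle through items shown singly, or return one to the inventory slot and exit.
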(event `/Game/ElCortijo/Features/Interaction/BPI_Interactable.Interact`
  (params (Interactor :type "Actor Object Reference"))
  (bind _inventory_slot (`self.Inventory Slot`))
  (bind _asbp_first_person_character (cast `/Game/FirstPerson/Blueprints/BP_FirstPersonCharacter` Interactor))
  (set `self.As BP First Person Character` _asbp_first_person_character)
  (bind _asplayer_controller (cast `PlayerController` (`Pawn.GetController` _asbp_first_person_character)))
  (set `self.As Player Controller` _asplayer_controller)
  (set `self.CameraOwner` (`ActorComponent.GetOwner` (`self.Camera`)))
  (if (`self.CanInteract`)
    (bind (_hasobjectinhand _iteminhand) (`self.Check Object InHand` (`self.As BP First Person Character`)))
    (if _hasobjectinhand
      (bind _output_get (set `self.Item in Hand` _iteminhand))
      (`KismetArrayLibrary.Array_Add` (`self.ItemsInCabinet`) _output_get)
      (bind _placedactor (`/Game/ElCortijo/Features/Character/BP_InventoryComponent.Place Actor` _inventory_slot (`SceneComponent.K2_GetComponentToWorld` (`self.ShowObject`))))
      (`self.SetActorHiddenInGame` _placedactor true)
      (`/Game/ElCortijo/Features/Character/BP_InventoryComponent.EmptyInventoryRef` _inventory_slot)
      (else
        (`/Engine/EditorBlueprintResources/StandardMacros.FlipFlop` :!label _label
          (:`A`
            (`Controller.SetIgnoreLookInput` (`self.As Player Controller`) true)
            (`Controller.SetIgnoreMoveInput` (`self.As Player Controller`) true)
            (`PlayerController.SetViewTargetWithBlend` (`self.As Player Controller`) (`self.CameraOwner`) (`self.Blend Time`) "VTBlend_Linear" 0.0 false)
            (set `PlayerController.bShowMouseCursor` true (`self.As Player Controller`))
            (set `self.CanInteract` false)
            (`WidgetBlueprintLibrary.SetInputMode_GameAndUIEx` (`self.As Player Controller`) (`self.WBP_FileCabinet`) "DoNotLock" false)
            (`KismetSystemLibrary.Delay` (`self.Blend Time`))
            (set `self.CanInteract` true)
            (set `self.PlayerInTable` true)
            (bind _returnvalue (`|CreateWidget` "/Game/ElCortijo/Features/FileCabinet/UI/WBP_FileCabinet.WBP_FileCabinet_C" (`self.As Player Controller`)))
            (bind _output_get_2 (set `self.WBP_FileCabinet` _returnvalue))
            (`UserWidget.AddToViewport` _output_get_2 0)
            (set `self.ViewID` 0)
            (add `/Game/ElCortijo/Features/FileCabinet/UI/WBP_FileCabinet.ClickGet` (`self.WBP_FileCabinet`) (delegate `Recive Item`))
            (add `/Game/ElCortijo/Features/FileCabinet/UI/WBP_FileCabinet.ClickLast` (`self.WBP_FileCabinet`) (delegate `Previous Item`))
            (add `/Game/ElCortijo/Features/FileCabinet/UI/WBP_FileCabinet.ClickNext` (`self.WBP_FileCabinet`) (delegate `Next Item`))
            (`self.SetItemView` (`self.ViewID`) true))
          (:`B`
            (`Widget.RemoveFromParent` (`self.WBP_FileCabinet`))
            (`self.SetItemView` (`self.ViewID`))
            (`KismetSystemLibrary.CollectGarbage`)
            (`PlayerController.SetViewTargetWithBlend` (`self.As Player Controller`) (`self.As BP First Person Character`) (`self.Blend Time`) "VTBlend_Linear" 0.0 false)
            (set `self.CanInteract` false)
            (`KismetSystemLibrary.Delay` (`self.Blend Time`))
            (set `self.CanInteract` true)
            (`Controller.SetIgnoreLookInput` (`self.As Player Controller`) false)
            (`Controller.SetIgnoreMoveInput` (`self.As Player Controller`) false)
            (set `PlayerController.bShowMouseCursor` false (`self.As Player Controller`))
            (`WidgetBlueprintLibrary.SetInputMode_GameOnly` (`self.As Player Controller`))
            (set `self.PlayerInTable` false)))))))

(event `Recive Item`
  (`self.Add Object To Hand`)
  (goto _label))

(event `Previous Item`
  (`self.Previous Item Logic`))

(event `Next Item`
  (`self.Next Item Logic`))

(fn `Add Object To Cabinet`)

(fn `Add Object To Hand`
  (bind _viewid (`self.ViewID`))
  (bind _itemsincabinet (`self.ItemsInCabinet`))
  (`/Game/ElCortijo/Features/Character/BP_InventoryComponent.PickUpActor` (`self.Inventory Slot`) (`|GetArrayItem` _itemsincabinet _viewid))
  (`KismetArrayLibrary.Array_Remove` _itemsincabinet _viewid)
  (set `self.ViewID` 0))

(fn `Check Object InHand`
  (params (Interactor :type "/Game/FirstPerson/Blueprints/BP_FirstPersonCharacter Object Reference"))
  (returns (HasObjectInHand :type Boolean) (ItemInHand :type "/Game/ElCortijo/Features/Interaction/Pickable/BP_Pickable Object Reference"))
  (bind _inventoryslot (`/Game/FirstPerson/Blueprints/BP_FirstPersonCharacter.InventorySlot` Interactor))
  ; Check if item can be picked up
  (bind _output_get (set `self.Inventory Slot` _inventoryslot))
  (bind _empty (`/Game/ElCortijo/Features/Character/BP_InventoryComponent.IsEmpty` _output_get))
  (return (not _empty) (`/Game/ElCortijo/Features/Character/BP_InventoryComponent.CurrentItemActor` _inventoryslot)))

(fn `Destroy Viewing Item`
  (`self.K2_DestroyActor` (`self.ResearchableObject`))
  (return))

(fn `Next Item Logic`
  (if (> (`KismetArrayLibrary.Array_Length` (`self.ItemsInCabinet`)) 1)
    (`self.SetItemView` (`self.ViewID`))
    (if (== (`self.ViewID`) (- (`KismetArrayLibrary.Array_Length` (`self.ItemsInCabinet`)) 1))
      (set `self.ViewID` 0)
      (else
        (set `self.ViewID` (+ (`self.ViewID`) 1))))
    (`self.SetItemView` (`self.ViewID`) true)))

(fn `Previous Item Logic`
  (if (> (`KismetArrayLibrary.Array_Length` (`self.ItemsInCabinet`)) 1)
    (`self.SetItemView` (`self.ViewID`))
    (if (== (`self.ViewID`) 0)
      (set `self.ViewID` (- (`KismetArrayLibrary.Array_Length` (`self.ItemsInCabinet`)) 1))
      (else
        (set `self.ViewID` (- (`self.ViewID`) 1))))
    (`self.SetItemView` (`self.ViewID`) true)))

(fn `SetItemView`
  (params (ViewID :type Integer) (Enabled :type Boolean))
  (bind _itemsincabinet (`self.ItemsInCabinet`))
  (bind _output (`|GetArrayItem` _itemsincabinet ViewID))
  (if (< ViewID (`KismetArrayLibrary.Array_Length` _itemsincabinet))
    (`self.SetActorHiddenInGame` _output (not Enabled))
    (bind _output_get (set `self.ResearchableObject` _output))
    (if Enabled
      (`KismetSystemLibrary.PrintString` (`KismetSystemLibrary.GetDisplayName` _output_get)))))

(fn `UserConstructionScript`)