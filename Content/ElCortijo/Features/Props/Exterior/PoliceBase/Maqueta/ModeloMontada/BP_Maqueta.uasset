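; Assembled scale model (maqueta) prop in the police base that shows a building up to a selected floor.
; SetVisibilityByFloor either shows only the ground floor as targetable, or adds the first floor and makes it the only targetable one.
; Per-floor functions propagate visibility from PlantaBaja or PrimeraPlanta and set child primitives' collision.
; Targetability is toggled through the response to custom trace channel GameTraceChannel3.
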(event `self.ReceiveBeginPlay`)

(event `SetVisibilityByFloor`
  (params (Selection :type Integer))
  (switch `int` Selection
    (:`0`
      (`self.SetFloor1Visibility` false)
      (`self.SetFloor0Visibility` true true))
    (:`1`
      (`self.SetFloor1Visibility` true true)
      (`self.SetFloor0Visibility` true))))

(fn `SetFloor0Visibility`
  (params (Visibility :type Boolean) (Targeteable :type Boolean))
  (bind _plantabaja (`self.PlantaBaja`))
  (for _array_element (`SceneComponent.GetChildrenComponents` _plantabaja true)
    (bind _asprimitive_component (cast `PrimitiveComponent` _array_element))
    (if Visibility
      (`PrimitiveComponent.SetCollisionEnabled` _asprimitive_component "QueryAndPhysics")
      (else
        (`PrimitiveComponent.SetCollisionEnabled` _asprimitive_component "NoCollision")))
    (if Targeteable
      (`PrimitiveComponent.SetCollisionResponseToChannel` _asprimitive_component "ECC_GameTraceChannel3" "ECR_Block")
      (else
        (`PrimitiveComponent.SetCollisionResponseToChannel` _asprimitive_component "ECC_GameTraceChannel3" "ECR_Ignore"))))
  (`SceneComponent.SetVisibility` _plantabaja Visibility true))

(fn `SetFloor1Visibility`
  (params (Visibility :type Boolean) (Targetable :type Boolean))
  (bind _primeraplanta (`self.PrimeraPlanta`))
  (for _array_element (`SceneComponent.GetChildrenComponents` _primeraplanta true)
    (bind _asprimitive_component (cast `PrimitiveComponent` _array_element))
    (if Visibility
      (`PrimitiveComponent.SetCollisionEnabled` _asprimitive_component "QueryAndPhysics")
      (else
        (`PrimitiveComponent.SetCollisionEnabled` _asprimitive_component "NoCollision")))
    (if Targetable
      (`PrimitiveComponent.SetCollisionResponseToChannel` _asprimitive_component "ECC_GameTraceChannel3" "ECR_Block")
      (else
        (`PrimitiveComponent.SetCollisionResponseToChannel` _asprimitive_component "ECC_GameTraceChannel3" "ECR_Ignore"))))
  (`SceneComponent.SetVisibility` _primeraplanta Visibility true))

(fn `UserConstructionScript`)