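; Interactable body examination table, usable only when the GameInstance reports HasCamera, extending a parent table class.
; While seated, an input mapping context drives a camera along a spline rail (wrapping on closed loops) with clamped vertical offset, always aimed at a focus point.
; Zoom eases FOV through a timeline.
; Child-actor hotspots activate on entry unless consumed, and left clicks raycast under the cursor to message BPI_Clickable actors.
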(event `self.ReceiveBeginPlay`
  (bind _railspline (`self.RailSpline`))
  (`parent.ReceiveBeginPlay`)
  (`|ExecutionSequence`
    (:`then_0`
      (set `self.TType` "NewEnumerator2")
      (bind _asbp_first_person_character (cast `/Game/ElCortijo/Features/1_MainCharacter/Blueprints/BP_FirstPersonCharacter` (`GameplayStatics.GetPlayerCharacter` 0)))
      (add `/Game/ElCortijo/Features/1_MainCharacter/Blueprints/BP_FirstPersonCharacter.OnLeftClickPress` _asbp_first_person_character (delegate `LeftClickHandler`)))
    (:`then_1`
      (for _array_element (`self.GetAllChildActors` false)
        (bind _asbp_world_element (cast `/Game/ElCortijo/Features/3_InteractableElements/1_IObjects/WorldElements/WorldElement/BP_WorldElement` _array_element))
        (`KismetArrayLibrary.Array_Add` (`self.Hostpots`) _asbp_world_element)
        (`/Game/ElCortijo/Features/3_InteractableElements/1_IObjects/WorldElements/WorldElement/BP_WorldElement.SetActive` _asbp_world_element false)))
    (:`then_2`
      (set `self.SplineLength` (`SplineComponent.GetSplineLength` _railspline))
      (set `self.RailDistance` (`SplineComponent.GetDistanceAlongSplineAtSplineInputKey` _railspline (`SplineComponent.FindInputKeyClosestToWorldLocation` _railspline (`SceneComponent.K2_GetComponentLocation` (`self.Camera`)))))
      (set `self.IsClosedLoop` (`SplineComponent.IsClosedLoop` (`self.RailSpline`)))
      (bind _output_get (set `self.DefaultFOV` (`CameraComponent.FieldOfView` (`self.Camera`))))
      (set `self.CurrentFOV` _output_get))))

(event `LeftClickHandler`
  (`self.LeftClickPress`))

(event `self.ReceiveTick`
  (params (DeltaSeconds :type "Float (single-precision)"))
  (`parent.ReceiveTick` DeltaSeconds)
  (if (`self.PlayerInTable`)
    _))

(event `/Game/ElCortijo/Features/2_InteractionSystem/BPI_Interactable.Interact`
  (params (Interactor :type "Actor Object Reference"))
  (bind _asbp_game_instance (cast `/Game/ElCortijo/Features/0_Unsorted/GameInstance/BP_GameInstance` (`GameplayStatics.GetGameInstance`)))
  (if (`/Game/ElCortijo/Features/0_Unsorted/GameInstance/BP_GameInstance.HasCamera` _asbp_game_instance)
    (`parent.Interact` Interactor)))

(event `self.EnterTable`
  (bind _character (`self.Character`))
  (`parent.EnterTable`)
  (`self.UpdateCameraFromSpline`)
  (`self.EnableHotspots` true)
  (`EnhancedInputSubsystemInterface.AddMappingContext` (pcsubsystem `EnhancedInputLocalPlayerSubsystem` (`self.Controller`)) "/Game/ElCortijo/Features/1_MainCharacter/Input/IMC_BodyTable.IMC_BodyTable" 100 (struct))
  (add `/Game/ElCortijo/Features/1_MainCharacter/Blueprints/BP_FirstPersonCharacter.OnCameraHPress` _character (delegate `CameraH`))
  (add `/Game/ElCortijo/Features/1_MainCharacter/Blueprints/BP_FirstPersonCharacter.OnCameraVPress` _character (delegate `CameraV`))
  (add `/Game/ElCortijo/Features/1_MainCharacter/Blueprints/BP_FirstPersonCharacter.OnCameraZoom` _character (delegate `CameraZoom`)))

(event `CameraH`
  (params (Value :type "Float (double-precision)"))
  (bind _splinelength (`self.SplineLength`))
  (bind _returnvalue (+ (* (* (`self.HorizontalSpeed`) Value) (`GameplayStatics.GetWorldDeltaSeconds`)) (`self.RailDistance`)))
  (bind _remainder (`KismetMathLibrary.FMod` _returnvalue _splinelength))
  (if (`self.IsClosedLoop`)
    (if (< _remainder 0.0)
      (set `self.RailDistance` (+ _remainder (`self.SplineLength`)))
      (else
        (set `self.RailDistance` _remainder)))
    (else
      (set `self.RailDistance` (`KismetMathLibrary.FClamp` _returnvalue 0.0 _splinelength))))
  (`self.UpdateCameraFromSpline`))

(event `CameraV`
  (params (Value :type "Float (double-precision)"))
  (set `self.VerticalOffset` (`KismetMathLibrary.FClamp` (+ (* (* (`self.VerticalSpeed`) Value) (`GameplayStatics.GetWorldDeltaSeconds`)) (`self.VerticalOffset`)) (`self.MinVerOffset`) (`self.MaxVerOffset`)))
  (`self.UpdateCameraFromSpline`))

(event `self.ExitTable`
  (bind _character (`self.Character`))
  (`self.EnableHotspots` false)
  (`parent.ExitTable`)
  (`EnhancedInputSubsystemInterface.RemoveMappingContext` (pcsubsystem `EnhancedInputLocalPlayerSubsystem` (`self.Controller`)) "/Game/ElCortijo/Features/1_MainCharacter/Input/IMC_BodyTable.IMC_BodyTable" (struct))
  (clear `/Game/ElCortijo/Features/1_MainCharacter/Blueprints/BP_FirstPersonCharacter.OnCameraHPress` _character)
  (clear `/Game/ElCortijo/Features/1_MainCharacter/Blueprints/BP_FirstPersonCharacter.OnCameraVPress` _character)
  (bind _output_get (set `self.CurrentFOV` (`self.DefaultFOV`)))
  (`CameraComponent.SetFieldOfView` (`self.Camera`) _output_get))

(event `CameraZoom`
  (params (Value :type "Float (double-precision)"))
  (bind _currentfov (`self.CurrentFOV`))
  (bind _output_get (set `self.LerpStartFOV` _currentfov))
  (bind _output_get_2 (set `self.LerpTargetFOV` (`KismetMathLibrary.FClamp` (+ _currentfov (* (`KismetMathLibrary.SignOfFloat` Value) (`self.ZoomStep`))) (`self.FOVMin`) (`self.FOVMax`))))
  (bind (_direction _zoom) (`Timeline|Zoom` :!via `PlayFromStart`)
    (:`Update`
      (bind _output_get_3 (set `self.CurrentFOV` (`KismetMathLibrary.Lerp` _output_get _output_get_2 _zoom)))
      (`CameraComponent.SetFieldOfView` (`self.Camera`) _output_get_3))))

(fn `EnableHotspots`
  (params (Enable :type Boolean))
  (for _array_element (`self.Hostpots`)
    (if (not (`/Game/ElCortijo/Features/3_InteractableElements/1_IObjects/WorldElements/WorldElement/BP_WorldElement.Consumed` _array_element))
      (`/Game/ElCortijo/Features/3_InteractableElements/1_IObjects/WorldElements/WorldElement/BP_WorldElement.SetActive` _array_element Enable))))

(fn `LeftClickPress`
  (bind (_bblockinghit _binitialoverlap _time _distance _location _impactpoint _normal _impactnormal _physmat _hitactor) (`GameplayStatics.BreakHitResult` (`PlayerController.GetHitResultUnderCursorByChannel` (`self.Controller`) "TraceTypeQuery5" true)))
  (if (`self.PlayerInTable`)
    (if (`KismetSystemLibrary.DoesImplementInterface` _hitactor "/Game/ElCortijo/Features/2_InteractionSystem/BPI_Clickable.BPI_Clickable_C")
      (message `/Game/ElCortijo/Features/2_InteractionSystem/BPI_Clickable.Click` _hitactor null))))

(fn `UpdateCameraFromSpline`
  (locals (`Final Location` :type "Vector Structure"))
  (bind _output_get (set `local.Final Location` (+ (`SplineComponent.GetLocationAtDistanceAlongSpline` (`self.RailSpline`) (`self.RailDistance`) "World") (* (`self.VerticalOffset`) (`SceneComponent.GetUpVector` (`self.FocusPoint`))))))
  (`SceneComponent.K2_SetWorldLocationAndRotation` (`self.Camera`) (`local.Final Location`) (`KismetMathLibrary.FindLookAtRotation` _output_get (`SceneComponent.K2_GetComponentLocation` (`self.FocusPoint`))) false false))

(fn `UserConstructionScript`
  (`parent.UserConstructionScript`))