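; Research table where the player examines the clue item held in their inventory, shown through a SceneCapture show-only list and separate lighting channel, then returns it on exit.
; Right-click snaps the item to its nearest face via timeline; a short press flips it, while holding applies Tick-driven, clamped, eased drag tilt.
; Left-click traces under the cursor to BPI_Clickable actors.
; Evidence actors spawn into placement slots gathered from ProofPlacement's children.
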(event `OnRightClickPressed_Handler`
  (bind _resettargetrot (`self.ResetTargetRot`))
  (bind (_locationx _locationy) (`PlayerController.GetMousePosition` (`GameplayStatics.GetPlayerController` 0)))
  (if (and (`self.PlayerInTable`) (!= (`self.ResearchableObject`) null))
    (if (and (`self.bIsSnaped`) (not (`self.bPlayingFlip`)))
      (set `self.bIsPressed` true)
      (set `self.bIsSnaped` false)
      (set `self.PressTime` (`KismetSystemLibrary.GetGameTimeInSeconds`))
      (set `self.StartMousePos` (`KismetMathLibrary.MakeVector2D` _locationx _locationy))
      (`self.SnapToNearestCanonicalRotation`)
      (bind (_direction _newtrack_0) (`Timeline|TL_ResetRotation` :!via `PlayFromStart`)
        (:`Update`
          (`self.K2_SetActorRotation` (`self.ResearchableObject`) (`KismetMathLibrary.RLerp` (`self.ResetStartRot`) _resettargetrot _newtrack_0 true) false)
          (set `self.bIsSnaped` false))
        (:`Finished`
          (set `self.bIsSnaped` true)
          (set `self.CurrentRot` _resettargetrot)
          (set `self.HoldStartLocalRotation` _resettargetrot)
          (set `self.CurrentOffsetPitch` 0.0)
          (set `self.CurrentOffsetRoll` 0.0)
          (if (`self.ShoudFlip`)
            (`self.StartFlip`)))))))

(event `OnRightClickHoldRelease_Handler`
  (if (and (`self.PlayerInTable`) (!= (`self.ResearchableObject`) null))
    (if (`self.bIsPressed`)
      (set `self.bIsPressed` false)
      (if (<= (- (`KismetSystemLibrary.GetGameTimeInSeconds`) (`self.PressTime`)) (`self.ShortPressThreshold`))
        (set `self.ShoudFlip` true)
        (else
          (set `self.ShoudFlip` false)
          (if (`self.bIsHolding`)
            (`self.EndHold`)))))))

(event `OnStartResearch`
  (params (PlayerRef :type "/Game/ElCortijo/Features/1_MainCharacter/Blueprints/BP_FirstPersonCharacter Object Reference"))
  (`parent.Interact` PlayerRef))

(event `self.ReceiveBeginPlay`
  (set `self.TType` "NewEnumerator0")
  (bind _asbp_first_person_character (cast `/Game/ElCortijo/Features/1_MainCharacter/Blueprints/BP_FirstPersonCharacter` (`GameplayStatics.GetPlayerCharacter` 0)))
  (`|ExecutionSequence`
    (:`then_0`
      (for _array_element (`SceneComponent.GetChildrenComponents` (`self.ProofPlacement`) true)
        (bind _asstatic_mesh_component (cast `StaticMeshComponent` _array_element))
        (`KismetArrayLibrary.Array_Add` (`self.HintPlacementsRef`) (make `/Game/ElCortijo/Features/4_InteratableTables/S_TablePlacements` _asstatic_mesh_component null))
        (`KismetSystemLibrary.PrintText` "Added")))
    (:`then_1`
      (add `/Game/ElCortijo/Features/1_MainCharacter/Blueprints/BP_FirstPersonCharacter.OnLeftClickPress` _asbp_first_person_character (delegate `OnLeftClick_Handler`)))))

(event `OnLeftClick_Handler`
  (`self.LeftClickPress`)
  (add `/Game/ElCortijo/Features/1_MainCharacter/Blueprints/BP_FirstPersonCharacter.OnRightClickPress` (stale `self.ReceiveBeginPlay` _asbp_first_person_character) (delegate `OnRightClickPressed_Handler`))
  (add `/Game/ElCortijo/Features/1_MainCharacter/Blueprints/BP_FirstPersonCharacter.OnRightClickRelease` (stale `self.ReceiveBeginPlay` _asbp_first_person_character) (delegate `OnRightClickHoldRelease_Handler`))
  (add `/Game/ElCortijo/Features/1_MainCharacter/Blueprints/BP_FirstPersonCharacter.OnResearchPress` (stale `self.ReceiveBeginPlay` _asbp_first_person_character) (delegate `OnStartResearch`)))

(event `self.EnterTable`
  (bind _output_get (set `self.Inventory Slot` (`/Game/ElCortijo/Features/1_MainCharacter/Blueprints/BP_FirstPersonCharacter.InventorySlot` (`self.Character`))))
  (bind _empty (`/Game/ElCortijo/Features/1_MainCharacter/BP_InventoryComponent.IsEmpty` _output_get))
  (if (not _empty)
    (`parent.EnterTable`)
    (`self.CreateResearchableObject` _output_get)
    (bind _returnvalue (`|CreateWidget` "/Game/ElCortijo/Features/4_InteratableTables/ResearchTable/UI/WBP_ResearchTable.WBP_ResearchTable_C"))
    (bind _output_get_2 (set `self.UIResearchTable` _returnvalue))
    (`UserWidget.AddToViewport` _output_get_2 0)))

(event `self.ExitTable`
  (`self.DestroyReserchableObject` (`self.Character`))
  (`self.DestroyReserchableObject` (`self.Character`))
  (`Widget.RemoveFromParent` (`self.UIResearchTable`))
  (`KismetSystemLibrary.CollectGarbage`)
  (`parent.ExitTable`))

(event `self.ReceiveTick`
  (params (DeltaSeconds :type "Float (single-precision)"))
  (`|ExecutionSequence`
    (:`then_0`
      (if (and (and (`self.PlayerInTable`) (!= (`self.ResearchableObject`) null)) (`self.bIsSnaped`))
        (if (`self.bPlayingFlip`)
          (`self.TickFlip` DeltaSeconds)
          (elif (and (`self.bIsPressed`) (not (`self.bIsHolding`)))
            (if (>= (- (`KismetSystemLibrary.GetGameTimeInSeconds`) (`self.PressTime`)) (`self.ShortPressThreshold`))
              (`self.StartHold`))
            (elif (`self.bIsHolding`)
              (`self.TickHold` DeltaSeconds))))))))

(fn `CreateEvidence`
  (params (Evidence :type "/Game/ElCortijo/Features/3_InteractableElements/1_IObjects/Evidence/BP_Evidence Class Reference"))
  (bind _slot (`self.GetFirstEmptySlot`))
  (bind (_placement _evidence) (break `/Game/ElCortijo/Features/4_InteratableTables/S_TablePlacements` (`|GetArrayItem` (`self.HintPlacementsRef`) _slot)))
  (bind _returnvalue (`|SpawnActorFromClass` Evidence (`KismetMathLibrary.MakeTransform` (`SceneComponent.K2_GetComponentLocation` _placement) (`SceneComponent.K2_GetComponentRotation` _placement)) "AlwaysSpawn" "MultiplyWithRoot" (`ActorComponent.GetOwner` (`self.Camera`)) true self _slot false null))
  (`|VariableSetRef` _evidence _returnvalue)
  (`/Game/ElCortijo/Features/2_InteractionSystem/Pickable/BP_Pickable.SetPhysics` _returnvalue true)
  (`/Game/ElCortijo/Features/2_InteractionSystem/Pickable/BP_Pickable.SetInteractable` _returnvalue true))

(fn `CreateResearchableObject`
  (params (InventSlot :type "/Game/ElCortijo/Features/1_MainCharacter/BP_InventoryComponent Object Reference"))
  (bind _output_get (set `self.Inventory Slot` InventSlot))
  (bind _asbp_clue_item (cast `/Game/ElCortijo/Features/3_InteractableElements/1_IObjects/Clues/ClueHotspot/BP_ClueItem` (`/Game/ElCortijo/Features/1_MainCharacter/BP_InventoryComponent.CurrentItemActor` _output_get)))
  (bind (_smc_ci _collision_ci) (`/Game/ElCortijo/Features/3_InteractableElements/1_IObjects/Clues/ClueHotspot/BP_ClueItem.OnPlacedOnTable` _asbp_clue_item self))
  (set `self.SMC_CI` _smc_ci)
  (set `self.Collision CI` _collision_ci)
  (set `self.ResearchableObject` _asbp_clue_item)
  (`/Game/ElCortijo/Features/1_MainCharacter/BP_InventoryComponent.EmptyInventoryRef` _output_get)
  (`self.ResetRotationValues`)
  (`SceneCaptureComponent.ClearShowOnlyComponents` (`self.SceneCaptureComponent2D`))
  (for _array_element (`self.SMC_CI`)
    (bind _asstatic_mesh_component (cast `StaticMeshComponent` _array_element))
    (`PrimitiveComponent.SetVisibleInSceneCaptureOnly` _asstatic_mesh_component true)
    (`SceneCaptureComponent.ShowOnlyComponent` (`self.SceneCaptureComponent2D`) _asstatic_mesh_component)
    (`PrimitiveComponent.SetLightingChannels` _asstatic_mesh_component false true false))
  (`PrimitiveComponent.SetCollisionEnabled` (`self.Collision CI`) "NoCollision")
  (return))

(fn `DestroyReserchableObject`
  (params (Interactor :type "/Game/ElCortijo/Features/1_MainCharacter/Blueprints/BP_FirstPersonCharacter Object Reference"))
  (bind _researchableobject (`self.ResearchableObject`))
  (if (!= _researchableobject null)
    (`/Game/ElCortijo/Features/3_InteractableElements/1_IObjects/Clues/ClueHotspot/BP_ClueItem.SetAllHotspotsActive` _researchableobject false)
    (`/Game/ElCortijo/Features/1_MainCharacter/BP_InventoryComponent.PickUpActor` (`/Game/ElCortijo/Features/1_MainCharacter/Blueprints/BP_FirstPersonCharacter.InventorySlot` Interactor) _researchableobject)
    (for _array_element (`self.SMC_CI`)
      (bind _asstatic_mesh_component (cast `StaticMeshComponent` _array_element))
      (`PrimitiveComponent.SetVisibleInSceneCaptureOnly` _asstatic_mesh_component false)
      (`PrimitiveComponent.SetLightingChannels` _asstatic_mesh_component true false false))
    (`SceneCaptureComponent.ClearShowOnlyComponents` (`self.SceneCaptureComponent2D`))
    (`PrimitiveComponent.SetCollisionEnabled` (`self.Collision CI`) "QueryAndPhysics")
    (`KismetArrayLibrary.Array_Clear` (`self.SMC_CI`))
    (set `self.Collision CI` null)
    (set `self.ResearchableObject` null)
    (return)))

(fn `EndHold`
  (set `self.bIsHolding` false))

(fn `GetFirstEmptySlot`
  (returns (Slot :type Integer) (IsRoom :type Boolean))
  (locals (TempSlot :type Integer) (TempIsRoom :type Boolean))
  (set `local.TempIsRoom` false)
  (for (_array_element _array_index) (`self.HintPlacementsRef`)
    (if (== (`.Evidence_7_18C52045475546F6D7C545884F8868D5` (break `/Game/ElCortijo/Features/4_InteratableTables/S_TablePlacements` _array_element)) null)
      (set `local.TempIsRoom` true)
      (set `local.TempSlot` _array_index)
      (break)))
  (return (`local.TempSlot`) (`local.TempIsRoom`)))

(fn `LeftClickPress`
  (bind (_bblockinghit _binitialoverlap _time _distance _location _impactpoint _normal _impactnormal _physmat _hitactor) (`GameplayStatics.BreakHitResult` (`PlayerController.GetHitResultUnderCursorByChannel` (`GameplayStatics.GetPlayerController` 0) "TraceTypeQuery5" true)))
  (if (!= (`self.ResearchableObject`) null)
    (if (`self.PlayerInTable`)
      (if (`KismetSystemLibrary.DoesImplementInterface` _hitactor "/Game/ElCortijo/Features/2_InteractionSystem/BPI_Clickable.BPI_Clickable_C")
        (message `/Game/ElCortijo/Features/2_InteractionSystem/BPI_Clickable.Click` _hitactor null)))))

(fn `RemoveEvidence`
  (params (SlotIndex :type Integer))
  (bind _output (`|GetArrayItem` (`self.HintPlacementsRef`) SlotIndex))
  (`|VariableSetRef` _output (make `/Game/ElCortijo/Features/4_InteratableTables/S_TablePlacements` (`.Placement_2_FD44286F48BEEE48D0811A9809672CC7` (break `/Game/ElCortijo/Features/4_InteratableTables/S_TablePlacements` _output)) null)))

(fn `ResetRotationValues`
  (set `self.bIsPressed` false)
  (set `self.bIsHolding` false)
  (set `self.bPlayingFlip` false)
  (set `self.StartMousePos` (0.0 0.0))
  (set `self.PressTime` 0.0)
  (set `self.HoldStartLocalRotation` (struct))
  (set `self.CurrentOffsetPitch` 0.0)
  (set `self.CurrentOffsetRoll` 0.0)
  (set `self.FlipElapsed` 0.0)
  (set `self.FlipStartRot` (struct))
  (set `self.FlipTargetRot` (struct))
  (set `self.BaseLocalRotation` (struct))
  (set `self.FlipLocalRotation` (struct))
  (set `self.bIsSnaped` true)
  (set `self.ResetStartRot` (struct))
  (set `self.ResetTargetRot` (struct))
  (set `self.bIsFliped` false)
  (set `self.ShoudFlip` false))

(fn `SnapToNearestCanonicalRotation`
  (locals (FlipDelta :type "Rotator Structure" :default (struct)) (DeltaBase :type "Rotator Structure" :default (struct)) (FlipBase :type "Rotator Structure" :default (struct)) (DistToBase :type "Float (double-precision)") (DistToFlip :type "Float (double-precision)"))
  (bind _returnvalue (`self.K2_GetActorRotation` self))
  (if (`KismetSystemLibrary.IsValid` (`self.ResearchableObject`))
    (set `self.BaseLocalRotation` _returnvalue)
    (set `self.CurrentRot` (`self.K2_GetActorRotation` (`self.ResearchableObject`)))
    (set `self.FlipLocalRotation` (`KismetMathLibrary.MakeRotator` (+ (.roll _returnvalue) 180.0) (.pitch _returnvalue) (.yaw _returnvalue)))
    (bind _output_get (set `local.DeltaBase` (`KismetMathLibrary.ComposeRotators` (`self.CurrentRot`) (`KismetMathLibrary.NegateRotator` (`self.BaseLocalRotation`)))))
    (set `local.DistToBase` (+ (+ (`KismetMathLibrary.Abs` (.roll _output_get)) (`KismetMathLibrary.Abs` (.pitch _output_get))) (`KismetMathLibrary.Abs` (.yaw _output_get))))
    (bind _output_get_2 (set `local.FlipBase` (`KismetMathLibrary.ComposeRotators` (`self.CurrentRot`) (`KismetMathLibrary.NegateRotator` (`self.FlipLocalRotation`)))))
    (set `local.DistToFlip` (+ (+ (`KismetMathLibrary.Abs` (.roll _output_get_2)) (`KismetMathLibrary.Abs` (.pitch _output_get_2))) (`KismetMathLibrary.Abs` (.yaw _output_get_2))))
    (set `self.ResetStartRot` (`self.CurrentRot`))
    (if (<= (`local.DistToBase`) (`local.DistToFlip`))
      (set `self.ResetTargetRot` (`self.BaseLocalRotation`))
      (else
        (set `self.ResetTargetRot` (`self.FlipLocalRotation`))))))

(fn `StartFlip`
  (if (not (`self.bPlayingFlip`))
    (set `self.bPlayingFlip` true)
    (set `self.FlipElapsed` 0.0)
    (if (`self.bIsFliped`)
      (set `self.FlipTargetRot` (`self.BaseLocalRotation`))
      (else
        (bind _output_get (set `self.FlipTargetRot` (`self.FlipLocalRotation`)))))
    (`KismetSystemLibrary.PrintString` (`KismetStringLibrary.Conv_RotatorToString` _output_get))))

(fn `StartHold`
  (set `self.bIsHolding` true))

(fn `TickFlip`
  (params (DeltaSeconds :type "Float (double-precision)"))
  (locals (Alpha :type "Float (double-precision)"))
  (bind _researchableobject (`self.ResearchableObject`))
  (bind _flipelapsed (`self.FlipElapsed`))
  (set `self.ShoudFlip` false)
  (set `self.bPlayingFlip` true)
  (set `self.FlipElapsed` (+ DeltaSeconds _flipelapsed))
  (set `local.Alpha` (/ _flipelapsed (`self.FlipDuration`)))
  (`self.K2_SetActorRotation` _researchableobject (`KismetMathLibrary.RLerp` (`self.CurrentRot`) (`self.FlipTargetRot`) (`local.Alpha`)) false)
  (if (< (`self.FlipDuration`) (`self.FlipElapsed`))
    (`self.K2_SetActorRotation` _researchableobject (`self.FlipTargetRot`) false)
    (set `self.bPlayingFlip` false)
    (set `self.bIsFliped` (not (`self.bIsFliped`)))))

(fn `TickHold`
  (params (DelataSeconds :type "Float (double-precision)"))
  (locals (Drag :type "Vector2D Structure") (Dist :type "Float (double-precision)" :default 0.0) (DistNorm :type "Float (double-precision)" :default 0.0) (SpeedScale :type "Float (double-precision)") (RawDesiredRoll :type "Float (double-precision)") (RawDesiredPitch :type "Float (double-precision)") (DesiredRollOffset :type "Float (double-precision)" :default 0.0) (DesiredPitchOffset :type "Float (double-precision)" :default 0.0) (DeltaSeconds :type "Float (double-precision)"))
  (bind _maxangle (`self.MaxAngle`))
  (bind _maxangle_2 (`self.MaxAngle`))
  (bind (_locationx _locationy _returnvalue) (`PlayerController.GetMousePosition` (`GameplayStatics.GetPlayerController` 0)))
  (bind (_x _y) (`KismetMathLibrary.BreakVector2D` (`local.Drag`)))
  (set `local.DeltaSeconds` DelataSeconds)
  (if _returnvalue
    (set `local.Drag` (- (`KismetMathLibrary.MakeVector2D` _locationx _locationy) (`self.StartMousePos`)))
    (set `local.Dist` (`KismetMathLibrary.VSize2D` (`local.Drag`)))
    (set `local.DistNorm` (`KismetMathLibrary.FClamp` (/ (`local.Dist`) (`self.MaxDragDistance`))))
    (set `local.SpeedScale` (- 1.0 (`local.DistNorm`)))
    (set `local.RawDesiredRoll` (* (* _x (`self.BaseRotateSpeed`)) (`local.SpeedScale`)))
    (set `local.RawDesiredPitch` (* (* _y (`self.BaseRotateSpeed`)) (`local.SpeedScale`)))
    (set `local.DesiredRollOffset` (`KismetMathLibrary.FClamp` (`local.RawDesiredRoll`) (* _maxangle_2 -1.0) _maxangle_2))
    (set `local.DesiredPitchOffset` (`KismetMathLibrary.FClamp` (`local.RawDesiredPitch`) (* _maxangle -1.0) _maxangle))
    (set `self.CurrentOffsetRoll` (`KismetMathLibrary.FInterpTo` (`self.CurrentOffsetRoll`) (`local.DesiredRollOffset`) (`local.DeltaSeconds`) 12.0))
    (set `self.CurrentOffsetPitch` (`KismetMathLibrary.FInterpTo` (`self.CurrentOffsetPitch`) (`local.DesiredPitchOffset`) (`local.DeltaSeconds`) 12.0))
    (`self.K2_SetActorRotation` (`self.ResearchableObject`) (`KismetMathLibrary.MakeRotator` (+ (.roll (`self.HoldStartLocalRotation`)) (`self.CurrentOffsetRoll`)) (+ (.pitch (`self.HoldStartLocalRotation`)) (`self.CurrentOffsetPitch`)) (.yaw (`self.HoldStartLocalRotation`))) false)))

(fn `UserConstructionScript`)