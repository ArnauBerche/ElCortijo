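; Interactable model board table where the player arranges evidence on a cell grid, with correct placements driving mission progress.
; Evidence in hand moves to a free side slot on entering; cursor traces handle right-click dragging and left-click descriptions in WBP_ModelBoard.
; Grid helpers map positions to cells and compare contents with each cell's expected class.
; Tick watches the correct count to ring the phone, update missions and spawn photo evidence.
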(event `self.ReceiveBeginPlay`
  (bind (_gridsize_x _gridsize_y) (`KismetMathLibrary.BreakVector2D` (`self.GridSize`)))
  (`|ExecutionSequence`
    (:`then_0`
      (set `self.TType` "NewEnumerator1"))
    (:`then_1`
      (`self.Generate Cell Grid` (`KismetMathLibrary.FTrunc` _gridsize_x) (`KismetMathLibrary.FTrunc` _gridsize_y)))
    (:`then_2`
      (for _array_element (`SceneComponent.GetChildrenComponents` (`self.EvidenceRelativeSlots`) true)
        (bind _asstatic_mesh_component (cast `StaticMeshComponent` _array_element))
        (`KismetArrayLibrary.Array_Add` (`self.HintPlacementsRef`) (make `/Game/ElCortijo/Features/4_InteratableTables/S_TablePlacements` _asstatic_mesh_component null))))
    (:`then_3`
      (bind _asbp_first_person_character (cast `/Game/ElCortijo/Features/1_MainCharacter/Blueprints/BP_FirstPersonCharacter` (`GameplayStatics.GetPlayerCharacter` 0)))
      (`|ExecutionSequence`
        (:`then_0`
          (add `/Game/ElCortijo/Features/1_MainCharacter/Blueprints/BP_FirstPersonCharacter.OnLeftClickPress` _asbp_first_person_character (delegate `OnLeftClickPress_Handler`)))
        (:`then_1`
          (add `/Game/ElCortijo/Features/1_MainCharacter/Blueprints/BP_FirstPersonCharacter.OnLeftClickRelease` _asbp_first_person_character (delegate `OnLeftClickRelease_Handler`)))
        (:`then_2`
          (add `/Game/ElCortijo/Features/1_MainCharacter/Blueprints/BP_FirstPersonCharacter.OnRightClickPress` _asbp_first_person_character (delegate `OnRightClickPress_Handler`)))
        (:`then_3`
          (add `/Game/ElCortijo/Features/1_MainCharacter/Blueprints/BP_FirstPersonCharacter.OnRightClickRelease` _asbp_first_person_character (delegate `OnRightClickRelease_Handler`)))))
    (:`then_4`
      (bind _returnvalue (`|CreateWidget` "/Game/ElCortijo/Features/4_InteratableTables/ModelBoard/UI/WBP_ModelBoard.WBP_ModelBoard_C" (`self.Controller`) self))
      (set `self.WBP_ModelBoard` _returnvalue))))

(event `OnLeftClickPress_Handler`
  (`self.LeftClickPressed`))

(event `OnLeftClickRelease_Handler`)

(event `OnRightClickPress_Handler`
  (`self.RightClickPress`))

(event `OnRightClickRelease_Handler`
  (`self.RightClickRelease`))

(event `/Game/ElCortijo/Features/2_InteractionSystem/BPI_Interactable.Interact`
  (params (Interactor :type "Actor Object Reference"))
  (`parent.Interact` Interactor))

(event `self.EnterTable`
  (bind _wbp_modelboard (`self.WBP_ModelBoard`))
  (bind (_hasobjectinhand _iteminhand) (`self.Check Object InHand` (`self.Character`)))
  (if _hasobjectinhand
    (bind _asbp_evidence (cast `/Game/ElCortijo/Features/3_InteractableElements/1_IObjects/Evidence/BP_Evidence` _iteminhand))
    (`self.CreateEvidence` _asbp_evidence))
  (`UserWidget.AddToViewport` _wbp_modelboard 0)
  (bind _asbp_game_instance (cast `/Game/ElCortijo/Features/0_Unsorted/GameInstance/BP_GameInstance` (`GameplayStatics.GetGameInstance`)))
  (set `self.GI_Ref` _asbp_game_instance)
  (`/Game/ElCortijo/Features/4_InteratableTables/ModelBoard/UI/WBP_ModelBoard.OnNotesUpdated_Handler_L` _wbp_modelboard)
  (`/Game/ElCortijo/Features/4_InteratableTables/ModelBoard/UI/WBP_ModelBoard.OnNotesUpdated_Handler_R` _wbp_modelboard)
  (`parent.EnterTable`))

(event `self.ExitTable`
  (`Widget.RemoveFromParent` (`self.WBP_ModelBoard`))
  (`parent.ExitTable`))

(event `self.ReceiveTick`
  (params (DeltaSeconds :type "Float (single-precision)"))
  (bind _correctplacementsamount (`self.CorrectPlacementsAmount`))
  (bind _missionshandled (`self.MissionsHandled`))
  (if (`self.PlayerInTable`)
    (if (== _missionshandled 0)
      (if (>= (`self.CorrectPlacementsAmount`) 2)
        (bind _returnvalue (`GameplayStatics.GetActorOfClass` "/Game/ElCortijo/Features/3_InteractableElements/2_IAsset/BP_Phone.BP_Phone_C"))
        (`/Game/ElCortijo/Features/3_InteractableElements/2_IAsset/BP_Phone.RingPhone` _returnvalue)
        (bind _asbp_game_instance (cast `/Game/ElCortijo/Features/0_Unsorted/GameInstance/BP_GameInstance` (`GameplayStatics.GetGameInstance`)))
        (`/Game/ElCortijo/Features/5_MissionSystem/BP_MissionManager.CompleteMission` (`/Game/ElCortijo/Features/0_Unsorted/GameInstance/BP_GameInstance.MissionManager` _asbp_game_instance) "Pruebas2" true)
        (set `self.MissionsHandled` 1))
      (elif (== _missionshandled 1)
        (if (>= _correctplacementsamount 3)
          (bind _asbp_game_instance_2 (cast `/Game/ElCortijo/Features/0_Unsorted/GameInstance/BP_GameInstance` (`GameplayStatics.GetGameInstance`)))
          (`/Game/ElCortijo/Features/5_MissionSystem/BP_MissionManager.AdvanceMission` (`/Game/ElCortijo/Features/0_Unsorted/GameInstance/BP_GameInstance.MissionManager` _asbp_game_instance_2) "Pruebas3" true)
          (bind _returnvalue_2 (`GameplayStatics.GetActorOfClass` "/Game/ElCortijo/Features/3_InteractableElements/2_IAsset/Spawner/BP_Spawner.BP_Spawner_C"))
          (`/Game/ElCortijo/Features/3_InteractableElements/2_IAsset/Spawner/BP_Spawner.SpawnItem` _returnvalue_2 "/Game/ElCortijo/Features/3_InteractableElements/1_IObjects/Clues/Caso1_Proto/BP_C_FotoTelefono.BP_C_FotoTelefono_C" (0.0 -10.0 0.0))
          (`/Game/ElCortijo/Features/3_InteractableElements/2_IAsset/Spawner/BP_Spawner.SpawnItem` _returnvalue_2 "/Game/ElCortijo/Features/3_InteractableElements/1_IObjects/Clues/Caso1_Proto/BP_C_FotoArañazos.BP_C_FotoArañazos_C" (0.0 10.0 0.0))
          (`/Game/ElCortijo/Features/7_AudioSystem/Blueprint/BP_SoundComponent.Play` (`/Game/ElCortijo/Features/3_InteractableElements/2_IAsset/Spawner/BP_Spawner.BP_SoundComponent` _returnvalue_2))
          (set `self.MissionsHandled` 2))
        (elif (== _missionshandled 2)
          (if (>= _correctplacementsamount 4)
            (bind _returnvalue_3 (`GameplayStatics.GetActorOfClass` "/Game/ElCortijo/Features/3_InteractableElements/2_IAsset/BP_Phone.BP_Phone_C"))
            (`/Game/ElCortijo/Features/3_InteractableElements/2_IAsset/BP_Phone.RingPhone` _returnvalue_3)))))))

(fn `Add ObjectToGrid`
  (params (Cell :type "Vector2D Structure") (Object :type "/Game/ElCortijo/Features/3_InteractableElements/1_IObjects/Evidence/Evidences/BP_ObjectEvidence Object Reference"))
  (locals (VIndex :type Integer))
  (bind _grid (`self.Grid`))
  (bind _gridsize_x (`KismetMathLibrary.BreakVector2D` (`self.GridSize`)))
  (bind _output_get (set `local.VIndex` (`KismetMathLibrary.FTrunc` (+ Cell_X (* (- Cell_Y 1.0) _gridsize_x)))))
  (bind _returnvalue (- _output_get 1))
  (bind (_output_posinarray _output_contains _output_correctcontainer _output_isvalid) (break `/Game/ElCortijo/Features/4_InteratableTables/ModelBoard/Blueprint/S_Cell` (`|GetArrayItem` _grid _returnvalue)))
  (bind _s_cell (make `/Game/ElCortijo/Features/4_InteratableTables/ModelBoard/Blueprint/S_Cell` (`KismetMathLibrary.MakeVector2D` Cell_X Cell_Y) Object _output_correctcontainer _output_isvalid))
  (`KismetArrayLibrary.Array_Set` _grid _returnvalue _s_cell)
  (bind _iscorrect (`self.CheckCorrectContains` _s_cell))
  (set `/Game/ElCortijo/Features/3_InteractableElements/1_IObjects/Evidence/Evidences/BP_ObjectEvidence.IsOnCorrectPlace` _iscorrect Object)
  (`self.UpdateCorrectPlacements`)
  (return))

(fn `BajarPiso`)

(fn `CellHasObject`
  (params (Cell :type "Vector2D Structure") (BP_Evidence :type "/Game/ElCortijo/Features/3_InteractableElements/1_IObjects/Evidence/BP_Evidence Object Reference"))
  (returns (HasSelf :type Boolean))
  (locals (VIndex :type Integer))
  (bind _gridsize_x (`KismetMathLibrary.BreakVector2D` (`self.GridSize`)))
  (bind _output_get (set `local.VIndex` (`KismetMathLibrary.FTrunc` (+ Cell_X (* (- Cell_Y 1.0) _gridsize_x)))))
  (bind (_output_posinarray _output_contains) (break `/Game/ElCortijo/Features/4_InteratableTables/ModelBoard/Blueprint/S_Cell` (`|GetArrayItem` (`self.Grid`) (- _output_get 1))))
  (return (== _output_contains BP_Evidence)))

(fn `Check Object InHand`
  (params (Interactor :type "/Game/ElCortijo/Features/1_MainCharacter/Blueprints/BP_FirstPersonCharacter Object Reference"))
  (returns (HasObjectInHand :type Boolean) (ItemInHand :type "/Game/ElCortijo/Features/2_InteractionSystem/Pickable/BP_Pickable Object Reference"))
  (bind _inventoryslot (`/Game/ElCortijo/Features/1_MainCharacter/Blueprints/BP_FirstPersonCharacter.InventorySlot` Interactor))
  (bind _output_get (set `self.Inventory Slot` _inventoryslot))
  (bind _empty (`/Game/ElCortijo/Features/1_MainCharacter/BP_InventoryComponent.IsEmpty` _output_get))
  (return (not _empty) (`/Game/ElCortijo/Features/1_MainCharacter/BP_InventoryComponent.CurrentItemActor` _inventoryslot)))

(fn `CheckCorrectContains`
  (params (Cell :type "/Game/ElCortijo/Features/4_InteratableTables/ModelBoard/Blueprint/S_Cell Structure"))
  (returns (IsCorrect :type Boolean))
  (return (== (`GameplayStatics.GetObjectClass` Cell_Contains_11_B344A4CA41F4978793DCCB8186FD342E) Cell_CorrectContainer_15_E16AA9D2474B63CDD6C68D8409073F82)))

(fn `CreateEvidence`
  (params (Object :type "/Game/ElCortijo/Features/3_InteractableElements/1_IObjects/Evidence/BP_Evidence Object Reference"))
  (`self.CreateEvidenceObject` Object)
  (`/Game/ElCortijo/Features/1_MainCharacter/BP_InventoryComponent.EmptyInventoryRef` (`self.Inventory Slot`))
  (`/Game/ElCortijo/Features/7_AudioSystem/Blueprint/BP_SoundComponent.Play` (`self.BP_SoundComponent`)))

(fn `CreateEvidenceObject`
  (params (`Evidence Object` :type "/Game/ElCortijo/Features/3_InteractableElements/1_IObjects/Evidence/BP_Evidence Object Reference"))
  (bind (_placement _emptyslot) (`self.SetEvidenceINHP` `Evidence Object`))
  (bind _asbp_object_evidence (cast `/Game/ElCortijo/Features/3_InteractableElements/1_IObjects/Evidence/Evidences/BP_ObjectEvidence` `Evidence Object`))
  (bind _placedactor (`/Game/ElCortijo/Features/1_MainCharacter/BP_InventoryComponent.Place Actor` (`self.Inventory Slot`) (`KismetMathLibrary.MakeTransform` (`KismetMathLibrary.MakeVector` (.x (.location (`SceneComponent.K2_GetComponentToWorld` _placement))) (.y (.location (`SceneComponent.K2_GetComponentToWorld` _placement))) (+ (`/Game/ElCortijo/Features/3_InteractableElements/1_IObjects/Evidence/Evidences/BP_ObjectEvidence.Offset` _asbp_object_evidence) (.z (.location (`SceneComponent.K2_GetComponentToWorld` _placement))))) (.rotation (`SceneComponent.K2_GetComponentToWorld` _placement)) (.scale (`SceneComponent.K2_GetComponentToWorld` _placement)))))
  (bind _asbp_evidence (cast `/Game/ElCortijo/Features/3_InteractableElements/1_IObjects/Evidence/BP_Evidence` _placedactor))
  (`/Game/ElCortijo/Features/3_InteractableElements/1_IObjects/Evidence/BP_Evidence.SetClickable` _asbp_evidence true)
  (`/Game/ElCortijo/Features/3_InteractableElements/1_IObjects/Evidence/BP_Evidence.SetTable` _asbp_evidence self)
  (set `/Game/ElCortijo/Features/3_InteractableElements/1_IObjects/Evidence/BP_Evidence.SlotIndex` _emptyslot _asbp_evidence)
  (`self.K2_AttachToActor` _asbp_evidence self "None" "KeepWorld" "KeepWorld" "KeepWorld" false)
  (`KismetArrayLibrary.Array_Insert` (`self.EvidenceObjectsInTable`) _asbp_evidence _emptyslot))

(fn `Generate Cell Grid`
  (params (X :type Integer) (Y :type Integer))
  (locals (HoldCell :type "/Game/ElCortijo/Features/4_InteratableTables/ModelBoard/Blueprint/S_Cell Structure") (_X :type Integer) (_Y :type Integer) (XTracker :type Integer) (YTracker :type Integer :default 1) (Index :type Integer))
  (bind _returnvalue (`KismetMathLibrary.MakeVector2D` (`KismetMathLibrary.Conv_IntToDouble` (`local.XTracker`)) (`KismetMathLibrary.Conv_IntToDouble` (`local.YTracker`))))
  (set `local._X` X)
  (set `local._Y` Y)
  (set `local.XTracker` 0)
  (set `local.YTracker` 1)
  (for _ (range (* (`local._X`) (`local._Y`)))
    (if (>= (`local.XTracker`) (`local._X`))
      (set `local.YTracker` (+ (`local.YTracker`) 1))
      (set `local.XTracker` 0))
    (set `local.XTracker` (+ 1 (`local.XTracker`)))
    (set `local.HoldCell` (make `/Game/ElCortijo/Features/4_InteratableTables/ModelBoard/Blueprint/S_Cell` _returnvalue null))
    (for _array_element (`self.ValidCellsPrototype`)
      (if (== (break `/Game/ElCortijo/Features/4_InteratableTables/ModelBoard/Blueprint/S_Cell` _array_element) _returnvalue)
        (set `local.HoldCell` (make `/Game/ElCortijo/Features/4_InteratableTables/ModelBoard/Blueprint/S_Cell` _returnvalue null (`.CorrectContainer_15_E16AA9D2474B63CDD6C68D8409073F82` (break `/Game/ElCortijo/Features/4_InteratableTables/ModelBoard/Blueprint/S_Cell` _array_element)) (`.IsValid_14_7034062B45B15D9000B556940AA850BD` (break `/Game/ElCortijo/Features/4_InteratableTables/ModelBoard/Blueprint/S_Cell` _array_element))))))
    (`KismetArrayLibrary.Array_Add` (`self.Grid`) (`local.HoldCell`))))

(fn `Get Cell From Object`
  (params (BP_Evidence :type "/Game/ElCortijo/Features/3_InteractableElements/1_IObjects/Evidence/BP_Evidence Object Reference"))
  (returns (Cell :type "Vector2D Structure") (IsCellValid :type Boolean))
  (bind (_gridsize_x _gridsize_y) (`KismetMathLibrary.BreakVector2D` (`self.GridSize`)))
  (bind (_returnvalue_x _returnvalue_y) (`KismetMathLibrary.BreakVector` (/ (`KismetMathLibrary.InverseTransformLocation` (`SceneComponent.K2_GetComponentToWorld` (`self.RelativeGridPlacement`)) (`self.K2_GetActorLocation` BP_Evidence)) (`self.Distance Between Cells`))))
  (bind _returnvalue (`KismetMathLibrary.FFloor` _returnvalue_y))
  (bind _returnvalue_2 (`KismetMathLibrary.FFloor` _returnvalue_x))
  (bind _returnvalue_3 (`KismetMathLibrary.MakeVector2D` (`KismetMathLibrary.Conv_IntToDouble` _returnvalue_2) (`KismetMathLibrary.Conv_IntToDouble` _returnvalue)))
  (bind _isvalid (`self.GetCellValidity` _returnvalue_3))
  (return _returnvalue_3 (and _isvalid (and (and (<= _returnvalue_2 (`KismetMathLibrary.FTrunc` _gridsize_x)) (> _returnvalue_2 0)) (and (<= _returnvalue (`KismetMathLibrary.FTrunc` _gridsize_y)) (> _returnvalue 0))))))

(fn `Get Cell Relative Pos`
  (params (Cell :type "Vector2D Structure"))
  (returns (`Relative Pos` :type "Vector Structure"))
  (return (+ (* Cell (`self.Distance Between Cells`)) (`SceneComponent.RelativeLocation` (`self.RelativeGridPlacement`)))))

(fn `GetCellValidity`
  (params (Cell :type "Vector2D Structure"))
  (returns (IsValid :type Boolean))
  (locals (VIndex :type Integer))
  (bind _gridsize_x (`KismetMathLibrary.BreakVector2D` (`self.GridSize`)))
  (bind _output_get (set `local.VIndex` (`KismetMathLibrary.FTrunc` (+ Cell_X (* (- Cell_Y 1.0) _gridsize_x)))))
  (bind (_output_posinarray _output_contains _output_correctcontainer _output_isvalid) (break `/Game/ElCortijo/Features/4_InteratableTables/ModelBoard/Blueprint/S_Cell` (`|GetArrayItem` (`self.Grid`) (- _output_get 1))))
  (return _output_isvalid))

(fn `GetFirstEmptySlot`
  (returns (Slot :type Integer) (IsRoom :type Boolean))
  (locals (TempSlot :type Integer) (TempIsRoom :type Boolean))
  (set `local.TempIsRoom` false)
  (for (_array_element _array_index) (`self.HintPlacementsRef`)
    (if (== (`.Evidence_7_18C52045475546F6D7C545884F8868D5` (break `/Game/ElCortijo/Features/4_InteratableTables/S_TablePlacements` _array_element)) null)
      (set `local.TempIsRoom` true)
      (set `local.TempSlot` _array_index)
      (break)))
  (return (`local.TempSlot`) (`local.TempIsRoom`)))

(fn `IsCellEmpty`
  (params (Cell :type "Vector2D Structure"))
  (returns (IsEmpty :type Boolean))
  (locals (VIndex :type Integer))
  (bind _gridsize_x (`KismetMathLibrary.BreakVector2D` (`self.GridSize`)))
  (bind _output_get (set `local.VIndex` (`KismetMathLibrary.FTrunc` (+ Cell_X (* (- Cell_Y 1.0) _gridsize_x)))))
  (bind (_output_posinarray _output_contains) (break `/Game/ElCortijo/Features/4_InteratableTables/ModelBoard/Blueprint/S_Cell` (`|GetArrayItem` (`self.Grid`) (- _output_get 1))))
  (return (== _output_contains null)))

(fn `LeftClickPressed`
  (bind (_bblockinghit _binitialoverlap _time _distance _location _impactpoint _normal _impactnormal _physmat _hitactor) (`GameplayStatics.BreakHitResult` (`PlayerController.GetHitResultUnderCursorByChannel` (`self.Controller`) "TraceTypeQuery5" true)))
  (if (== (`self.MovingObject`) null)
    (if (`KismetArrayLibrary.Array_IsNotEmpty` (`self.EvidenceObjectsInTable`))
      (if (`self.PlayerInTable`)
        (if (`KismetSystemLibrary.DoesImplementInterface` _hitactor "/Game/ElCortijo/Features/2_InteractionSystem/BPI_Clickable.BPI_Clickable_C")
          (bind _asbp_evidence (cast `/Game/ElCortijo/Features/3_InteractableElements/1_IObjects/Evidence/BP_Evidence` _hitactor))
          (set `self.DescriptinObject` _asbp_evidence)
          (`self.SetDescriptonOnScreen`))))))

(fn `Remove ObjectFromGrid`
  (params (Cell :type "Vector2D Structure"))
  (locals (VIndex :type Integer))
  (bind _grid (`self.Grid`))
  (bind _gridsize_x (`KismetMathLibrary.BreakVector2D` (`self.GridSize`)))
  (bind _output_get (set `local.VIndex` (`KismetMathLibrary.FTrunc` (+ Cell_X (* (- Cell_Y 1.0) _gridsize_x)))))
  (bind _returnvalue (- _output_get 1))
  (bind (_output_posinarray _output_contains _output_correctcontainer _output_isvalid) (break `/Game/ElCortijo/Features/4_InteratableTables/ModelBoard/Blueprint/S_Cell` (`|GetArrayItem` _grid _returnvalue)))
  (`KismetArrayLibrary.Array_Set` _grid _returnvalue (make `/Game/ElCortijo/Features/4_InteratableTables/ModelBoard/Blueprint/S_Cell` (`KismetMathLibrary.MakeVector2D` Cell_X Cell_Y) null _output_correctcontainer _output_isvalid))
  (return))

(fn `RemoveEvidenceINHP`
  (params (index :type Integer))
  (bind _output (`|GetArrayItem` (`self.HintPlacementsRef`) index))
  (`|VariableSetRef` _output (make `/Game/ElCortijo/Features/4_InteratableTables/S_TablePlacements` (`.Placement_2_FD44286F48BEEE48D0811A9809672CC7` (break `/Game/ElCortijo/Features/4_InteratableTables/S_TablePlacements` _output)) null)))

(fn `RightClickPress`
  (bind (_bblockinghit _binitialoverlap _time _distance _location _impactpoint _normal _impactnormal _physmat _hitactor) (`GameplayStatics.BreakHitResult` (`PlayerController.GetHitResultUnderCursorByChannel` (`self.Controller`) "TraceTypeQuery5" true)))
  (if (== (`self.MovingObject`) null)
    (if (`KismetArrayLibrary.Array_IsNotEmpty` (`self.EvidenceObjectsInTable`))
      (if (`self.PlayerInTable`)
        (if (`KismetSystemLibrary.DoesImplementInterface` _hitactor "/Game/ElCortijo/Features/2_InteractionSystem/BPI_Clickable.BPI_Clickable_C")
          (message `/Game/ElCortijo/Features/2_InteractionSystem/BPI_Clickable.Click` _hitactor null)
          (bind _asbp_evidence (cast `/Game/ElCortijo/Features/3_InteractableElements/1_IObjects/Evidence/BP_Evidence` _hitactor))
          (set `self.MovingObject` _asbp_evidence))))))

(fn `RightClickRelease`
  (bind _movingobject (`self.MovingObject`))
  (if (`KismetArrayLibrary.Array_IsNotEmpty` (`self.EvidenceObjectsInTable`))
    (if (!= _movingobject null)
      (if (`self.PlayerInTable`)
        (message `/Game/ElCortijo/Features/2_InteractionSystem/BPI_Clickable.Release` _movingobject null)
        (`/Game/ElCortijo/Features/7_AudioSystem/Blueprint/BP_SoundComponent.Play` (`self.BP_SoundComponent`))
        (set `self.MovingObject` null)))))

(fn `SetDescriptonOnScreen`
  (`/Game/ElCortijo/Features/4_InteratableTables/ModelBoard/UI/WBP_ModelBoard.SetEvidenceNotesOnDescription` (`self.WBP_ModelBoard`) (`self.DescriptinObject`)))

(fn `SetEvidenceINHP`
  (params (BP_Evidence :type "/Game/ElCortijo/Features/3_InteractableElements/1_IObjects/Evidence/BP_Evidence Object Reference"))
  (returns (Placement :type "StaticMeshComponent Object Reference") (EmptySlot :type Integer))
  (bind (_slot _isroom) (`self.GetFirstEmptySlot`))
  (if _isroom
    (bind (_output_placement _output_evidence) (break `/Game/ElCortijo/Features/4_InteratableTables/S_TablePlacements` (`|GetArrayItem` (`self.HintPlacementsRef`) _slot)))
    (`|VariableSetRef` _output_evidence BP_Evidence)
    (return _output_placement _slot)))

(fn `SetVisor Pos`
  (params (Cell :type "Vector2D Structure") (`is Valid` :type Boolean))
  (bind _visor (`self.Visor`))
  (if `is Valid`
    (bind _relative_pos (`self.Get Cell Relative Pos` Cell))
    (`SceneComponent.SetVisibility` _visor true false)
    (`SceneComponent.K2_SetRelativeLocation` _visor _relative_pos false false)
    (else
      (`SceneComponent.SetVisibility` _visor false false))))

(fn `SubirPiso`)

(fn `UpdateCorrectPlacements`
  (set `self.CorrectPlacementsAmount` 0)
  (for _array_element (`self.EvidenceObjectsInTable`)
    (bind _asbp_object_evidence (cast `/Game/ElCortijo/Features/3_InteractableElements/1_IObjects/Evidence/Evidences/BP_ObjectEvidence` _array_element))
    (if (`/Game/ElCortijo/Features/3_InteractableElements/1_IObjects/Evidence/Evidences/BP_ObjectEvidence.IsOnCorrectPlace` _asbp_object_evidence)
      (set `self.CorrectPlacementsAmount` (+ (`self.CorrectPlacementsAmount`) 1)))))

(fn `UserConstructionScript`)