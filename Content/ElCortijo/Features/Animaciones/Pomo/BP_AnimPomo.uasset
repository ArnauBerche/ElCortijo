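; BP_AnimPomo is an actor that plays a scripted doorknob (pomo) cutscene when HacerAnim is called.
; It blends the player view to the owner of its Camera, reveals the mesh, and slides it along Y.
; Six chained timelines then animate the mesh's pitch, before the view blends back to the player character.
; The rotation updates feed the mesh's relative location X and Z into roll and yaw.
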(event `self.HacerAnim`
  (bind _mesh (`self.Mesh`))
  (bind _mesh_2 (`self.Mesh`))
  (bind _mesh_3 (`self.Mesh`))
  (bind _mesh_4 (`self.Mesh`))
  (bind _mesh_5 (`self.Mesh`))
  (bind _mesh_6 (`self.Mesh`))
  (bind _mesh_7 (`self.Mesh`))
  (bind (_relativelocation_x _relativelocation_y _relativelocation_z) (`KismetMathLibrary.BreakVector` (`SceneComponent.RelativeLocation` _mesh)))
  (bind (_relativelocation_x_2 _relativelocation_y_2 _relativelocation_z_2) (`KismetMathLibrary.BreakVector` (`SceneComponent.RelativeLocation` _mesh_2)))
  (bind (_relativelocation_x_3 _relativelocation_y_3 _relativelocation_z_3) (`KismetMathLibrary.BreakVector` (`SceneComponent.RelativeLocation` _mesh_4)))
  (bind (_relativelocation_x_4 _relativelocation_y_4 _relativelocation_z_4) (`KismetMathLibrary.BreakVector` (`SceneComponent.RelativeLocation` _mesh_3)))
  (bind (_relativelocation_x_5 _relativelocation_y_5 _relativelocation_z_5) (`KismetMathLibrary.BreakVector` (`SceneComponent.RelativeLocation` _mesh_6)))
  (bind (_relativelocation_x_6 _relativelocation_y_6 _relativelocation_z_6) (`KismetMathLibrary.BreakVector` (`SceneComponent.RelativeLocation` _mesh_7)))
  (bind (_relativelocation_x_7 _relativelocation_y_7 _relativelocation_z_7) (`KismetMathLibrary.BreakVector` (`SceneComponent.RelativeLocation` _mesh_5)))
  (`PlayerController.SetViewTargetWithBlend` (`GameplayStatics.GetPlayerController` 0) (`ActorComponent.GetOwner` (`self.Camera`)) 1.0 "VTBlend_Linear" 0.0 false)
  (`KismetSystemLibrary.Delay` 2.0)
  (`SceneComponent.SetVisibility` (`self.Mesh`) true false)
  (`KismetSystemLibrary.Delay` 0.8)
  (bind (_direction _newtrack_0) (`Timeline|Cronograma` :!via `PlayFromStart`)
    (:`Update`
      (`SceneComponent.K2_SetRelativeLocation` _mesh_4 (`KismetMathLibrary.MakeVector` _relativelocation_x_3 _newtrack_0 _relativelocation_z_3) false false))
    (:`Finished`
      (`KismetSystemLibrary.Delay` 0.2)
      (bind (_direction_2 _newtrack_0_2) (`Timeline|Cronograma_0` :!via `PlayFromStart`)
        (:`Update`
          (`SceneComponent.K2_SetRelativeRotation` _mesh_7 (`KismetMathLibrary.MakeRotator` _relativelocation_x_6 _newtrack_0_2 _relativelocation_z_6) false false))
        (:`Finished`
          (bind (_direction_3 _newtrack_0_3) (`Timeline|Cronograma_1` :!via `PlayFromStart`)
            (:`Update`
              (`SceneComponent.K2_SetRelativeRotation` _mesh (`KismetMathLibrary.MakeRotator` _relativelocation_x _newtrack_0_3 _relativelocation_z) false false))
            (:`Finished`
              (`KismetSystemLibrary.Delay` 0.2)
              (bind (_direction_4 _newtrack_0_4) (`Timeline|Cronograma_2` :!via `PlayFromStart`)
                (:`Update`
                  (`SceneComponent.K2_SetRelativeRotation` _mesh_2 (`KismetMathLibrary.MakeRotator` _relativelocation_x_2 _newtrack_0_4 _relativelocation_z_2) false false))
                (:`Finished`
                  (bind (_direction_5 _newtrack_0_5) (`Timeline|Cronograma_3` :!via `PlayFromStart`)
                    (:`Update`
                      (`SceneComponent.K2_SetRelativeRotation` _mesh_3 (`KismetMathLibrary.MakeRotator` _relativelocation_x_4 _newtrack_0_5 _relativelocation_z_4) false false))
                    (:`Finished`
                      (bind (_direction_6 _newtrack_0_6) (`Timeline|Cronograma_4` :!via `PlayFromStart`)
                        (:`Update`
                          (`SceneComponent.K2_SetRelativeRotation` _mesh_6 (`KismetMathLibrary.MakeRotator` _relativelocation_x_5 _newtrack_0_6 _relativelocation_z_5) false false))
                        (:`Finished`
                          (bind (_direction_7 _newtrack_0_7) (`Timeline|Cronograma_5` :!via `PlayFromStart`)
                            (:`Update`
                              (`SceneComponent.K2_SetRelativeRotation` _mesh_5 (`KismetMathLibrary.MakeRotator` _relativelocation_x_7 _newtrack_0_7 _relativelocation_z_7) false false))
                            (:`Finished`
                              (`KismetSystemLibrary.Delay` 0.2)
                              (`PlayerController.SetViewTargetWithBlend` (`GameplayStatics.GetPlayerController` 0) (`GameplayStatics.GetPlayerCharacter` 0) 1.0 "VTBlend_Linear" 0.0 false))))))))))))))))

(fn `UserConstructionScript`
  (`parent.UserConstructionScript`))