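; Police light actor that flashes a blue light component (LuzAzul) in an endless strobe pattern.
; BeginPlay starts a self-looping chain of Delay nodes that switches the light's intensity between full and zero, giving an uneven double blink.
; Tick, overlap and the construction script hold no logic.
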(event `self.ReceiveBeginPlay`
  (`KismetSystemLibrary.Delay` 0.1 :!label _label)
  (`LightComponent.SetIntensity` (`self.LuzAzul`) 30000.0)
  (`KismetSystemLibrary.Delay` 0.1)
  (`LightComponent.SetIntensity` (`self.LuzAzul`) 0.0)
  (`KismetSystemLibrary.Delay` 0.1)
  (`LightComponent.SetIntensity` (`self.LuzAzul`) 30000.0)
  (`KismetSystemLibrary.Delay` 0.2)
  (`LightComponent.SetIntensity` (`self.LuzAzul`) 0.0)
  (goto _label))

(event `self.ReceiveTick`
  (params (DeltaSeconds :type "Float (single-precision)")))

(fn `UserConstructionScript`)