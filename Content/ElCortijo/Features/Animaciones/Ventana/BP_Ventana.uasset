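; BP_Ventana is an ambient animated window that keeps swinging on its own from BeginPlay.
; PlayAnim picks a random target yaw and duration within min/max variables, then plays the MovVentana timeline to lerp the Pivot's yaw from its current angle.
; When the timeline finishes, a short random delay calls PlayAnim again, producing an endless, irregular sway.
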(event `self.ReceiveBeginPlay`
  (`self.PlayAnim`))

(event `PlayAnim`
  (bind (_relativerotation_roll _relativerotation_pitch _relativerotation_yaw) (`KismetMathLibrary.BreakRotator` (`SceneComponent.RelativeRotation` (`self.Pivot`))))
  (bind (_relativerotation_roll_2 _relativerotation_pitch_2) (`KismetMathLibrary.BreakRotator` (`SceneComponent.RelativeRotation` (`self.Pivot`))))
  (set `self.StartAngle` _relativerotation_yaw)
  (bind _output_get (set `self.TargetAngle` (`KismetMathLibrary.RandomFloatInRange` (`self.MinAngle`) (`self.MaxAngle`))))
  (bind _output_get_2 (set `self.Duration` (`KismetMathLibrary.RandomFloatInRange` (`self.MinDuration`) (`self.MaxDuration`))))
  (bind (_direction _newtrack_0) (`Timeline|MovVentana` :`NewTime` _output_get_2)
    (:`Update`
      (`SceneComponent.K2_SetRelativeRotation` (`self.Pivot`) (`KismetMathLibrary.MakeRotator` _relativerotation_roll_2 _relativerotation_pitch_2 (`KismetMathLibrary.Lerp` (`self.StartAngle`) _output_get _newtrack_0)) false false))
    (:`Finished`
      (`KismetSystemLibrary.Delay` (`KismetMathLibrary.RandomFloatInRange` 0.3 0.5))
      (`self.PlayAnim`))))

(fn `UserConstructionScript`)