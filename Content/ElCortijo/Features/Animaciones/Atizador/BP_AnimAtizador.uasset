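; BP_AnimAtizador is a scripted animation of a poker (atizador) that starts on BeginPlay.
; After timed delays, it blends the player's view to the Camara component's owner and reveals the Atizador.
; Timeline Palanca01 slides Punta along local Y, then chains into Palanca02, which only sets Punta's rotation to constant zero.
; The blend back to the player character is unconnected, so the view never returns.
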(event `self.ReceiveBeginPlay`
  (bind _punta (`self.Punta`))
  (bind (_relativelocation_x _relativelocation_y _relativelocation_z) (`KismetMathLibrary.BreakVector` (`SceneComponent.RelativeLocation` _punta)))
  (`KismetSystemLibrary.Delay` 2.0)
  (`PlayerController.SetViewTargetWithBlend` (`GameplayStatics.GetPlayerController` 0) (`ActorComponent.GetOwner` (`self.Camara`)) 1.0 "VTBlend_Linear" 0.0 false)
  (`KismetSystemLibrary.Delay` 2.0)
  (`SceneComponent.SetVisibility` (`self.Atizador`) true false)
  (bind (_direction _newtrack_0) (`Timeline|Palanca01` :!via `PlayFromStart`)
    (:`Update`
      (`SceneComponent.K2_SetRelativeLocation` _punta (`KismetMathLibrary.MakeVector` _relativelocation_x _newtrack_0 _relativelocation_z) false false))
    (:`Finished`
      (`Timeline|Palanca02` :!via `PlayFromStart`
        (:`Update`
          (`SceneComponent.K2_SetRelativeRotation` (`self.Punta`) (`KismetMathLibrary.MakeRotator` 0.0) false false))))))

(fn `UserConstructionScript`)