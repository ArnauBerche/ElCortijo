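; BP_SustoRYA is a scare trigger actor that detects when the player keeps looking at a specific component.
; Overlapping the Trigger stores the first-person character and enables vision checks; leaving clears both.
; While IsOpen is also true, Tick traces from the camera on the Camera channel, accumulating time on ViewDetection and resetting on other results.
; Reaching MaxTime fires once, currently only printing "PlayAnimation".
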(event `self.ReceiveBeginPlay`)

(event `self.ReceiveTick`
  (params (DeltaSeconds :type "Float (single-precision)"))
  (bind _first_person_character (`self.First Person Character`))
  (bind _firstpersoncamera (`/Game/ElCortijo/Features/1_MainCharacter/Blueprints/BP_FirstPersonCharacter.FirstPersonCamera` _first_person_character))
  (bind _returnvalue (`SceneComponent.K2_GetComponentLocation` _firstpersoncamera))
  (set `self.Delta Seconds` DeltaSeconds)
  (if (`self.IsOpen`)
    (if (`self.IsVisionEnabled`)
      (if (!= (`self.First Person Character`) null)
        (bind _outhit (`KismetSystemLibrary.LineTraceSingle` _returnvalue (+ _returnvalue (* (`SceneComponent.GetForwardVector` _firstpersoncamera) (`self.Distance`))) "TraceTypeQuery2" false (`|MakeArray` _first_person_character :!type "Actor Object Reference") "None" false (struct :`R` 1.0 :`A` 1.0) (struct :`G` 1.0 :`A` 1.0) 0.1))
        (if (== (`.HitComponent` (`GameplayStatics.BreakHitResult` _outhit)) (`self.ViewDetection`))
          (if (< (`self.TimeLooking`) (`self.MaxTime`))
            (set `self.TimeLooking` (+ (`self.TimeLooking`) (`self.Delta Seconds`)))
            (else
              (`/Engine/EditorBlueprintResources/StandardMacros.DoOnce` false
                (:`Completed`
                  (`KismetSystemLibrary.PrintString` "PlayAnimation")))))
          (else
            (set `self.TimeLooking` 0.0)))))))

(event `self.Trigger.OnComponentBeginOverlap`
  (params (OverlappedComponent :type "PrimitiveComponent Object Reference") (OtherActor :type "Actor Object Reference") (OtherComp :type "PrimitiveComponent Object Reference") (OtherBodyIndex :type Integer) (bFromSweep :type Boolean) (SweepResult :type "HitResult Structure (by ref)"))
  (bind _asbp_first_person_character (cast `/Game/ElCortijo/Features/1_MainCharacter/Blueprints/BP_FirstPersonCharacter` OtherActor))
  (set `self.First Person Character` _asbp_first_person_character)
  (set `self.IsVisionEnabled` true))

(event `self.Trigger.OnComponentEndOverlap`
  (params (OverlappedComponent :type "PrimitiveComponent Object Reference") (OtherActor :type "Actor Object Reference") (OtherComp :type "PrimitiveComponent Object Reference") (OtherBodyIndex :type Integer))
  (cast `/Game/ElCortijo/Features/1_MainCharacter/Blueprints/BP_FirstPersonCharacter` OtherActor)
  (set `self.First Person Character` null)
  (set `self.IsVisionEnabled` false))

(fn `UserConstructionScript`)