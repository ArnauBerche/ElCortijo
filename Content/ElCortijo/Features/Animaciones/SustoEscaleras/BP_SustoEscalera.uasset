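; BP_SustoEscalera is a staircase scare trigger that disorients the player when its volume is overlapped.
; An overlap plays a dizzy camera shake and a timeline that repeatedly divides the character's walk speed, compounding the slowdown.
; Do-once gates reveal a post-process component and fire a delayed camera-drop shake.
; When the timeline ends, it swaps the post-process settings, with a debug print marking an intended black screen.
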(event `self.ReceiveBeginPlay`
  (set `self.HasBeenActivated` true))

(event `self.Trigger.OnComponentBeginOverlap`
  (params (OverlappedComponent :type "PrimitiveComponent Object Reference") (OtherActor :type "Actor Object Reference") (OtherComp :type "PrimitiveComponent Object Reference") (OtherBodyIndex :type Integer) (bFromSweep :type Boolean) (SweepResult :type "HitResult Structure (by ref)"))
  (bind _postprocess (`self.PostProcess`))
  (if (`self.HasBeenActivated`)
    (`GameplayStatics.PlayWorldCameraShake` "/Game/ElCortijo/Features/Animaciones/SustoEscaleras/BP_CameraShakeDizzy.BP_CameraShakeDizzy_C" (`PlayerCameraManager.GetCameraLocation` (`GameplayStatics.GetPlayerCameraManager` 0)) 0.0 1000.0)
    (bind _asbp_first_person_character (cast `/Game/ElCortijo/Features/1_MainCharacter/Blueprints/BP_FirstPersonCharacter` (`GameplayStatics.GetPlayerCharacter` 0)))
    (bind (_direction _newtrack_0) (`Timeline|ReduceSpeedOvertime` :!via `PlayFromStart`)
      (:`Update`
        (bind _charactermovement (`Character.CharacterMovement` _asbp_first_person_character))
        (set `CharacterMovementComponent.MaxWalkSpeed` (/ (`CharacterMovementComponent.MaxWalkSpeed` _charactermovement) _newtrack_0) _charactermovement)
        (`|ExecutionSequence`
          (:`then_0`
            (`/Engine/EditorBlueprintResources/StandardMacros.DoOnce` false :!label _label
              (:`Completed`
                (`KismetSystemLibrary.Delay` 3.0)
                (`GameplayStatics.PlayWorldCameraShake` "/Game/ElCortijo/Features/Animaciones/SustoEscaleras/BP_CameraDrop.BP_CameraDrop_C" (`PlayerCameraManager.GetCameraLocation` (`GameplayStatics.GetPlayerCameraManager` 0)) 0.0 1000.0))))
          (:`then_1`
            (`/Engine/EditorBlueprintResources/StandardMacros.DoOnce` false
              (:`Completed`
                (`KismetSystemLibrary.PrintString` "Poner postpocess")
                (`SceneComponent.SetHiddenInGame` _postprocess false false)
                (`SceneComponent.SetVisibility` _postprocess true false))))))
      (:`Finished`
        (`|ExecutionSequence`
          (:`then_0`
            (goto _label :!via `Reset`))
          (:`then_1`
            (`KismetSystemLibrary.PrintString` "Poner Pantalla en negro")
            (set `PostProcessComponent.Settings` (`self.PostProces`) (`self.PostProcess`))))))))

(fn `UserConstructionScript`)