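; BP_LuzApagadaPoint is a point light fixture that flickers and then goes out when anything overlaps its collision volume.
; The overlap applies a flicker light function material and adds an audio component at the light's relative position.
; After a random delay of a few seconds it plays a blackout sound, destroys the light, trigger and audio, and swaps the bulb to a non-emissive material.
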(event `self.Collision.OnComponentBeginOverlap`
  (params (OverlappedComponent :type "PrimitiveComponent Object Reference") (OtherActor :type "Actor Object Reference") (OtherComp :type "PrimitiveComponent Object Reference") (OtherBodyIndex :type Integer) (bFromSweep :type Boolean) (SweepResult :type "HitResult Structure (by ref)"))
  (bind _pointlight (`self.PointLight`))
  (bind _relativelocation (`SceneComponent.RelativeLocation` _pointlight))
  (`LightComponent.SetLightFunctionMaterial` _pointlight "/Game/ElCortijo/Features/Animaciones/Parpadeo/M_Parpadeo2.M_Parpadeo2")
  (bind _returnvalue (`AddComponent|NODE_AddAudioComponent-0` :`RelativeTransform` (`KismetMathLibrary.MakeTransform` _relativelocation)))
  (`KismetSystemLibrary.Delay` (`KismetMathLibrary.RandomFloatInRange` 1.0 4.0))
  (`GameplayStatics.PlaySoundAtLocation` "/Game/ElCortijo/Features/Animaciones/LuzApagada/S_Apagon2.S_Apagon2" _relativelocation (struct) 1.0 1.0 0.0 null null null null)
  (`ActorComponent.K2_DestroyComponent` (`self.PointLight`))
  (`ActorComponent.K2_DestroyComponent` (`self.Collision`))
  (`ActorComponent.K2_DestroyComponent` _returnvalue)
  (`PrimitiveComponent.SetMaterial` (`self.Bombilla`) 0 "/Game/ElCortijo/Features/Props/Interior/Iluminacion/BombillaColgada/Textura/M_Bombilla_NoEmisive.M_Bombilla_NoEmisive"))

(fn `UserConstructionScript`)