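; Pickable world actor that the first-person character can pick up through interaction.
; Interact calls PickUp, which casts the interactor to BP_FirstPersonCharacter and passes itself to that character's InventorySlot.
; Helper functions toggle physics and gravity on its Collision component, and switch interactability by blocking or ignoring a custom trace channel.
; The inventory-full message and destroy-on-pickup logic are present but never run.
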(event `self.ReceiveBeginPlay`)

(event `/Game/ElCortijo/Features/Interaction/BPI_Interactable.Interact`
  (params (Interactor :type "Actor Object Reference"))
  (`self.PickUp` Interactor))

(fn `PickUp`
  (params (Character :type "Actor Object Reference"))
  (bind _asbp_first_person_character (cast `/Game/FirstPerson/Blueprints/BP_FirstPersonCharacter` Character))
  (`/Game/ElCortijo/Features/Character/BP_InventoryComponent.PickUpActor` (`/Game/FirstPerson/Blueprints/BP_FirstPersonCharacter.InventorySlot` _asbp_first_person_character) self))

(fn `SetInteractable`
  (params (Enabled :type Boolean))
  (bind _collision (`self.Collision`))
  (if Enabled
    (`PrimitiveComponent.SetCollisionResponseToChannel` _collision "ECC_GameTraceChannel1" "ECR_Block")
    (else
      (`PrimitiveComponent.SetCollisionResponseToChannel` _collision "ECC_GameTraceChannel1" "ECR_Ignore"))))

(fn `SetPhysics`
  (params (bActive :type Boolean))
  (bind _collision (`self.Collision`))
  (`PrimitiveComponent.SetSimulatePhysics` _collision bActive)
  (`PrimitiveComponent.SetEnableGravity` _collision bActive))

(fn `UserConstructionScript`)