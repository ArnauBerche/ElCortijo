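; Interactable evidence board where the player, toggled into a blended camera view with cursor and widget, handles evidence carried from the inventory.
; Object evidence spawns into the first free side slot, while other evidence goes to the widget's list.
; Cursor traces grab and release pieces through click messages.
; A grid with per-cell validity and expected class provides helpers for snapping, occupancy and correctness checks.
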(event `self.ReceiveBeginPlay`
  (bind (_gridsize_x _gridsize_y) (`KismetMathLibrary.BreakVector2D` (`self.GridSize`)))
  (`|ExecutionSequence`
    (:`then_0`
      (set `self.TType` "NewEnumerator1"))
    (:`then_1`
      (`self.Generate Cell Grid` (`KismetMathLibrary.FTrunc` _gridsize_x) (`KismetMathLibrary.FTrunc` _gridsize_y)))
    (:`then_2`
      (for _array_element (`SceneComponent.GetChildrenComponents` (`self.EvidenceRelativeSlots`) true)
        (bind _asstatic_mesh_component (cast `StaticMeshComponent` _array_element))
        (`KismetArrayLibrary.Array_Add` (`self.HintPlacementsRef`) (make `/Game/ElCortijo/Features/ResearchTable/S_TablePlacements` _asstatic_mesh_component null))))
    (:`then_3`
      (bind _asbp_first_person_character (cast `/Game/FirstPerson/Blueprints/BP_FirstPersonCharacter` (`GameplayStatics.GetPlayerCharacter` 0)))
      (add `/Game/FirstPerson/Blueprints/BP_FirstPersonCharacter.OnLeftClickPress` _asbp_first_person_character (delegate `OnLeftClickPress_Handler`))
      (add `/Game/FirstPerson/Blueprints/BP_FirstPersonCharacter.OnLeftClickRelease` _asbp_first_person_character (delegate `OnLeftClickRelease_Handler`)))
    (:`then_4`
      (bind _returnvalue (`|CreateWidget` "/Game/ElCortijo/Features/ModelBoard/UI/WBP_ModelBoard.WBP_ModelBoard_C" (`self.As Player Controller`)))
      (set `self.WBP_ModelBoard` _returnvalue))))

(event `OnLeftClickPress_Handler`
  (`self.LeftClickPress`))

(event `OnLeftClickRelease_Handler`
  (`self.LeftClickRelease`))

(event `self.ReceiveTick`
  (params (DeltaSeconds :type "Float (single-precision)")))

(event `/Game/ElCortijo/Features/Interaction/BPI_Interactable.Interact`
  (params (Interactor :type "Actor Object Reference"))
  (bind _wbp_modelboard (`self.WBP_ModelBoard`))
  (bind _asbp_first_person_character (cast `/Game/FirstPerson/Blueprints/BP_FirstPersonCharacter` Interactor))
  (set `self.As BP First Person Character` _asbp_first_person_character)
  (bind _asplayer_controller (cast `PlayerController` (`Pawn.GetController` _asbp_first_person_character)))
  (set `self.As Player Controller` _asplayer_controller)
  (set `self.CameraOwner` (`ActorComponent.GetOwner` (`self.Camera`)))
  (if (`self.CanInteract`)
    (`/Engine/EditorBlueprintResources/StandardMacros.FlipFlop`
      (:`A`
        (`UserWidget.AddToViewport` _wbp_modelboard 0)
        (`self.CreateEvidence` (`self.As BP First Person Character`))
        (`Controller.SetIgnoreLookInput` (`self.As Player Controller`) true)
        (`Controller.SetIgnoreMoveInput` (`self.As Player Controller`) true)
        (`PlayerController.SetViewTargetWithBlend` (`self.As Player Controller`) (`self.CameraOwner`) (`self.Blend Time`) "VTBlend_Linear" 0.0 false)
        (set `PlayerController.bShowMouseCursor` true (`self.As Player Controller`))
        (set `self.CanInteract` false)
        (`WidgetBlueprintLibrary.SetInputMode_GameAndUIEx` (`self.As Player Controller`) (`self.WBP_ModelBoard`) "LockAlways" false true)
        (`KismetSystemLibrary.Delay` (`self.Blend Time`))
        (set `self.CanInteract` true)
        (set `self.PlayerInTable` true))
      (:`B`
        (`Widget.RemoveFromParent` _wbp_modelboard)
        (`PlayerController.SetViewTargetWithBlend` (`self.As Player Controller`) (`self.As BP First Person Character`) (`self.Blend Time`) "VTBlend_Linear" 0.0 false)
        (set `self.CanInteract` false)
        (`KismetSystemLibrary.Delay` (`self.Blend Time`))
        (set `self.CanInteract` true)
        (`Controller.SetIgnoreLookInput` (`self.As Player Controller`) false)
        (`Controller.SetIgnoreMoveInput` (`self.As Player Controller`) false)
        (set `PlayerController.bShowMouseCursor` false (`self.As Player Controller`))
        (`WidgetBlueprintLibrary.SetInputMode_GameOnly` (`self.As Player Controller`) true)
        (set `self.PlayerInTable` false)))))

(fn `Add ObjectToGrid`
  (params (Cell :type "Vector2D Structure") (Object :type "/Game/ElCortijo/Features/Evidence/Evidences/BP_ObjectEvidence Object Reference"))
  (locals (VIndex :type Integer))
  (bind _grid (`self.Grid`))
  (bind _gridsize_x (`KismetMathLibrary.BreakVector2D` (`self.GridSize`)))
  (bind _output_get (set `local.VIndex` (`KismetMathLibrary.FTrunc` (+ Cell_X (* (- Cell_Y 1.0) _gridsize_x)))))
  (bind _returnvalue (- _output_get 1))
  (bind (_output_posinarray _output_contains _output_correctcontainer _output_isvalid) (break `/Game/ElCortijo/Features/ModelBoard/Blueprint/S_Cell` (`|GetArrayItem` _grid _returnvalue)))
  (`KismetArrayLibrary.Array_Set` _grid _returnvalue (make `/Game/ElCortijo/Features/ModelBoard/Blueprint/S_Cell` (`KismetMathLibrary.MakeVector2D` Cell_X Cell_Y) Object _output_correctcontainer _output_isvalid))
  (return))

(fn `CellHasObject`
  (params (Cell :type "Vector2D Structure") (BP_Evidence :type "/Game/ElCortijo/Features/Evidence/BP_Evidence Object Reference"))
  (returns (HasSelf :type Boolean))
  (locals (VIndex :type Integer))
  (bind _gridsize_x (`KismetMathLibrary.BreakVector2D` (`self.GridSize`)))
  (bind _output_get (set `local.VIndex` (`KismetMathLibrary.FTrunc` (+ Cell_X (* (- Cell_Y 1.0) _gridsize_x)))))
  (bind (_output_posinarray _output_contains) (break `/Game/ElCortijo/Features/ModelBoard/Blueprint/S_Cell` (`|GetArrayItem` (`self.Grid`) (- _output_get 1))))
  (return (== _output_contains BP_Evidence)))

(fn `CheckCorrectContains`
  (params (Cell :type "/Game/ElCortijo/Features/ModelBoard/Blueprint/S_Cell Structure"))
  (returns (IsCorrect :type Boolean))
  (return (== (`GameplayStatics.GetObjectClass` Cell_Contains_11_B344A4CA41F4978793DCCB8186FD342E) Cell_CorrectContainer_15_E16AA9D2474B63CDD6C68D8409073F82)))

(fn `CreateEvidence`
  (params (Interactor :type "/Game/FirstPerson/Blueprints/BP_FirstPersonCharacter Object Reference"))
  (bind _inventoryslot (`/Game/FirstPerson/Blueprints/BP_FirstPersonCharacter.InventorySlot` Interactor))
  (bind _output_get (set `self.Inventory Slot` _inventoryslot))
  (bind _empty (`/Game/ElCortijo/Features/Character/BP_InventoryComponent.IsEmpty` _output_get))
  (if (not _empty)
    (bind _asbp_evidence (cast `/Game/ElCortijo/Features/Evidence/BP_Evidence` (`/Game/ElCortijo/Features/Character/BP_InventoryComponent.CurrentItemActor` _inventoryslot)))
    (if (== (`/Game/ElCortijo/Features/Evidence/BP_Evidence.EType` _asbp_evidence) 0)
      (`self.CreateEvidenceObject` _asbp_evidence)
      (`/Game/ElCortijo/Features/Character/BP_InventoryComponent.EmptyInventoryRef` (`self.Inventory Slot`))
      (else
        (`self.CreateEvidenceNote` _asbp_evidence)))))

(fn `CreateEvidenceNote`
  (params (EvidenceNote :type "/Game/ElCortijo/Features/Evidence/BP_Evidence Object Reference"))
  (`ListView.AddItem` (`/Game/ElCortijo/Features/ModelBoard/UI/WBP_ModelBoard.ListView` (`self.WBP_ModelBoard`)) EvidenceNote))

(fn `CreateEvidenceObject`
  (params (`Evidence Object` :type "/Game/ElCortijo/Features/Evidence/BP_Evidence Object Reference"))
  (bind (_placement _emptyslot) (`self.SetEvidenceINHP` `Evidence Object`))
  (bind _asbp_object_evidence (cast `/Game/ElCortijo/Features/Evidence/Evidences/BP_ObjectEvidence` `Evidence Object`))
  (bind _placedactor (`/Game/ElCortijo/Features/Character/BP_InventoryComponent.Place Actor` (`self.Inventory Slot`) (`KismetMathLibrary.MakeTransform` (`KismetMathLibrary.MakeVector` (.x (.location (`SceneComponent.K2_GetComponentToWorld` _placement))) (.y (.location (`SceneComponent.K2_GetComponentToWorld` _placement))) (+ (`/Game/ElCortijo/Features/Evidence/Evidences/BP_ObjectEvidence.Offset` _asbp_object_evidence) (.z (.location (`SceneComponent.K2_GetComponentToWorld` _placement))))) (.rotation (`SceneComponent.K2_GetComponentToWorld` _placement)) (.scale (`SceneComponent.K2_GetComponentToWorld` _placement)))))
  (bind _asbp_evidence (cast `/Game/ElCortijo/Features/Evidence/BP_Evidence` _placedactor))
  (`/Game/ElCortijo/Features/Evidence/BP_Evidence.SetClickable` _asbp_evidence true)
  (set `/Game/ElCortijo/Features/Evidence/BP_Evidence.CurrentTable` self _asbp_evidence)
  (set `/Game/ElCortijo/Features/Evidence/BP_Evidence.bIsOnTable` true _asbp_evidence)
  (set `/Game/ElCortijo/Features/Evidence/BP_Evidence.SlotIndex` _emptyslot _asbp_evidence)
  (`self.K2_AttachToActor` _asbp_evidence self "None" "KeepWorld" "KeepWorld" "KeepWorld" false)
  (`KismetArrayLibrary.Array_Insert` (`self.EvidenceObjectsInTable`) _asbp_evidence _emptyslot))

(fn `Generate Cell Grid`
  (params (X :type Integer) (Y :type Integer))
  (locals (HoldCell :type "/Game/ElCortijo/Features/ModelBoard/Blueprint/S_Cell Structure") (_X :type Integer) (_Y :type Integer) (XTracker :type Integer) (YTracker :type Integer :default 1) (Index :type Integer))
  (bind _returnvalue (`KismetMathLibrary.MakeVector2D` (`KismetMathLibrary.Conv_IntToDouble` (`local.XTracker`)) (`KismetMathLibrary.Conv_IntToDouble` (`local.YTracker`))))
  (set `local._X` X)
  (set `local._Y` Y)
  (set `local.XTracker` 0)
  (set `local.YTracker` 1)
  (for _ (range (* (`local._X`) (`local._Y`)))
    (if (>= (`local.XTracker`) (`local._X`))
      (set `local.YTracker` (+ (`local.YTracker`) 1))
      (set `local.XTracker` 0))
    (set `local.XTracker` (+ 1 (`local.XTracker`)))
    (set `local.HoldCell` (make `/Game/ElCortijo/Features/ModelBoard/Blueprint/S_Cell` _returnvalue null))
    (for _array_element (`self.ValidCellsPrototype`)
      (if (== (break `/Game/ElCortijo/Features/ModelBoard/Blueprint/S_Cell` _array_element) _returnvalue)
        (set `local.HoldCell` (make `/Game/ElCortijo/Features/ModelBoard/Blueprint/S_Cell` _returnvalue null (`.CorrectContainer_15_E16AA9D2474B63CDD6C68D8409073F82` (break `/Game/ElCortijo/Features/ModelBoard/Blueprint/S_Cell` _array_element)) (`.IsValid_14_7034062B45B15D9000B556940AA850BD` (break `/Game/ElCortijo/Features/ModelBoard/Blueprint/S_Cell` _array_element))))))
    (`KismetArrayLibrary.Array_Add` (`self.Grid`) (`local.HoldCell`))))

(fn `Get Cell From Object`
  (params (BP_Evidence :type "/Game/ElCortijo/Features/Evidence/BP_Evidence Object Reference"))
  (returns (Cell :type "Vector2D Structure") (IsCellValid :type Boolean))
  (bind (_gridsize_x _gridsize_y) (`KismetMathLibrary.BreakVector2D` (`self.GridSize`)))
  (bind (_returnvalue_x _returnvalue_y) (`KismetMathLibrary.BreakVector` (/ (`KismetMathLibrary.InverseTransformLocation` (`SceneComponent.K2_GetComponentToWorld` (`self.RelativeGridPlacement`)) (`self.K2_GetActorLocation` BP_Evidence)) (`self.Distance Between Cells`))))
  (bind _returnvalue (`KismetMathLibrary.FFloor` _returnvalue_y))
  (bind _returnvalue_2 (`KismetMathLibrary.FFloor` _returnvalue_x))
  (bind _returnvalue_3 (`KismetMathLibrary.MakeVector2D` (`KismetMathLibrary.Conv_IntToDouble` _returnvalue_2) (`KismetMathLibrary.Conv_IntToDouble` _returnvalue)))
  (bind _isvalid (`self.GetCellValidity` _returnvalue_3))
  (return _returnvalue_3 (and _isvalid (and (and (<= _returnvalue_2 (`KismetMathLibrary.FTrunc` _gridsize_x)) (> _returnvalue_2 0)) (and (<= _returnvalue (`KismetMathLibrary.FTrunc` _gridsize_y)) (> _returnvalue 0))))))

(fn `Get Cell Relative Pos`
  (params (Cell :type "Vector2D Structure"))
  (returns (`Relative Pos` :type "Vector Structure"))
  (return (+ (* Cell (`self.Distance Between Cells`)) (`SceneComponent.RelativeLocation` (`self.RelativeGridPlacement`)))))

(fn `GetCellValidity`
  (params (Cell :type "Vector2D Structure"))
  (returns (IsValid :type Boolean))
  (locals (VIndex :type Integer))
  (bind _gridsize_x (`KismetMathLibrary.BreakVector2D` (`self.GridSize`)))
  (bind _output_get (set `local.VIndex` (`KismetMathLibrary.FTrunc` (+ Cell_X (* (- Cell_Y 1.0) _gridsize_x)))))
  (bind (_output_posinarray _output_contains _output_correctcontainer _output_isvalid) (break `/Game/ElCortijo/Features/ModelBoard/Blueprint/S_Cell` (`|GetArrayItem` (`self.Grid`) (- _output_get 1))))
  (return _output_isvalid))

(fn `GetFirstEmptySlot`
  (returns (Slot :type Integer) (IsRoom :type Boolean))
  (locals (TempSlot :type Integer) (TempIsRoom :type Boolean))
  (set `local.TempIsRoom` false)
  (for (_array_element _array_index) (`self.HintPlacementsRef`)
    (if (== (`.Evidence_7_18C52045475546F6D7C545884F8868D5` (break `/Game/ElCortijo/Features/ResearchTable/S_TablePlacements` _array_element)) null)
      (set `local.TempIsRoom` true)
      (set `local.TempSlot` _array_index)
      (break)))
  (return (`local.TempSlot`) (`local.TempIsRoom`)))

(fn `IsCellEmpty`
  (params (Cell :type "Vector2D Structure"))
  (returns (IsEmpty :type Boolean))
  (locals (VIndex :type Integer))
  (bind _gridsize_x (`KismetMathLibrary.BreakVector2D` (`self.GridSize`)))
  (bind _output_get (set `local.VIndex` (`KismetMathLibrary.FTrunc` (+ Cell_X (* (- Cell_Y 1.0) _gridsize_x)))))
  (bind (_output_posinarray _output_contains) (break `/Game/ElCortijo/Features/ModelBoard/Blueprint/S_Cell` (`|GetArrayItem` (`self.Grid`) (- _output_get 1))))
  (return (== _output_contains null)))

(fn `LeftClickPress`
  (bind (_bblockinghit _binitialoverlap _time _distance _location _impactpoint _normal _impactnormal _physmat _hitactor) (`GameplayStatics.BreakHitResult` (`PlayerController.GetHitResultUnderCursorByChannel` (`GameplayStatics.GetPlayerController` 0) "TraceTypeQuery5" true)))
  (if (== (`self.MovingObject`) null)
    (if (`KismetArrayLibrary.Array_IsNotEmpty` (`self.EvidenceObjectsInTable`))
      (if (`self.PlayerInTable`)
        (if (`KismetSystemLibrary.DoesImplementInterface` _hitactor "/Game/ElCortijo/Features/Interaction/BPI_Clickable.BPI_Clickable_C")
          (message `/Game/ElCortijo/Features/Interaction/BPI_Clickable.Click` _hitactor null)
          (bind _asbp_evidence (cast `/Game/ElCortijo/Features/Evidence/BP_Evidence` _hitactor))
          (set `self.MovingObject` _asbp_evidence))))))

(fn `LeftClickRelease`
  (bind _movingobject (`self.MovingObject`))
  (if (`KismetArrayLibrary.Array_IsNotEmpty` (`self.EvidenceObjectsInTable`))
    (if (!= _movingobject null)
      (if (`self.PlayerInTable`)
        (message `/Game/ElCortijo/Features/Interaction/BPI_Clickable.Release` _movingobject null)
        (set `self.MovingObject` null)))))

(fn `Remove ObjectFromGrid`
  (params (Cell :type "Vector2D Structure"))
  (locals (VIndex :type Integer))
  (bind _grid (`self.Grid`))
  (bind _gridsize_x (`KismetMathLibrary.BreakVector2D` (`self.GridSize`)))
  (bind _output_get (set `local.VIndex` (`KismetMathLibrary.FTrunc` (+ Cell_X (* (- Cell_Y 1.0) _gridsize_x)))))
  (bind _returnvalue (- _output_get 1))
  (bind (_output_posinarray _output_contains _output_correctcontainer _output_isvalid) (break `/Game/ElCortijo/Features/ModelBoard/Blueprint/S_Cell` (`|GetArrayItem` _grid _returnvalue)))
  (`KismetArrayLibrary.Array_Set` _grid _returnvalue (make `/Game/ElCortijo/Features/ModelBoard/Blueprint/S_Cell` (`KismetMathLibrary.MakeVector2D` Cell_X Cell_Y) null _output_correctcontainer _output_isvalid))
  (return))

(fn `RemoveEvidenceINHP`
  (params (index :type Integer))
  (bind _output (`|GetArrayItem` (`self.HintPlacementsRef`) index))
  (`|VariableSetRef` _output (make `/Game/ElCortijo/Features/ResearchTable/S_TablePlacements` (`.Placement_2_FD44286F48BEEE48D0811A9809672CC7` (break `/Game/ElCortijo/Features/ResearchTable/S_TablePlacements` _output)) null)))

(fn `SetEvidenceINHP`
  (params (BP_Evidence :type "/Game/ElCortijo/Features/Evidence/BP_Evidence Object Reference"))
  (returns (Placement :type "StaticMeshComponent Object Reference") (EmptySlot :type Integer))
  (bind (_slot _isroom) (`self.GetFirstEmptySlot`))
  (if _isroom
    (bind (_output_placement _output_evidence) (break `/Game/ElCortijo/Features/ResearchTable/S_TablePlacements` (`|GetArrayItem` (`self.HintPlacementsRef`) _slot)))
    (`|VariableSetRef` _output_evidence BP_Evidence)
    (return _output_placement _slot)))

(fn `SetVisor Pos`
  (params (Cell :type "Vector2D Structure") (`is Valid` :type Boolean))
  (if `is Valid`
    (bind _relative_pos (`self.Get Cell Relative Pos` Cell))
    (`SceneComponent.K2_SetRelativeLocation` (`self.Visor`) _relative_pos false false)))

(fn `UserConstructionScript`)