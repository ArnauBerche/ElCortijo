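; BP_HalfOpenDoor is an interactable door that opens, refuses with player dialogue, or gets slammed shut by a falling shelf.
; Interact toggles a rotation timeline with sound when unlocked and keyless; otherwise it calls CantOpen and shows key or locked dialogue, animating the door if locked.
; LockDoorEvent waits, stops the Box responding to a custom trace channel, then drops the shelf and shuts the door on one timeline, ending with a metal-break sound.
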(event `/Game/ElCortijo/Features/2_InteractionSystem/BPI_Interactable.Interact`
  (params (Interactor :type "Actor Object Reference"))
  (bind _doorroot (`self.DoorRoot`))
  (bind _sfx (`self.SFX`))
  (bind _sfx_2 (`self.SFX`))
  (bind (_relativerotation_roll _relativerotation_pitch) (`KismetMathLibrary.BreakRotator` (`SceneComponent.RelativeRotation` _doorroot)))
  (if (`self.IsUnlocked`)
    (if (`self.NeedsKey`)
      (bind _asbp_first_person_character (cast `/Game/ElCortijo/Features/1_MainCharacter/Blueprints/BP_FirstPersonCharacter` Interactor))
      (`/Game/ElCortijo/Features/1_MainCharacter/Blueprints/BP_FirstPersonCharacter.SetRealTimeDialogue` _asbp_first_person_character (`self.DialogueKEY`) 1.5)
      (`self.CantOpen`)
      (else
        (`/Engine/EditorBlueprintResources/StandardMacros.FlipFlop`
          (:`A`
            ; Visual
            (set `self.IsOpen` true)
            (`FMODAudioComponent.SetEvent` _sfx_2 "/Game/FMOD/Events/SFX/Objetos/SFX_24_PuertaAbrir.SFX_24_PuertaAbrir")
            (`FMODAudioComponent.Play` _sfx_2)
            (bind (_direction _doorrotationvalue) (`Timeline|Cronograma_0` :!label _label)
              (:`Update`
                (`SceneComponent.K2_SetRelativeRotation` (`self.DoorRoot`) (`KismetMathLibrary.MakeRotator` 0.0 0.0 _doorrotationvalue) false false))))
          (:`B`
            (set `self.IsOpen` false)
            (`FMODAudioComponent.SetEvent` _sfx "/Game/FMOD/Events/SFX/Objetos/SFX_24_PuertaAbrir.SFX_24_PuertaAbrir")
            (`FMODAudioComponent.Play` _sfx)
            (goto _label :!via `Reverse`)))))
    (else
      (`self.CantOpen`)
      (bind (_direction_2 _newtrack_0) (`Timeline|Cronograma_1` :!via `PlayFromStart`)
        (:`Update`
          (`SceneComponent.K2_SetRelativeRotation` _doorroot (`KismetMathLibrary.MakeRotator` _relativerotation_roll _relativerotation_pitch _newtrack_0) false false))
        (:`Finished`
          (bind _asbp_first_person_character_2 (cast `/Game/ElCortijo/Features/1_MainCharacter/Blueprints/BP_FirstPersonCharacter` Interactor))
          (`/Game/ElCortijo/Features/1_MainCharacter/Blueprints/BP_FirstPersonCharacter.SetRealTimeDialogue` _asbp_first_person_character_2 (`self.DialogueLOCKED`) 1.5))))))

(event `LockDoorEvent`
  (bind _sfx (`self.SFX`))
  (`KismetSystemLibrary.Delay` 5.0)
  (set `self.TempTransform` (`self.GetTransform` (`self.FallingShelf`)))
  (`PrimitiveComponent.SetCollisionResponseToChannel` (`self.Box`) "ECC_GameTraceChannel1" "ECR_Ignore")
  (bind (_direction _fall _doorshutting) (`Timeline|ShelfFall` :!via `PlayFromStart`)
    (:`Update`
      (`self.K2_SetActorRelativeTransform` (`self.FallingShelf`) (`KismetMathLibrary.TLerp` (`self.TempTransform`) (`KismetMathLibrary.MakeTransform` (-182.131734 690.993135 100.247562) (struct :`Pitch` 33.0 :`Roll` 60.0) (0.9 0.9 0.9)) _fall) false false)
      (`SceneComponent.K2_SetRelativeRotation` (`self.DoorRoot`) (`KismetMathLibrary.MakeRotator` 0.0 0.0 _doorshutting) false false))
    (:`Finished`
      (`FMODAudioComponent.SetEvent` _sfx "/Game/FMOD/Events/SFX/Objetos/SFX_29_MetalRoto.SFX_29_MetalRoto")
      (`FMODAudioComponent.SetVolume` _sfx 3.0)
      (`FMODAudioComponent.Play` _sfx))))

(fn `UserConstructionScript`
  (`parent.UserConstructionScript`))