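; Interactable door actor that opens and closes with animated yaw rotation and sound, or refuses when locked or needing a key.
; Interact toggles a timeline forward and in reverse through a FlipFlop, updating IsOpen.
; A key-required door plays a refusal sound and shows player dialogue; a locked one also animates its yaw before the dialogue.
; UnlockDoor and LockDoor set the lock state, while NeedsKey is only read here.
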(event `/Game/ElCortijo/Features/2_InteractionSystem/BPI_Interactable.Interact`
  (params (Interactor :type "Actor Object Reference"))
  (bind _doorroot (`self.DoorRoot`))
  (bind _sfx (`self.SFX`))
  (bind _sfx_2 (`self.SFX`))
  (bind (_relativerotation_roll _relativerotation_pitch) (`KismetMathLibrary.BreakRotator` (`SceneComponent.RelativeRotation` _doorroot)))
  (if (`self.IsUnlocked`)
    (if (`self.NeedsKey`)
      (bind _asbp_first_person_character (cast `/Game/ElCortijo/Features/1_MainCharacter/Blueprints/BP_FirstPersonCharacter` Interactor))
      (`/Game/ElCortijo/Features/1_MainCharacter/Blueprints/BP_FirstPersonCharacter.SetRealTimeDialogue` _asbp_first_person_character (`self.DialogueKEY`) 1.5)
      (`self.CantOpen`)
      (else
        (`/Engine/EditorBlueprintResources/StandardMacros.FlipFlop`
          (:`A`
            ; Visual
            (set `self.IsOpen` true)
            (`FMODAudioComponent.SetEvent` _sfx_2 "/Game/FMOD/Events/SFX/Objetos/SFX_24_PuertaAbrir.SFX_24_PuertaAbrir")
            (`FMODAudioComponent.Play` _sfx_2)
            (bind (_direction _doorrotationvalue) (`Timeline|Cronograma` :!label _label)
              (:`Update`
                (`SceneComponent.K2_SetRelativeRotation` (`self.DoorRoot`) (`KismetMathLibrary.MakeRotator` 0.0 0.0 _doorrotationvalue) false false))))
          (:`B`
            (set `self.IsOpen` false)
            (`FMODAudioComponent.SetEvent` _sfx "/Game/FMOD/Events/SFX/Objetos/SFX_25_PuertaCerrar.SFX_25_PuertaCerrar")
            (`FMODAudioComponent.Play` _sfx)
            (goto _label :!via `Reverse`)))))
    (else
      (`self.CantOpen`)
      (bind (_direction_2 _newtrack_0) (`Timeline|Timeline` :!via `PlayFromStart`)
        (:`Update`
          (`SceneComponent.K2_SetRelativeRotation` _doorroot (`KismetMathLibrary.MakeRotator` _relativerotation_roll _relativerotation_pitch _newtrack_0) false false))
        (:`Finished`
          (bind _asbp_first_person_character_2 (cast `/Game/ElCortijo/Features/1_MainCharacter/Blueprints/BP_FirstPersonCharacter` Interactor))
          (`/Game/ElCortijo/Features/1_MainCharacter/Blueprints/BP_FirstPersonCharacter.SetRealTimeDialogue` _asbp_first_person_character_2 (`self.DialogueLOCKED`) 1.5))))))

(fn `CantOpen`
  (bind _sfx (`self.SFX`))
  (`FMODAudioComponent.SetEvent` _sfx "/Game/FMOD/Events/SFX/Objetos/SFX_27_PuertaNoAbrir.SFX_27_PuertaNoAbrir")
  (`FMODAudioComponent.Play` _sfx))

(fn `LockDoor`
  (set `self.IsUnlocked` false))

(fn `PrintDialogue`
  (params (Dialogue :type String)))

(fn `UnlockDoor`
  (set `self.IsUnlocked` true))

(fn `UserConstructionScript`)