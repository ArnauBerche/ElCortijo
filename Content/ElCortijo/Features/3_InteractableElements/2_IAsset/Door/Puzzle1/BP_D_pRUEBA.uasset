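; Test door Blueprint (BP_D_pRUEBA) for Puzzle1 that slides open and closed along a spline when interacted with.
; Interact, gated by IsEnabled and AnimationEnded, toggles IsOpen and plays or reverses the Move timeline, lerping the root between spline endpoints.
; Hold and Release are empty; disconnected leftover logic covers strength-versus-weight dragging along the spline and note-dependent Spanish dialogue hints.
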(event `self.ReceiveTick`
  (params (DeltaSeconds :type "Float (single-precision)")))

(event `self.Interact`
  (params (Interactor :type "Actor Object Reference"))
  (bind _spline (`self.Spline`))
  (if (`self.IsEnabled`)
    (if (`self.AnimationEnded`)
      (set `self.AnimationEnded` false)
      (if (`self.IsOpen`)
        (set `self.IsOpen` false)
        (bind (_direction _newtrack_0) (`Timeline|Move` :!via `PlayFromStart` :!label _label)
          (:`Update`
            (bind (_returnvalue_x _returnvalue_y _returnvalue_z) (`KismetMathLibrary.BreakVector` (`KismetMathLibrary.VLerp` (`.Position` (break `SplinePoint` (`SplineComponent.GetSplinePointAt` _spline 0 "World"))) (`.Position` (break `SplinePoint` (`SplineComponent.GetSplinePointAt` _spline (`SplineComponent.GetNumberOfSplinePoints` _spline) "World"))) _newtrack_0)))
            (`SceneComponent.K2_SetWorldLocation` (`self.ROOT`) (`KismetMathLibrary.MakeVector` _returnvalue_x _returnvalue_y _returnvalue_z) false false))
          (:`Finished`
            (set `self.AnimationEnded` true)))
        (else
          (set `self.IsOpen` true)
          (goto _label :!via `ReverseFromEnd`))))))

(event `self.Hold`
  (params (Interactor :type "Actor Object Reference"))
  ;[0.15 0 0 0.5] Not in Use
)

(event `self.Release`
  ;[0.15 0 0 0.5] Not in Use
)

(fn `UserConstructionScript`)