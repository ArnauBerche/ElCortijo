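; BP_Door_Rect is an interactable door Blueprint that swings open and closed on Interact.
; A locked door prints its locked dialogue, and an unlocked one that still needs a key prints the key dialogue.
; Otherwise a FlipFlop toggles IsOpen and plays or reverses a Timeline that drives the yaw of DoorRoot.
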(event `/Game/ElCortijo/Features/2_InteractionSystem/BPI_Interactable.Interact`
  (params (Interactor :type "Actor Object Reference"))
  (if (`self.IsUnlocked`)
    (if (`self.NeedsKey`)
      (`self.PrintDialogue` (`self.DialogueKEY`))
      (else
        (`/Engine/EditorBlueprintResources/StandardMacros.FlipFlop`
          (:`A`
            ; Visual
            (set `self.IsOpen` true)
            (bind (_direction _doorrotationvalue) (`Timeline|Timeline` :!label _label)
              (:`Update`
                (`SceneComponent.K2_SetRelativeRotation` (`self.DoorRoot`) (`KismetMathLibrary.MakeRotator` 0.0 0.0 _doorrotationvalue) false false))))
          (:`B`
            (set `self.IsOpen` false)
            (goto _label :!via `Reverse`)))))
    (else
      (`self.PrintDialogue` (`self.DialogueLOCKED`)))))

(fn `UserConstructionScript`
  (`parent.UserConstructionScript`))