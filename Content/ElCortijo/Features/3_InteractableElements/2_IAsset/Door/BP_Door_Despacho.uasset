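; Office (Despacho) door interactable that also drives the "Capilla" mission through the GameInstance's MissionManager.
; The first interaction starts the mission, then every interaction checks lock and key state, printing dialogue if blocked.
; Otherwise a FlipFlop plays or reverses a Timeline that rotates DoorRoot to open or close it.
; The first time that Timeline finishes, the mission advances, guarded by HasOpened to run only once.
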(event `self.Interact`
  (params (Interactor :type "Actor Object Reference"))
  (if (not (`self.HasAdvanced`))
    (bind _asbp_game_instance (cast `/Game/ElCortijo/Features/0_Unsorted/GameInstance/BP_GameInstance` (`GameplayStatics.GetGameInstance`)))
    (`/Game/ElCortijo/Features/5_MissionSystem/BP_MissionManager.StartMission` (`/Game/ElCortijo/Features/0_Unsorted/GameInstance/BP_GameInstance.MissionManager` _asbp_game_instance) "Capilla" false)
    (set `self.HasAdvanced` true))
  (if (`self.IsUnlocked`)
    (if (`self.NeedsKey`)
      (`self.PrintDialogue` (`self.DialogueKEY`))
      (else
        (`/Engine/EditorBlueprintResources/StandardMacros.FlipFlop`
          (:`A`
            ; Visual
            (set `self.IsOpen` true)
            (bind (_direction _doorrotationvalue) (`Timeline|Timeline` :!label _label)
              (:`Update`
                (`SceneComponent.K2_SetRelativeRotation` (`self.DoorRoot`) (`KismetMathLibrary.MakeRotator` 0.0 0.0 _doorrotationvalue) false false))
              (:`Finished`
                (if (not (`self.HasOpened`))
                  (bind _asbp_game_instance_2 (cast `/Game/ElCortijo/Features/0_Unsorted/GameInstance/BP_GameInstance` (`GameplayStatics.GetGameInstance`)))
                  (`/Game/ElCortijo/Features/5_MissionSystem/BP_MissionManager.AdvanceMission` (`/Game/ElCortijo/Features/0_Unsorted/GameInstance/BP_GameInstance.MissionManager` _asbp_game_instance_2) "Capilla" false)
                  (set `self.HasOpened` true)))))
          (:`B`
            (set `self.IsOpen` false)
            (goto _label :!via `Reverse`)))))
    (else
      (`self.PrintDialogue` (`self.DialogueLOCKED`)))))

(fn `UserConstructionScript`
  (`parent.UserConstructionScript`))