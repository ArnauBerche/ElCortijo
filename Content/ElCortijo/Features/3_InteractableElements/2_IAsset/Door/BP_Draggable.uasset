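; BP_Draggable is an interactable object that the first-person character drags back and forth along a spline.
; While held, it traces from the player's view and moves only when the impact point leaves its Box bounds.
; The nearer of two track markers sets the direction; step size scales with pull distance and the strength-to-weight ratio.
; Travel is checked against zero and the straight-line distance between spline endpoints, and each move prints the current distance.
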(event `self.ReceiveTick`
  (params (DeltaSeconds :type "Float (single-precision)")))

(event `/Game/ElCortijo/Features/2_InteractionSystem/BPI_Movable.Hold`
  (params (Interactor :type "Actor Object Reference"))
  (bind _currentdistance (`self.CurrentDistance`))
  (bind _box (`self.Box`))
  (bind _impact_point (`self.Impact Point`))
  (bind _spline (`self.Spline`))
  (bind _currentdistance_2 (`self.CurrentDistance`))
  (bind _returnvalue_location (`KismetMathLibrary.BreakTransform` (`SplineComponent.GetTransformAtDistanceAlongSpline` (`self.Spline`) (`self.CurrentDistance`) "World" false)))
  (bind _returnvalue (* (/ (`self.CharacterStrenght`) (`self.ObjectWeight`)) (`KismetMathLibrary.Vector_Distance` (`self.Impact Point`) (`SceneComponent.K2_GetComponentLocation` (`self.ROOT`)))))
  (if (`self.IsEnabled`)
    (bind _asbp_first_person_character (cast `/Game/ElCortijo/Features/1_MainCharacter/Blueprints/BP_FirstPersonCharacter` Interactor))
    (bind (_hit _impactpoint) (`/Game/ElCortijo/Features/1_MainCharacter/Blueprints/BP_FirstPersonCharacter.RayCastForwardLocation` _asbp_first_person_character "TraceTypeQuery1"))
    (bind _output_get (set `self.Impact Point` _impactpoint))
    (if (`self.IsHolding`)
      (if (not (and (and (<= (`KismetMathLibrary.Abs` (.x (`KismetMathLibrary.InverseTransformLocation` (`SceneComponent.K2_GetComponentToWorld` _box) (`self.Impact Point`)))) (.x (`BoxComponent.GetScaledBoxExtent` _box))) (<= (`KismetMathLibrary.Abs` (.y (`KismetMathLibrary.InverseTransformLocation` (`SceneComponent.K2_GetComponentToWorld` _box) (`self.Impact Point`)))) (.y (`BoxComponent.GetScaledBoxExtent` _box)))) (<= (`KismetMathLibrary.Abs` (.z (`KismetMathLibrary.InverseTransformLocation` (`SceneComponent.K2_GetComponentToWorld` _box) (`self.Impact Point`)))) (.z (`BoxComponent.GetScaledBoxExtent` _box)))))
        (if (< (`KismetMathLibrary.Vector_Distance` _impact_point (`SceneComponent.K2_GetComponentLocation` (`self.Behinf_Track`))) (`KismetMathLibrary.Vector_Distance` _impact_point (`SceneComponent.K2_GetComponentLocation` (`self.Ahead_Track`))))
          (if (> _currentdistance_2 0.0)
            ; Back
            (set `self.CurrentDistance` (- _currentdistance _returnvalue))
            (`SceneComponent.K2_SetWorldLocation` (`self.ROOT`) _returnvalue_location false false :!label _label)
            (`KismetSystemLibrary.PrintString` (`KismetStringLibrary.Conv_DoubleToString` (`self.CurrentDistance`))))
          (elif (< _currentdistance_2 (`KismetMathLibrary.Vector_Distance` (`.Position` (break `SplinePoint` (`SplineComponent.GetSplinePointAt` _spline 0 "World"))) (`.Position` (break `SplinePoint` (`SplineComponent.GetSplinePointAt` _spline (`SplineComponent.GetNumberOfSplinePoints` _spline) "World")))))
            ; Forward
            (set `self.CurrentDistance` (+ _currentdistance _returnvalue))
            (goto _label))))
      (else
        (set `self.FirstHit` _output_get)
        (set `self.IsHolding` true)))))

(event `/Game/ElCortijo/Features/2_InteractionSystem/BPI_Movable.Release`
  (if (`self.IsEnabled`)
    (set `self.IsHolding` false)))

(fn `UserConstructionScript`)