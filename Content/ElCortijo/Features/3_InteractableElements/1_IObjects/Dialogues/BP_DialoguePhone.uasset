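; BP_DialoguePhone is an interactable phone that rings when the player approaches and offers a dialogue.
; A one-shot RingTrigger overlap plays the ring sound, shows a timed on-screen interaction hint, then destroys itself.
; Interacting runs the parent logic, stops the ring and clears the hint.
; Dialogue component start and end events swap the PhoneModel mesh between open and closed.
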(event `self.ReceiveBeginPlay`
  (bind _bp_dialoguecomponent (`self.BP_DialogueComponent`))
  (`parent.ReceiveBeginPlay`)
  (add `/Game/ElCortijo/Features/3_InteractableElements/1_IObjects/Dialogues/BP_DialogueComponent.OnDialogueStarted` _bp_dialoguecomponent (delegate `OpenPhone`))
  (add `/Game/ElCortijo/Features/3_InteractableElements/1_IObjects/Dialogues/BP_DialogueComponent.OnDialogueEnded` _bp_dialoguecomponent (delegate `ClosePhone`)))

(event `OpenPhone`
  (params (Dialogue :type "/Game/ElCortijo/Features/3_InteractableElements/1_IObjects/Dialogues/S_Dialogue Structure"))
  (`StaticMeshComponent.SetStaticMesh` (`StaticMeshActor.StaticMeshComponent` (`self.PhoneModel`)) "/Game/ElCortijo/Features/Props/Interior/Despacho/Telefono/SM_TelefonoAbierto.SM_TelefonoAbierto"))

(event `ClosePhone`
  (`StaticMeshComponent.SetStaticMesh` (`StaticMeshActor.StaticMeshComponent` (`self.PhoneModel`)) "/Game/ElCortijo/Features/Props/Interior/Despacho/Telefono/SM_TelefonoCerrado.SM_TelefonoCerrado"))

(event `self.RingTrigger.OnComponentBeginOverlap`
  (params (OverlappedComponent :type "PrimitiveComponent Object Reference") (OtherActor :type "Actor Object Reference") (OtherComp :type "PrimitiveComponent Object Reference") (OtherBodyIndex :type Integer) (bFromSweep :type Boolean) (SweepResult :type "HitResult Structure (by ref)"))
  (bind _asbp_first_person_character (cast `/Game/ElCortijo/Features/1_MainCharacter/Blueprints/BP_FirstPersonCharacter` OtherActor))
  (`/Game/ElCortijo/Features/1_MainCharacter/Blueprints/BP_FirstPersonCharacter.SetRealTimeDialogue` _asbp_first_person_character "(Suena el teléfono) \nAcércate para interactuar (E o Click Izquierdo)" 3.0)
  (`/Game/ElCortijo/Features/7_AudioSystem/Blueprint/BP_SoundComponent.PlayWithSound` (`self.BP_SoundComponent`) "/Game/ElCortijo/Features/7_AudioSystem/Sound/SFX/General/SFX_Telefono.SFX_Telefono")
  (`ActorComponent.K2_DestroyComponent` (`self.RingTrigger`)))

(event `/Game/ElCortijo/Features/2_InteractionSystem/BPI_Interactable.Interact`
  (params (Interactor :type "Actor Object Reference"))
  (`parent.Interact` Interactor)
  (`/Game/ElCortijo/Features/7_AudioSystem/Blueprint/BP_SoundComponent.Stop` (`self.BP_SoundComponent`))
  (bind _asbp_first_person_character (cast `/Game/ElCortijo/Features/1_MainCharacter/Blueprints/BP_FirstPersonCharacter` (`GameplayStatics.GetPlayerCharacter` 0)))
  (`/Game/ElCortijo/Features/1_MainCharacter/Blueprints/BP_FirstPersonCharacter.ResetRealTimeDialogue` _asbp_first_person_character))

(fn `UserConstructionScript`
  (`parent.UserConstructionScript`))