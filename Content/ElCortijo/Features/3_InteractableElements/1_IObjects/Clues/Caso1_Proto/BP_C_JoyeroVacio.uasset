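; BP_C_JoyeroVacio is an interactable empty jewelry box clue for the Caso1 prototype.
; On its first interaction, after calling the parent logic, it adds its evidence to the Table and marks itself as interacted.
; It then searches its attached actors recursively for BP_BillBoard markers, hiding each one and disabling the Collision component inside that loop.
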(event `/Game/ElCortijo/Features/2_InteractionSystem/BPI_Interactable.Interact`
  (params (Interactor :type "Actor Object Reference"))
  (`parent.Interact` Interactor)
  (if (not (`self.Interacted`))
    (`/Game/ElCortijo/Features/4_InteractableTables/ModelBoard/Blueprint/BP_ModelBoardV2.AddNewOBJEvidence` (`self.Table`) (`self.Evidence`))
    (set `self.Interacted` true)
    (for _array_element (`self.GetAttachedActors` true true)
      (bind _asbp_bill_board (cast `/Game/ElCortijo/Features/0_Unsorted/BP_BillBoard` _array_element))
      (`SceneComponent.SetVisibility` (`/Game/ElCortijo/Features/0_Unsorted/BP_BillBoard.Scene` _asbp_bill_board) false true)
      (`PrimitiveComponent.SetCollisionEnabled` (`self.Collision`) "NoCollision"))))

(fn `UserConstructionScript`
  (`parent.UserConstructionScript`))