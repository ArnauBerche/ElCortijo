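; Phone photo clue for the Case 1 prototype that advances a mission once all its hotspots are consumed.
; It overrides OnAllHotspotsConsumed, runs the parent logic, then tells the MissionManager on BP_GameInstance to advance the Pruebas3 mission with audio.
; All other behavior comes from the parent class, as the event graph holds only disabled placeholder events.
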(fn `OnAllHotspotsConsumed`
  (`parent.OnAllHotspotsConsumed`)
  (bind _asbp_game_instance (cast `/Game/ElCortijo/Features/0_Unsorted/GameInstance/BP_GameInstance` (`GameplayStatics.GetGameInstance`)))
  (`/Game/ElCortijo/Features/5_MissionSystem/BP_MissionManager.AdvanceMission` (`/Game/ElCortijo/Features/0_Unsorted/GameInstance/BP_GameInstance.MissionManager` _asbp_game_instance) "Pruebas3" true))

(fn `UserConstructionScript`
  (`parent.UserConstructionScript`))