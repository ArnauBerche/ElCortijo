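; BP_C_Taza is an interactable cup clue object for the Caso1_Proto case.
; Interact runs the parent behavior, then on the first use shows a brief control hint (Q to drop, R to investigate) through the first-person character's real-time dialogue.
; A TakenOnce flag keeps the hint from repeating; BeginPlay, overlap and Tick are disabled stubs.
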(event `/Game/ElCortijo/Features/2_InteractionSystem/BPI_Interactable.Interact`
  (params (Interactor :type "Actor Object Reference"))
  (`parent.Interact` Interactor)
  (if (not (`self.TakenOnce`))
    (bind _asbp_first_person_character (cast `/Game/ElCortijo/Features/1_MainCharacter/Blueprints/BP_FirstPersonCharacter` (`GameplayStatics.GetPlayerCharacter` 0)))
    (`/Game/ElCortijo/Features/1_MainCharacter/Blueprints/BP_FirstPersonCharacter.SetRealTimeDialogue` _asbp_first_person_character "Q: Soltar objeto \nR: Investigar objeto" 3.0)
    (set `self.TakenOnce` true)))

(fn `UserConstructionScript`
  (`parent.UserConstructionScript`))