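; Clue object for the Case 1 prototype, a simple personal report that drives progress of the "Prueba1" mission.
; On its first placement on a table it advances that mission with audio through the GameInstance's MissionManager, using a flag to prevent repeats.
; When all its hotspots are consumed, it advances the same mission again without audio, with no repeat guard of its own.
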(event `self.ReceiveTick`
  (params (DeltaSeconds :type "Float (single-precision)"))
  (`parent.ReceiveTick` DeltaSeconds))

(fn `OnAllHotspotsConsumed`
  (bind _asbp_game_instance (cast `/Game/ElCortijo/Features/0_Unsorted/GameInstance/BP_GameInstance` (`GameplayStatics.GetGameInstance`)))
  (`/Game/ElCortijo/Features/5_MissionSystem/BP_MissionManager.AdvanceMission` (`/Game/ElCortijo/Features/0_Unsorted/GameInstance/BP_GameInstance.MissionManager` _asbp_game_instance) "Prueba1" false))

(fn `OnPlacedOnTable`
  (params (Table :type "/Game/ElCortijo/Features/4_InteratableTables/ResearchTable/Blueprint/BP_ResearchTable Object Reference"))
  (`parent.OnPlacedOnTable` Table)
  (if (not (`self.hasGeneratedMission`))
    (bind _asbp_game_instance (cast `/Game/ElCortijo/Features/0_Unsorted/GameInstance/BP_GameInstance` (`GameplayStatics.GetGameInstance`)))
    (`/Game/ElCortijo/Features/5_MissionSystem/BP_MissionManager.AdvanceMission` (`/Game/ElCortijo/Features/0_Unsorted/GameInstance/BP_GameInstance.MissionManager` _asbp_game_instance) "Prueba1" true)
    (set `self.hasGeneratedMission` true)))

(fn `UserConstructionScript`
  (`parent.UserConstructionScript`))