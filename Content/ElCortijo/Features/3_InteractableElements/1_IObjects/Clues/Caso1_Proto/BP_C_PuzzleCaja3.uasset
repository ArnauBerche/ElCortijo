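; Interactable clue for the third puzzle box in the Case 1 prototype, extending its parent's Interact behavior.
; Until flagged as interacted, it calls CheckForAdd on a linked note and sets that flag only if the first-person game mode reports that a camera is held.
; A door lock call is left unconnected and never runs.
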(event `/Game/ElCortijo/Features/2_InteractionSystem/BPI_Interactable.Interact`
  (params (Interactor :type "Actor Object Reference"))
  (`parent.Interact` Interactor)
  (if (not (`self.Interacted`))
    (bind _asbp_first_person_game_mode (cast `/Game/ElCortijo/Features/1_MainCharacter/Blueprints/BP_FirstPersonGameMode` (`GameplayStatics.GetGameMode`)))
    (if (`/Game/ElCortijo/Features/1_MainCharacter/Blueprints/BP_FirstPersonGameMode.HasCamera` _asbp_first_person_game_mode)
      (set `self.Interacted` true))
    (`/Game/ElCortijo/Features/3_InteractableElements/1_IObjects/Clues/Caso1_Proto/BP_C_PuzzleCaja2.CheckForAdd` (`self.OtherNote`))))

(fn `UserConstructionScript`
  (`parent.UserConstructionScript`))