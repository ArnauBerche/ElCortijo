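; Interactable pistol clue for the Case 1 prototype, which adds its evidence to the Table the first time the player interacts with it.
; If the Table's first notes are not enabled, it shows a dialogue line about following Pedro's instructions instead.
; On collection, it starts the "Maqueta" mission if the bullet-holes clue was already interacted with, otherwise advances "Patio".
; It then loops through attached actors to hide billboards and disable the object's collision.
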(event `/Game/ElCortijo/Features/2_InteractionSystem/BPI_Interactable.Interact`
  (params (Interactor :type "Actor Object Reference"))
  (`parent.Interact` Interactor)
  (if (`/Game/ElCortijo/Features/4_InteractableTables/ModelBoard/Blueprint/BP_ModelBoardV2.AreFirstNotesEnabled` (`self.Table`))
    (if (not (`self.Interacted`))
      (`/Game/ElCortijo/Features/4_InteractableTables/ModelBoard/Blueprint/BP_ModelBoardV2.AddNewOBJEvidence` (`self.Table`) (`self.Evidence`))
      (set `self.Interacted` true)
      (`|ExecutionSequence`
        (:`then_0`
          (bind _returnvalue (`GameplayStatics.GetActorOfClass` "/Game/ElCortijo/Features/3_InteractableElements/1_IObjects/Clues/Caso1_Proto/BP_C_AgujerosDeBala_Especifico.BP_C_AgujerosDeBala_Especifico_C"))
          (if (`/Game/ElCortijo/Features/3_InteractableElements/1_IObjects/Clues/Caso1_Proto/BP_C_AgujerosDeBala_Especifico.Interacted` _returnvalue)
            (bind _asbp_first_person_game_mode (cast `/Game/ElCortijo/Features/1_MainCharacter/Blueprints/BP_FirstPersonGameMode` (`GameplayStatics.GetGameMode`)))
            (`/Game/ElCortijo/Features/5_MissionSystem/BP_MissionManager.StartMission` (`/Game/ElCortijo/Features/1_MainCharacter/Blueprints/BP_FirstPersonGameMode.MissionManager` _asbp_first_person_game_mode) "Maqueta" false)
            (else
              (bind _asbp_first_person_game_mode_2 (cast `/Game/ElCortijo/Features/1_MainCharacter/Blueprints/BP_FirstPersonGameMode` (`GameplayStatics.GetGameMode`)))
              (`/Game/ElCortijo/Features/5_MissionSystem/BP_MissionManager.AdvanceMission` (`/Game/ElCortijo/Features/1_MainCharacter/Blueprints/BP_FirstPersonGameMode.MissionManager` _asbp_first_person_game_mode_2) "Patio" false))))
        (:`then_1`
          (for _array_element (`self.GetAttachedActors` true true)
            (bind _asbp_bill_board (cast `/Game/ElCortijo/Features/0_Unsorted/BP_BillBoard` _array_element))
            (`SceneComponent.SetVisibility` (`/Game/ElCortijo/Features/0_Unsorted/BP_BillBoard.Scene` _asbp_bill_board) false true)
            (`PrimitiveComponent.SetCollisionEnabled` (`self.Object`) "NoCollision")))))
    (else
      (bind _asbp_first_person_character (cast `/Game/ElCortijo/Features/1_MainCharacter/Blueprints/BP_FirstPersonCharacter` (`GameplayStatics.GetPlayerCharacter` 0)))
      (`/Game/ElCortijo/Features/1_MainCharacter/Blueprints/BP_FirstPersonCharacter.SetRealTimeDialogue` _asbp_first_person_character "Primero debería seguir las intrucciones de Pedro." 3.0))))

(fn `UserConstructionScript`
  (`parent.UserConstructionScript`))