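; BP_ClueHotspot is a clickable hotspot belonging to a clue, which creates evidence on the research table holding that clue.
; Its owner and evidence data are set on initialization, and Active and Consumed states toggle the collider and decal.
; While available, Tick traces under the cursor and drives the decal's dynamic material Strength higher as the cursor nears.
; A click requests evidence creation from BP_ResearchTable and consumes the hotspot if the clue is placed there.
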(event `self.ReceiveBeginPlay`
  (bind _returnvalue (`DecalComponent.CreateDynamicMaterialInstance` (`self.Decal`)))
  (set `self.DecalMID` _returnvalue))

(event `self.ReceiveTick`
  (params (DeltaSeconds :type "Float (single-precision)"))
  (bind (_hitresult _returnvalue) (`PlayerController.GetHitResultUnderCursorByChannel` (`GameplayStatics.GetPlayerController` 0) "TraceTypeQuery1" true))
  (if (and (`self.bActive`) (not (`self.bConsumed`)))
    (if _returnvalue
      (`self.DecalMouseStrength` (`.Location` (`GameplayStatics.BreakHitResult` _hitresult))))))

(event `/Game/ElCortijo/Features/2_InteractionSystem/BPI_Clickable.Click`
  (params (Interactor :type "Actor Object Reference"))
  (if (and (`self.bActive`) (not (`self.bConsumed`)))
    (`self.RequestCreateEvidence` (`self.EvidenceData`))))

(fn `DecalMouseStrength`
  (params (MousePos :type "Vector Structure"))
  (locals (MaxRange :type "Float (double-precision)" :default 500.0))
  (`MaterialInstanceDynamic.SetScalarParameterValue` (`self.DecalMID`) "Strength" (`KismetMathLibrary.MapRangeClamped` (`KismetMathLibrary.Vector_Distance` MousePos (`SceneComponent.K2_GetComponentLocation` (`self.Collider`))) 2.0 10.0 1.0)))

(fn `Initialize`
  (params (Owner :type "/Game/ElCortijo/Features/3_InteractableElements/1_IObjects/Clues/ClueHotspot/BP_ClueItem Object Reference") (Evidence :type "/Game/ElCortijo/Features/3_InteractableElements/1_IObjects/WorldElements/S_Note Structure"))
  (set `self.OwnerClue` Owner)
  (set `self.EvidenceData` Evidence)
  (`self.SetConsumed` false)
  (`self.SetActive` false))

(fn `RequestCreateEvidence`
  (params (Evidence :type "/Game/ElCortijo/Features/3_InteractableElements/1_IObjects/WorldElements/S_Note Structure"))
  (bind _ownerclue (`self.OwnerClue`))
  (bind _currenttable (`/Game/ElCortijo/Features/3_InteractableElements/1_IObjects/Clues/ClueHotspot/BP_ClueItem.CurrentTable` _ownerclue))
  (if (`self.bConsumed`)
    _
    (elif (and (and (!= _ownerclue null) (`/Game/ElCortijo/Features/3_InteractableElements/1_IObjects/Clues/ClueHotspot/BP_ClueItem.bPlacedOnResearchTable` _ownerclue)) (!= _currenttable null))
      (bind _asbp_research_table (cast `/Game/ElCortijo/Features/4_InteractableTables/ResearchTable/Blueprint/BP_ResearchTable` _currenttable))
      (`/Game/ElCortijo/Features/4_InteractableTables/ResearchTable/Blueprint/BP_ResearchTable.CreateEvidence` _asbp_research_table Evidence)
      (`self.SetConsumed` true))))

(fn `SetActive`
  (params (bActive :type Boolean))
  (bind _collider (`self.Collider`))
  (bind _output_get (set `self.bActive` bActive))
  (bind _returnvalue (and _output_get (not (`self.bConsumed`))))
  (if _returnvalue
    (`PrimitiveComponent.SetCollisionEnabled` _collider "QueryOnly")
    (else
      (`PrimitiveComponent.SetCollisionEnabled` _collider "NoCollision")))
  (`SceneComponent.SetHiddenInGame` (`self.Decal`) (not _returnvalue) false))

(fn `SetConsumed`
  (params (bConsumed :type Boolean))
  (bind _output_get (set `self.bConsumed` bConsumed))
  (if _output_get
    (`self.SetActive` false)))

(fn `UserConstructionScript`)