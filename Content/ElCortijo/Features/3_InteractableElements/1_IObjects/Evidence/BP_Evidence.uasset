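; BP_Evidence is an interactable evidence item that the player picks up and that can be registered as placed on a table.
; It holds assigned notes up to the number of correct ones and supports removing them.
; Its answer check requires equal counts and matches notes regardless of order, using the GameInstance's CompareNotes.
; Clickability is toggled through the collision response on a custom trace channel.
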(event `self.ReceiveBeginPlay`
  (bind _asbp_game_instance (cast `/Game/ElCortijo/Features/0_Unsorted/GameInstance/BP_GameInstance` (`GameplayStatics.GetGameInstance`)))
  (set `self.Game Instance` _asbp_game_instance)
  (`parent.ReceiveBeginPlay`))

(event `self.ReceiveTick`
  (params (DeltaSeconds :type "Float (single-precision)"))
  (`parent.ReceiveTick` DeltaSeconds))

(event `/Game/ElCortijo/Features/2_InteractionSystem/BPI_Interactable.Interact`
  (params (Interactor :type "Actor Object Reference"))
  (`self.PickUp` (`GameplayStatics.GetPlayerCharacter` 0)))

(fn `AddCurrentNote`
  (params (S_Note :type "/Game/ElCortijo/Features/3_InteractableElements/1_IObjects/WorldElements/S_Note Structure"))
  (returns (CorrectlyAdded :type Boolean))
  (locals (CanFit :type Boolean :default true))
  (bind _output_get (set `local.CanFit` (< (`KismetArrayLibrary.Array_Length` (`self.CurrentNotes`)) (`KismetArrayLibrary.Array_Length` (`self.CorrectNotes`)))))
  (if _output_get
    (`KismetArrayLibrary.Array_Add` (`self.CurrentNotes`) S_Note))
  (return (`local.CorrectlyAdded`)))

(fn `CheckCorrectNotes`
  (returns (isCorrect :type Boolean))
  (locals (AllCorrect :type Boolean :default false) (CorrectAmount :type Integer) (`1Correct` :type Boolean))
  (if (== (`KismetArrayLibrary.Array_Length` (`self.CorrectNotes`)) (`KismetArrayLibrary.Array_Length` (`self.CurrentNotes`)))
    (set `local.1Correct` false)
    (for _array_element (`self.CurrentNotes`)
      (for _array_element_2 (`self.CorrectNotes`)
        (bind _isequal (`/Game/ElCortijo/Features/0_Unsorted/GameInstance/BP_GameInstance.CompareNotes` (`self.Game Instance`) _array_element_2 _array_element))
        (if _isequal
          (set `local.1Correct` true)))
      (if (`local.1Correct`)
        (set `local.1Correct` false)
        (else
          (set `local.AllCorrect` false :!label _label)
          (return (`local.AllCorrect`)))))
    (set `local.AllCorrect` true)
    (else
      (goto _label)))
  (return (`local.AllCorrect`)))

(fn `RemoveNote`
  (params (Note :type "/Game/ElCortijo/Features/3_InteractableElements/1_IObjects/WorldElements/S_Note Structure"))
  (bind _currentnotes (`self.CurrentNotes`))
  (for _array_element _currentnotes
    (bind _isequal (`/Game/ElCortijo/Features/0_Unsorted/GameInstance/BP_GameInstance.CompareNotes` (`self.Game Instance`) Note _array_element))
    (if _isequal
      (`KismetArrayLibrary.Array_RemoveItem` _currentnotes _array_element))))

(fn `SetClickable`
  (params (Enabled :type Boolean))
  (bind _collision (`self.Collision`))
  (if Enabled
    (`PrimitiveComponent.SetCollisionResponseToChannel` _collision "ECC_GameTraceChannel3" "ECR_Block")
    (else
      (`PrimitiveComponent.SetCollisionResponseToChannel` _collision "ECC_GameTraceChannel3" "ECR_Ignore"))))

(fn `SetTable`
  (params (Table :type "/Game/ElCortijo/Features/4_InteractableTables/BP_Table Object Reference"))
  (set `self.CurrentTable` Table)
  (set `self.bIsOnTable` true))

(fn `UserConstructionScript`
  (`parent.UserConstructionScript`))