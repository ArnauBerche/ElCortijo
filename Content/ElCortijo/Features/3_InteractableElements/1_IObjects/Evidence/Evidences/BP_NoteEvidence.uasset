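; BP_NoteEvidence is a note-type evidence Blueprint that shows its written text in the world through a text render component.
; On BeginPlay it sets its evidence type enum, writes its Text variable to the TextRender, then calls the parent BeginPlay.
; All other behavior is left to the parent class, as the Tick and overlap events are disabled and the construction script only calls the parent.
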(event `self.ReceiveBeginPlay`
  (set `self.EType` "NewEnumerator1")
  (`TextRenderComponent.K2_SetText` (`self.TextRender`) (`KismetTextLibrary.Conv_StringToText` (`self.Text`)))
  (`parent.ReceiveBeginPlay`))

(fn `UserConstructionScript`
  (`parent.UserConstructionScript`))