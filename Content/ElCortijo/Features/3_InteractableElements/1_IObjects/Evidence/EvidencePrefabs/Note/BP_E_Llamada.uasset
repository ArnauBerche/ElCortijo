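; BP_E_Llamada is an evidence prefab in the Note group of interactable elements, representing the "Llamada" (call) clue.
; On BeginPlay it sets its evidence type, Id and text, then calls the parent BeginPlay.
; It adds no other logic: the construction script defers to the parent, and the overlap and Tick events are disabled stubs.
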(event `self.ReceiveBeginPlay`
  (set `self.EType` "NewEnumerator1")
  (set `self.Id` (`self.Id_0`))
  (set `self.Text` (`self.Text_0`))
  (`parent.ReceiveBeginPlay`))

(fn `UserConstructionScript`
  (`parent.UserConstructionScript`))