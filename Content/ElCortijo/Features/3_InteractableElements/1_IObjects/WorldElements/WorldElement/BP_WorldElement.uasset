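; BP_WorldElement is a clickable world element that adds its Note to the game instance when the player has the camera.
; SetActive toggles collider collision, while EnableUI shows the icon and sets the CorrectDistance flag that Click requires.
; Tick turns the icon widget toward the player camera while enabled.
; A successful click consumes the element permanently, disabling its collision and hiding the icon.
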(event `self.ReceiveTick`
  (params (DeltaSeconds :type "Float (single-precision)"))
  (bind _iconwidget (`self.IconWidget`))
  (if (`self.IsEnabled`)
    (`SceneComponent.K2_SetWorldRotation` _iconwidget (`KismetMathLibrary.FindLookAtRotation` (`SceneComponent.K2_GetComponentLocation` _iconwidget) (`PlayerCameraManager.GetCameraLocation` (`GameplayStatics.GetPlayerCameraManager` 0))) false false)))

(event `self.ReceiveBeginPlay`
  (bind _returnvalue (`DecalComponent.CreateDynamicMaterialInstance` (`self.Decal`)))
  (set `self.DecalMID` _returnvalue))

(event `/Game/ElCortijo/Features/2_InteractionSystem/BPI_Clickable.Click`
  (params (Interactor :type "Actor Object Reference"))
  (if (and (and (`self.IsEnabled`) (not (`self.Consumed`))) (`self.CorrectDistance`))
    (bind _asbp_game_instance (cast `/Game/ElCortijo/Features/0_Unsorted/GameInstance/BP_GameInstance` (`GameplayStatics.GetGameInstance`)))
    (if (`/Game/ElCortijo/Features/0_Unsorted/GameInstance/BP_GameInstance.HasCamera` _asbp_game_instance)
      (`/Game/ElCortijo/Features/0_Unsorted/GameInstance/BP_GameInstance.AddNote` _asbp_game_instance (`self.Note`))
      (set `self.Consumed` true)
      (`self.SetActive` false))))

(fn `EnableUI`
  (params (Enable :type Boolean))
  (`SceneComponent.SetHiddenInGame` (`self.IconWidget`) (not Enable) false)
  (set `self.CorrectDistance` Enable))

(fn `SetActive`
  (params (Enable :type Boolean))
  (bind _collider (`self.Collider`))
  (bind _output_get (set `self.IsEnabled` Enable))
  (if (and _output_get (not (`self.Consumed`)))
    (`PrimitiveComponent.SetCollisionEnabled` _collider "QueryOnly")
    (else
      (`PrimitiveComponent.SetCollisionEnabled` _collider "NoCollision")
      (`self.EnableUI` false))))

(fn `UserConstructionScript`)