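; BP_SoundComponent is an audio component that gives its owning actor sound playback through a separate proxy actor.
; On BeginPlay it spawns the proxy with the configured sound, looping and initial volume, then attaches it to the owner's root.
; Its events forward playback, sound, volume, pitch and fade calls to the proxy, and a function returns the sound's duration.
; EndPlay calls a short fade-out followed immediately by Stop.
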(event `self.ReceiveEndPlay`
  (params (EndPlayReason :type "EEndPlayReason Enum" :default "Destroyed"))
  (if (!= (`self.ProxyRef`) null)
    (`self.FadeOut` 0.1)
    (`self.Stop`)))

(event `self.ReceiveBeginPlay`
  (if (== (`self.ProxyRef`) null)
    (bind _output_get (set `self.Owner` (`self.GetOwner`)))
    (bind _returnvalue (`|SpawnActorFromClass` (`self.ProxyClass`) (`Actor.GetTransform` _output_get) "Undefined" "MultiplyWithRoot" null (`self.Looping`) (`self.InitialVolume`) (`self.Sound`) null))
    (bind _output_get_2 (set `self.ProxyRef` _returnvalue))
    (`Actor.K2_AttachToComponent` _output_get_2 (`Actor.RootComponent` (`self.GetOwner`)) "None" "KeepRelative" "KeepRelative" "KeepRelative" true)))

(event `Play`
  (`/Game/ElCortijo/Features/7_AudioSystem/Blueprint/BP_SoundEmitter.PlaySound` (`self.ProxyRef`)))

(event `Stop`
  (`/Game/ElCortijo/Features/7_AudioSystem/Blueprint/BP_SoundEmitter.StopSound` (`self.ProxyRef`)))

(event `SetVolume`
  (params (Volume :type "Float (double-precision)"))
  (`/Game/ElCortijo/Features/7_AudioSystem/Blueprint/BP_SoundEmitter.SetVolume` (`self.ProxyRef`) Volume))

(event `SetPitch`
  (params (Pitch :type "Float (double-precision)"))
  (`/Game/ElCortijo/Features/7_AudioSystem/Blueprint/BP_SoundEmitter.SetPitch` (`self.ProxyRef`) Pitch))

(event `PlayWithSound`
  (params (Sound :type "SoundBase Object Reference"))
  (`/Game/ElCortijo/Features/7_AudioSystem/Blueprint/BP_SoundEmitter.SetSoundAndPlay` (`self.ProxyRef`) Sound))

(event `SetSound`
  (params (Sound :type "SoundBase Object Reference"))
  (`/Game/ElCortijo/Features/7_AudioSystem/Blueprint/BP_SoundEmitter.SetSound` (`self.ProxyRef`) Sound))

(event `FadeIn`
  (params (Duration :type "Float (double-precision)") (TargetVolume :type "Float (double-precision)"))
  (`/Game/ElCortijo/Features/7_AudioSystem/Blueprint/BP_SoundEmitter.FadeIn` (`self.ProxyRef`) Duration TargetVolume))

(event `FadeOut`
  (params (Duration :type "Float (double-precision)"))
  (`/Game/ElCortijo/Features/7_AudioSystem/Blueprint/BP_SoundEmitter.FadeOut` (`self.ProxyRef`) Duration))

(fn `GetAudioDuration`
  (returns (Float :type "Float (double-precision)"))
  (return (`SoundBase.Duration` (`AudioComponent.Sound` (`/Game/ElCortijo/Features/7_AudioSystem/Blueprint/BP_SoundEmitter.Audio` (`self.ProxyRef`))))))