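; BP_SoundEmitter is an audio emitter Blueprint in the audio system that wraps an Audio component behind a simple control interface.
; Its functions set, play and stop a sound, including a combined set-and-play call, and adjust fades, volume and pitch by forwarding directly to that component.
; It has no active event logic, so playback is driven entirely by calls to these functions.
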(event `self.ReceiveBeginPlay`)

(fn `FadeIn`
  (params (Duration :type "Float (double-precision)") (TargetVolume :type "Float (double-precision)"))
  (`AudioComponent.FadeIn` (`self.Audio`) Duration TargetVolume 0.0 "Linear"))

(fn `FadeOut`
  (params (Duration :type "Float (double-precision)"))
  (`AudioComponent.FadeOut` (`self.Audio`) Duration 0.0 "Linear"))

(fn `PlaySound`
  (`AudioComponent.Play` (`self.Audio`) 0.0))

(fn `SetPitch`
  (params (Pitch :type "Float (double-precision)"))
  (`AudioComponent.SetPitchMultiplier` (`self.Audio`) Pitch))

(fn `SetSound`
  (params (Sound :type "SoundBase Object Reference"))
  (`AudioComponent.SetSound` (`self.Audio`) Sound))

(fn `SetSoundAndPlay`
  (params (Sound :type "SoundBase Object Reference"))
  (bind _audio (`self.Audio`))
  (`AudioComponent.SetSound` _audio Sound)
  (`AudioComponent.Play` _audio 0.0))

(fn `SetVolume`
  (params (Volume :type "Float (double-precision)"))
  (`AudioComponent.SetVolumeMultiplier` (`self.Audio`) Volume))

(fn `StopSound`
  (`AudioComponent.Stop` (`self.Audio`)))

(fn `UserConstructionScript`)