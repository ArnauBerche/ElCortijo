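; BP_SafeBox is a puzzle safe, opened by turning a combination dial while the player is at its table view.
; Entering adds an input mapping and HUD, and binds horizontal camera input to rotate the wheel, which snaps to the nearest digit on release.
; DialUpdate converts roll into ten digits and tracks a four-number combination requiring alternating directions.
; Success exits the view, swings the door open and starts tension music.
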(event `self.EnterTable`
  (bind _character (`self.Character`))
  (`parent.EnterTable`)
  (`EnhancedInputSubsystemInterface.AddMappingContext` (pcsubsystem `EnhancedInputLocalPlayerSubsystem` (`self.Controller`)) "/Game/ElCortijo/Features/1_MainCharacter/Input/IMC_Table.IMC_Table" 100 (struct))
  (bind _returnvalue (`|CreateWidget` "/Game/ElCortijo/Features/8_MenuInterface/WBP_SafeBox.WBP_SafeBox_C" (`self.Controller`)))
  (bind _output_get (set `self.SafeHUD` _returnvalue))
  (`UserWidget.AddToViewport` _output_get 0)
  (add `/Game/ElCortijo/Features/1_MainCharacter/Blueprints/BP_FirstPersonCharacter.OnCameraHPress` _character (delegate `WheelRotate`))
  (add `/Game/ElCortijo/Features/1_MainCharacter/Blueprints/BP_FirstPersonCharacter.OnCameraHRelease` _character (delegate `ClampToNumber`)))

(event `WheelRotate`
  (params (Value :type "Float (double-precision)"))
  (bind _sfx (`self.SFX`))
  (bind (_relativerotation_roll _relativerotation_pitch _relativerotation_yaw) (`KismetMathLibrary.BreakRotator` (`SceneComponent.RelativeRotation` (`self.RuedaCajaFuerte_low`))))
  (`|ExecutionSequence`
    (:`then_0`
      (bind (_direction _clamp) (`Timeline|Clamp` :!via `Stop` :!label _label)
        (:`Update`
          (`SceneComponent.K2_SetRelativeRotation` (`self.RuedaCajaFuerte_low`) (`KismetMathLibrary.MakeRotator` (`KismetMathLibrary.Lerp` _relativerotation_roll (`KismetMathLibrary.Conv_IntToDouble` (* (`KismetMathLibrary.Round` (/ _relativerotation_roll 36.0)) 36)) _clamp) _relativerotation_pitch _relativerotation_yaw) false false))
        (:`Finished`
          (`FMODAudioComponent.Stop` (`self.SFX`))
          (set `self.IsRotating` false))))
    (:`then_1`
      (`self.Rotate` Value)
      (if (not (`self.IsRotating`))
        (`FMODAudioComponent.SetEvent` _sfx "/Game/FMOD/Events/SFX/Objetos/SFX_32_CajaFuerteRotacion.SFX_32_CajaFuerteRotacion")
        (`FMODAudioComponent.Play` _sfx)
        (set `self.IsRotating` true)))))

(event `ClampToNumber`
  (goto _label :!via `PlayFromStart`))

(event `self.ExitTable`
  (bind _character (`self.Character`))
  (`Widget.RemoveFromParent` (`self.SafeHUD`))
  (`parent.ExitTable`)
  (`EnhancedInputSubsystemInterface.RemoveMappingContext` (pcsubsystem `EnhancedInputLocalPlayerSubsystem` (`self.Controller`)) "/Game/ElCortijo/Features/1_MainCharacter/Input/IMC_Table.IMC_Table" (struct))
  (clear `/Game/ElCortijo/Features/1_MainCharacter/Blueprints/BP_FirstPersonCharacter.OnCameraHPress` _character)
  (clear `/Game/ElCortijo/Features/1_MainCharacter/Blueprints/BP_FirstPersonCharacter.OnCameraHRelease` _character))

(event `OpenSafe`
  (bind _sfx (`self.SFX`))
  (`FMODAudioComponent.SetEvent` _sfx "/Game/FMOD/Events/SFX/Objetos/SFX_30_CajaFuerteAbrir.SFX_30_CajaFuerteAbrir")
  (`FMODAudioComponent.Play` _sfx)
  (`self.ExitTable`)
  (`ActorComponent.K2_DestroyComponent` (`self.InteractBox`))
  (bind (_direction _alpha) (`Timeline|OpenDoor`)
    (:`Update`
      (`SceneComponent.K2_SetRelativeRotation` (`self.PuertaCajaFuerte_low`) (`KismetMathLibrary.MakeRotator` 0.0 0.0 (`KismetMathLibrary.Lerp` 90.0 0.0 _alpha)) false false)
      (bind _returnvalue (`GameplayStatics.GetActorOfClass` "/Game/ElCortijo/Features/SFX/BP_MusicaTension.BP_MusicaTension_C"))
      (set `/Game/ElCortijo/Features/SFX/BP_MusicaTension.Enabled` true _returnvalue)
      (bind _asbp_first_person_character (cast `/Game/ElCortijo/Features/1_MainCharacter/Blueprints/BP_FirstPersonCharacter` (`GameplayStatics.GetPlayerCharacter` 0)))
      (`FMODAudioComponent.Play` (`/Game/ElCortijo/Features/1_MainCharacter/Blueprints/BP_FirstPersonCharacter.SFX_Tension` _asbp_first_person_character)))))

(fn `DialUpdate`
  (bind _relativerotation_roll (`KismetMathLibrary.BreakRotator` (`SceneComponent.RelativeRotation` (`self.RuedaCajaFuerte_low`))))
  (bind _returnvalue (mod (`KismetMathLibrary.Round` (/ _relativerotation_roll 36.0)) 10))
  (if (< _returnvalue 0)
    (set `self.DialNumber` (+ _returnvalue 10))
    (else
      (set `self.DialNumber` _returnvalue)))
  (if (`self.CorrectNumber`)
    (if (!= (`self.DialNumber`) (`|GetArrayItem` (`self.Combination`) (`self.StepIndex`)))
      (set `self.CorrectNumber` false)
      (if (!= (`self.ExpectedDirIsRight`) (`self.DirectionIsRight`))
        (`/Engine/EditorBlueprintResources/StandardMacros.IncrementInt` (`self.StepIndex`)
          (:`  `
            _))
        (else
          (set `self.StepIndex` 0 :!label _label)))
      (set `self.ExpectedDirIsRight` (== (mod (`self.StepIndex`) 2) 0)))
    (elif (== (`self.ExpectedDirIsRight`) (`self.DirectionIsRight`))
      (if (== (`self.DialNumber`) (`|GetArrayItem` (`self.Combination`) (`self.StepIndex`)))
        (set `self.CorrectNumber` true)
        (if (== (`self.StepIndex`) 3)
          (`self.OpenSafe`)))
      (else
        (goto _label)))))

(fn `Rotate`
  (params (Value :type "Float (double-precision)"))
  (bind _ruedacajafuerte_low (`self.RuedaCajaFuerte_low`))
  (bind (_relativerotation_roll _relativerotation_pitch _relativerotation_yaw) (`KismetMathLibrary.BreakRotator` (`SceneComponent.RelativeRotation` _ruedacajafuerte_low)))
  (if (> Value 0.0)
    (set `self.DirectionIsRight` false)
    (`SceneComponent.K2_SetRelativeRotation` _ruedacajafuerte_low (`KismetMathLibrary.MakeRotator` (+ (* (* Value (`self.WheelSpeed`)) (`GameplayStatics.GetWorldDeltaSeconds`)) _relativerotation_roll) _relativerotation_pitch _relativerotation_yaw) false false :!label _label)
    (`self.DialUpdate`)
    (elif (< Value 0.0)
      (set `self.DirectionIsRight` true)
      (goto _label))))

(fn `UserConstructionScript`
  (`parent.UserConstructionScript`))