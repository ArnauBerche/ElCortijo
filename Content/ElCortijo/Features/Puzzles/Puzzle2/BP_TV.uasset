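; BP_TV is an interactable television prop in the El Cortijo Puzzle2 feature that changes its screen and sound on first use.
; It plays one audio component from BeginPlay.
; On the first Interact, guarded by a one-shot flag, it swaps to a second audio track, turns off its RectLight and changes the screen material.
; After a short delay it applies another screen material and restores the light.
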(event `self.ReceiveBeginPlay`
  (`AudioComponent.Play` (`self.Audio`) 0.0))

(event `self.Interact`
  (params (Interactor :type "Actor Object Reference"))
  (if (not (`self.HasInteracted`))
    (set `self.HasInteracted` true)
    (`AudioComponent.Stop` (`self.Audio`))
    (`AudioComponent.Play` (`self.Audio2`) 0.0)
    (`LightComponent.SetIntensity` (`self.RectLight`) 0.0)
    (`PrimitiveComponent.SetMaterial` (`self.Pantalla`) 0 "/Game/ElCortijo/Features/Props/Interior/Salon/TV/MI_TV_A.MI_TV_A")
    (`KismetSystemLibrary.Delay` 3.0)
    (`PrimitiveComponent.SetMaterial` (`self.Pantalla`) 0 "/Game/ElCortijo/Features/Props/Interior/Salon/TV/MI_TV_E2.MI_TV_E2")
    (`LightComponent.SetIntensity` (`self.RectLight`) 2000.0)))

(fn `UserConstructionScript`)