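; BP_PuertaSinPomo is an interactable Puzzle 2 door that is missing its knob and, while locked, needs a BP_Pomo to unlock.
; Interact checks the first-person character's current inventory item, destroys a matching knob and unlocks without opening; the inventory-clearing call is left disconnected.
; Once unlocked, each interaction toggles IsOpen and plays or reverses the OpenClose timeline, whose DoorAngle drives the mesh's yaw through a quarter turn.
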(event `self.Interact`
  (params (Interactor :type "Actor Object Reference"))
  (bind _mesh (`self.Mesh`))
  (bind (_relativerotation_roll _relativerotation_pitch) (`KismetMathLibrary.BreakRotator` (`SceneComponent.RelativeRotation` _mesh)))
  (if (`self.Locked`)
    (bind _asbp_first_person_character (cast `/Game/ElCortijo/Features/1_MainCharacter/Blueprints/BP_FirstPersonCharacter` Interactor))
    (bind _currentitemactor (`/Game/ElCortijo/Features/1_MainCharacter/BP_InventoryComponent.CurrentItemActor` (`/Game/ElCortijo/Features/1_MainCharacter/Blueprints/BP_FirstPersonCharacter.InventorySlot` _asbp_first_person_character)))
    (if (== "/Game/ElCortijo/Features/Puzzles/Puzzle2/BP_Pomo.BP_Pomo_C" (`GameplayStatics.GetObjectClass` _currentitemactor))
      (set `self.Locked` false)
      (`self.K2_DestroyActor` _currentitemactor))
    (elif (`self.IsOpen`)
      (set `self.IsOpen` false)
      (bind (_direction _doorangle) (`Timeline|Open/Close` :!via `Reverse` :!label _label)
        (:`Update`
          (`SceneComponent.K2_SetRelativeRotation` _mesh (`KismetMathLibrary.MakeRotator` _relativerotation_roll _relativerotation_pitch (`KismetMathLibrary.MapRangeClamped` _doorangle 0.0 1.0 0.0 90.0)) false false)))
      (else
        (set `self.IsOpen` true)
        (goto _label)))))

(fn `UserConstructionScript`)