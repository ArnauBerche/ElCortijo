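; BP_PuertaFumar is an interactable puzzle door that starts locked and is forced open with the poker item (BP_Atizador).
; Without the poker, it plays a locked sound, rattle timeline and hint dialogue.
; With it, it consumes the item, blends to a cinematic camera, disables player control and plays a Level Sequence before unlocking.
; Once unlocked, interaction toggles a sound-backed timeline that swings the mesh, with input blocked during the sequence.
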(event `/Game/ElCortijo/Features/2_InteractionSystem/BPI_Interactable.Interact`
  (params (Interactor :type "Actor Object Reference"))
  (bind _returnvalue (`GameplayStatics.GetPlayerController` 0))
  (bind _returnvalue_2 (`GameplayStatics.GetPlayerController` 0))
  (bind _returnvalue_3 (`GameplayStatics.GetPlayerController` 0))
  (bind _returnvalue_4 (`GameplayStatics.GetPlayerController` 0))
  (bind _sfx (`self.SFX`))
  (bind _sfx_2 (`self.SFX`))
  (bind _sfx_3 (`self.SFX`))
  (bind _mesh (`self.Mesh`))
  (bind _mesh_2 (`self.Mesh`))
  (bind (_relativerotation_roll _relativerotation_pitch) (`KismetMathLibrary.BreakRotator` (`SceneComponent.RelativeRotation` _mesh)))
  (bind (_relativerotation_roll_2 _relativerotation_pitch_2) (`KismetMathLibrary.BreakRotator` (`SceneComponent.RelativeRotation` _mesh_2)))
  (if (`self.SequencePlaying`)
    _
    (elif (`self.Locked`)
      (bind _asbp_first_person_character (cast `/Game/ElCortijo/Features/1_MainCharacter/Blueprints/BP_FirstPersonCharacter` Interactor))
      (bind _inventoryslot (`/Game/ElCortijo/Features/1_MainCharacter/Blueprints/BP_FirstPersonCharacter.InventorySlot` _asbp_first_person_character))
      (if (== "/Game/ElCortijo/Features/Puzzles/Puzzle2/BP_Atizador.BP_Atizador_C" (`GameplayStatics.GetObjectClass` (`/Game/ElCortijo/Features/1_MainCharacter/BP_InventoryComponent.CurrentItemActor` _inventoryslot)))
        (`PrimitiveComponent.SetCollisionResponseToChannel` (`self.Collider`) "ECC_GameTraceChannel1" "ECR_Ignore")
        (set `self.SequencePlaying` true)
        (bind (_outactor _returnvalue_5) (`LevelSequencePlayer.CreateLevelSequencePlayer` "/Game/ElCortijo/Features/Animaciones/Atizador/CinAtizador.CinAtizador" (make `MovieSceneSequencePlaybackSettings` false (struct) (struct :`bAllowRounding` true) 1.0 0.0 false false false false false false "ForceKeepState")))
        (`Controller.SetIgnoreLookInput` _returnvalue_4 true)
        (`Controller.SetIgnoreMoveInput` _returnvalue_4 true)
        (`/Game/ElCortijo/Features/1_MainCharacter/BP_InventoryComponent.DestroyAndClear` _inventoryslot)
        (`PlayerController.SetViewTargetWithBlend` _returnvalue_3 (`self.CamAtizador`) 0.3 "VTBlend_Linear" 0.0 false)
        (`self.DisableInput` _returnvalue_3 _returnvalue_3)
        (`KismetSystemLibrary.Delay` 0.3)
        (`MovieSceneSequencePlayer.Play` _returnvalue_5)
        (`KismetSystemLibrary.Delay` (`TimeManagementBlueprintLibrary.Conv_QualifiedFrameTimeToSeconds` (`MovieSceneSequencePlayer.GetDuration` _returnvalue_5)))
        (`MovieSceneSequencePlayer.Stop` _returnvalue_5)
        (`MovieSceneSequencePlayer.Stop` _returnvalue_5)
        (`self.K2_DestroyActor` _outactor)
        (`PrimitiveComponent.SetCollisionResponseToChannel` (`self.Collider`) "ECC_GameTraceChannel1" "ECR_Block")
        (`self.EnableInput` _returnvalue _returnvalue)
        (`PlayerController.SetViewTargetWithBlend` _returnvalue (`GameplayStatics.GetPlayerCharacter` 0) 0.3 "VTBlend_Linear" 0.0 false)
        (set `self.SequencePlaying` false)
        (set `self.Locked` false)
        (`Controller.SetIgnoreLookInput` _returnvalue_2 false)
        (`Controller.SetIgnoreMoveInput` _returnvalue_2 false)
        (else
          (`FMODAudioComponent.SetEvent` _sfx "/Game/FMOD/Events/SFX/Objetos/SFX_27_PuertaNoAbrir.SFX_27_PuertaNoAbrir")
          (`FMODAudioComponent.Play` _sfx)
          (bind (_direction _newtrack_0) (`Timeline|Cerrada` :!via `PlayFromStart`)
            (:`Update`
              (`SceneComponent.K2_SetRelativeRotation` _mesh_2 (`KismetMathLibrary.MakeRotator` _relativerotation_roll_2 _relativerotation_pitch_2 _newtrack_0) false false))
            (:`Finished`
              (`/Game/ElCortijo/Features/1_MainCharacter/Blueprints/BP_FirstPersonCharacter.SetRealTimeDialogue` _asbp_first_person_character "Parece que podría forzarse con algo" 1.5)))))
      (elif (`self.IsOpen`)
        (set `self.IsOpen` false)
        (`FMODAudioComponent.SetEvent` _sfx_2 "/Game/FMOD/Events/SFX/Objetos/SFX_25_PuertaCerrar.SFX_25_PuertaCerrar")
        (`FMODAudioComponent.Play` _sfx_2)
        (bind (_direction_2 _doorangle) (`Timeline|Open/Close` :!via `Reverse` :!label _label)
          (:`Update`
            (`SceneComponent.K2_SetRelativeRotation` _mesh (`KismetMathLibrary.MakeRotator` _relativerotation_roll _relativerotation_pitch (`KismetMathLibrary.MapRangeClamped` _doorangle 0.0 1.0 0.0 84.0)) false false)))
        (else
          (set `self.IsOpen` true)
          (`FMODAudioComponent.SetEvent` _sfx_3 "/Game/FMOD/Events/SFX/Objetos/SFX_24_PuertaAbrir.SFX_24_PuertaAbrir")
          (`FMODAudioComponent.Play` _sfx_3)
          (goto _label))))))

(fn `UserConstructionScript`)