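; BP_CuadroTorcido is an interactable crooked object in Puzzle 2 that straightens when used and reveals a note.
; Interact plays the Tilt timeline, which lerps the Box pitch from 20 degrees to level while keeping roll and yaw.
; When the timeline finishes, it spawns BP_P2Note1 at the Scene component's transform and sets HasRotated, which blocks later interactions.
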(event `/Game/ElCortijo/Features/2_InteractionSystem/BPI_Interactable.Interact`
  (params (Interactor :type "Actor Object Reference"))
  (bind _box (`self.Box`))
  (bind (_relativerotation_roll _relativerotation_pitch _relativerotation_yaw) (`KismetMathLibrary.BreakRotator` (`SceneComponent.RelativeRotation` _box)))
  (if (not (`self.HasRotated`))
    (bind (_direction _tilt) (`Timeline|Tilt`)
      (:`Update`
        (`SceneComponent.K2_SetRelativeRotation` _box (`KismetMathLibrary.MakeRotator` _relativerotation_roll (`KismetMathLibrary.Lerp` 20.0 0.0 _tilt) _relativerotation_yaw) false false))
      (:`Finished`
        (`|SpawnActorFromClass` "/Game/ElCortijo/Features/Puzzles/Puzzle2/BP_P2Note1.BP_P2Note1_C" (`SceneComponent.K2_GetComponentToWorld` (`self.Scene`)) "Undefined" "MultiplyWithRoot" null null)
        (set `self.HasRotated` true)))))

(fn `UserConstructionScript`)