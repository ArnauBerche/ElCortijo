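; Interactable switch for Puzzle 2 that toggles a light and has a continuously animated moving part.
; Each Interact flips HasRotated, switching the light's visibility and the sphere's material between bulb and cushion while the Boton timeline rolls Mesh1 forward or back.
; Independently, Tick uses a DoOnce that resets when its Timeline finishes, looping an animation of the Scene component's roll.
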(event `self.ReceiveTick`
  (params (DeltaSeconds :type "Float (single-precision)"))
  (bind (_relativerotation_roll _relativerotation_pitch _relativerotation_yaw) (`KismetMathLibrary.BreakRotator` (`SceneComponent.RelativeRotation` (`self.Scene`))))
  (`/Engine/EditorBlueprintResources/StandardMacros.DoOnce` false :!label _label
    (:`Completed`
      (bind (_direction _alpha) (`Timeline|Timeline` :!via `PlayFromStart`)
        (:`Update`
          (`SceneComponent.K2_SetRelativeRotation` (`self.Scene`) (`KismetMathLibrary.MakeRotator` _alpha _relativerotation_pitch _relativerotation_yaw) false false))
        (:`Finished`
          (goto _label :!via `Reset`))))))

(event `self.Interact`
  (params (Interactor :type "Actor Object Reference"))
  (if (`self.HasRotated`)
    (set `self.HasRotated` false)
    (`PrimitiveComponent.SetMaterial` (`self.Sphere`) 0 "/Game/ElCortijo/Features/Props/M_Cojin.M_Cojin")
    (`SceneComponent.SetVisibility` (`self.Luz`) false false)
    (bind (_direction _newtrack_0) (`Timeline|Boton` :!via `PlayFromStart` :!label _label_2)
      (:`Update`
        (`SceneComponent.K2_SetRelativeRotation` (`self.Mesh1`) (`KismetMathLibrary.MakeRotator` _newtrack_0) false false)))
    (else
      (set `self.HasRotated` true)
      (`PrimitiveComponent.SetMaterial` (`self.Sphere`) 0 "/Game/ElCortijo/Features/Props/Interior/Iluminacion/Bombilla/M_Bombilla.M_Bombilla")
      (`SceneComponent.SetVisibility` (`self.Luz`) true false)
      (goto _label_2 :!via `ReverseFromEnd`))))

(fn `UserConstructionScript`)