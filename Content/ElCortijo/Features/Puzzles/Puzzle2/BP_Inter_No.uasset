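; Non-working switch for Puzzle 2 that toggles its position on Interact and has no other effect.
; The HasRotated flag alternates the Boton timeline between forward and reverse, rolling Mesh1 around X.
; The forward branch also shows a Spanish real-time dialogue line on the first-person character saying it doesn't seem to work.
; When the timeline finishes, that dialogue resets after a short delay.
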(event `self.ReceiveBeginPlay`)

(event `self.Interact`
  (params (Interactor :type "Actor Object Reference"))
  (if (`self.HasRotated`)
    (set `self.HasRotated` false)
    (bind _asbp_first_person_character (cast `/Game/ElCortijo/Features/1_MainCharacter/Blueprints/BP_FirstPersonCharacter` (`GameplayStatics.GetPlayerCharacter` 0)))
    (`/Game/ElCortijo/Features/1_MainCharacter/Blueprints/BP_FirstPersonCharacter.SetRealTimeDialogue` _asbp_first_person_character "Vaya parece que no funciona." 0.0)
    (bind (_direction _newtrack_0) (`Timeline|Boton` :!via `PlayFromStart` :!label _label)
      (:`Update`
        (`SceneComponent.K2_SetRelativeRotation` (`self.Mesh1`) (`KismetMathLibrary.MakeRotator` _newtrack_0) false false))
      (:`Finished`
        (`KismetSystemLibrary.Delay` 1.0)
        (`/Game/ElCortijo/Features/1_MainCharacter/Blueprints/BP_FirstPersonCharacter.ResetRealTimeDialogue` _asbp_first_person_character)))
    (else
      (set `self.HasRotated` true)
      (goto _label :!via `ReverseFromEnd`))))

(fn `UserConstructionScript`)