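; BP_Inter_Func is a working light switch in Puzzle 2 that turns a bulb and spot light on or off.
; Each Interact call flips HasRotated, swapping the Bombilla (bulb) material and toggling the SpotLight's visibility.
; The Boton timeline animates Mesh1's roll as the switch button, playing from start when switching off and reversing from end when switching on.
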(event `self.Interact`
  (params (Interactor :type "Actor Object Reference"))
  (if (`self.HasRotated`)
    (set `self.HasRotated` false)
    (`PrimitiveComponent.SetMaterial` (`self.Bombilla`) 0 "/Game/ElCortijo/Features/Props/M_Cojin.M_Cojin")
    (`SceneComponent.SetVisibility` (`self.SpotLight`) false false)
    (bind (_direction _newtrack_0) (`Timeline|Boton` :!via `PlayFromStart` :!label _label)
      (:`Update`
        (`SceneComponent.K2_SetRelativeRotation` (`self.Mesh1`) (`KismetMathLibrary.MakeRotator` _newtrack_0) false false)))
    (else
      (set `self.HasRotated` true)
      (`PrimitiveComponent.SetMaterial` (`self.Bombilla`) 0 "/Game/ElCortijo/Features/Props/Interior/Iluminacion/Bombilla/M_Bombilla.M_Bombilla")
      (`SceneComponent.SetVisibility` (`self.SpotLight`) true false)
      (goto _label :!via `ReverseFromEnd`))))

(fn `UserConstructionScript`)