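; BP_ClueHotspot is a clickable hotspot belonging to a clue, intended to create evidence at the research table.
; Initialize stores the owner clue and evidence data and starts it inactive; SetActive toggles query collision and visibility unless consumed.
; Clicking checks that the owner clue is placed on a research table, then consumes and hides the hotspot.
; Evidence creation is currently only a debug print, and the stored evidence data is unused.
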(event `/Game/ElCortijo/Features/Interaction/BPI_Clickable.Click`
  (params (Interactor :type "Actor Object Reference"))
  (if (and (`self.bActive`) (not (`self.bConsumed`)))
    (`self.RequestCreateEvidence`)))

(fn `Initialize`
  (params (Owner :type "/Game/ElCortijo/Features/ReserchTable/BP_ClueItem Object Reference") (Evidence :type "/Game/ElCortijo/Features/Evidence/DA_Evidence Object Reference"))
  (set `self.OwnerClue` Owner)
  (set `self.EvidenceData` Evidence)
  (`self.SetConsumed` false)
  (`self.SetActive` false))

(fn `RequestCreateEvidence`
  (bind _ownerclue (`self.OwnerClue`))
  (if (`self.bConsumed`)
    _
    (elif (and (and (!= _ownerclue null) (`/Game/ElCortijo/Features/ReserchTable/BP_ClueItem.bPlacedOnResearchTable` _ownerclue)) (!= (`/Game/ElCortijo/Features/ReserchTable/BP_ClueItem.CurrentResearchTable` _ownerclue) null))
      (`KismetSystemLibrary.PrintText` "Crear prueba desde mesa")
      (`self.SetConsumed` true))))

(fn `SetActive`
  (params (bActive :type Boolean))
  (bind _collider (`self.Collider`))
  (bind _output_get (set `self.bActive` bActive))
  (bind _returnvalue (and _output_get (not (`self.bConsumed`))))
  (if _returnvalue
    (`PrimitiveComponent.SetCollisionEnabled` _collider "QueryOnly")
    (else
      (`PrimitiveComponent.SetCollisionEnabled` _collider "NoCollision")))
  (`SceneComponent.SetHiddenInGame` (`self.Visual`) (not _returnvalue) false))

(fn `SetConsumed`
  (params (bConsumed :type Boolean))
  (bind _output_get (set `self.bConsumed` bConsumed))
  (if _output_get
    (`self.SetActive` false)))

(fn `UserConstructionScript`)