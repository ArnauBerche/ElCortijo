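; Research table actor where the player examines the held inventory item and extracts hint pickups.
; Interact toggles a blended table camera with mouse input, spawning the item as a BP_Pickable or returning it to inventory.
; Right click snaps to the nearest base or flipped rotation via timeline; short press flips 180°, holding tilts by clamped, Tick-interpolated mouse drag.
; Left click on an interactable under the cursor spawns hints once, marking the item researched.
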(event `OnRightClickPressed_Handler`
  (bind _resettargetrot (`self.ResetTargetRot`))
  (bind (_locationx _locationy) (`PlayerController.GetMousePosition` (`GameplayStatics.GetPlayerController` 0)))
  (if (and (`self.PlayerInTable`) (!= (`self.ResearchableObject`) null))
    (if (`self.bIsSnaped`)
      (set `self.bIsPressed` true)
      (set `self.bIsSnaped` false)
      (set `self.PressTime` (`KismetSystemLibrary.GetGameTimeInSeconds`))
      (set `self.StartMousePos` (`KismetMathLibrary.MakeVector2D` _locationx _locationy))
      (`self.SnapToNearestCanonicalRotation`)
      (bind (_direction _newtrack_0) (`Timeline|TL_ResetRotation` :!via `PlayFromStart`)
        (:`Update`
          (`self.K2_SetActorRotation` (`self.ResearchableObject`) (`KismetMathLibrary.RLerp` (`self.ResetStartRot`) _resettargetrot _newtrack_0 true) false))
        (:`Finished`
          (set `self.bIsSnaped` true)
          (set `self.HoldStartLocalRotation` _resettargetrot)
          (set `self.CurrentOffsetPitch` 0.0)
          (set `self.CurrentOffsetRoll` 0.0)
          (if (`self.ShoudFlip`)
            (`self.StartFlip`)
            (set `self.ShoudFlip` false)))))))

(event `OnRightClickHoldRelease_Handler`
  (if (and (`self.PlayerInTable`) (!= (`self.ResearchableObject`) null))
    (if (`self.bIsPressed`)
      (set `self.bIsPressed` false)
      (if (<= (- (`KismetSystemLibrary.GetGameTimeInSeconds`) (`self.PressTime`)) (`self.ShortPressThreshold`))
        (set `self.ShoudFlip` true)
        (else
          (set `self.ShoudFlip` false)
          (if (`self.bIsHolding`)
            (`self.EndHold`)))))))

(event `self.ReceiveBeginPlay`
  (bind _asbp_first_person_character (cast `/Game/FirstPerson/Blueprints/BP_FirstPersonCharacter` (`GameplayStatics.GetPlayerCharacter` 0)))
  (`|ExecutionSequence`
    (:`then_0`
      (`KismetArrayLibrary.Array_Add` (`self.HintPlacementsRef`) (`self.HintPlacement1`))
      (`KismetArrayLibrary.Array_Add` (`self.HintPlacementsRef`) (`self.HintPlacement2`))
      (`KismetArrayLibrary.Array_Add` (`self.HintPlacementsRef`) (`self.HintPlacement3`)))
    (:`then_1`
      (add `/Game/FirstPerson/Blueprints/BP_FirstPersonCharacter.OnLeftClick` _asbp_first_person_character (delegate `OnLeftClick_Handler`))
      (add `/Game/FirstPerson/Blueprints/BP_FirstPersonCharacter.OnRightClickPress` _asbp_first_person_character (delegate `OnRightClickPressed_Handler`))
      (add `/Game/FirstPerson/Blueprints/BP_FirstPersonCharacter.OnRightClickRelease` _asbp_first_person_character (delegate `OnRightClickHoldRelease_Handler`)))))

(event `OnLeftClick_Handler`
  (`self.LeftClickPress`))

(event `self.ReceiveTick`
  (params (DeltaSeconds :type "Float (single-precision)"))
  (`|ExecutionSequence`
    (:`then_0`
      (if (and (`self.PlayerInTable`) (!= (`self.ResearchableObject`) null))
        (if (`self.bPlayingFlip`)
          (`self.TickFlip` DeltaSeconds)
          (elif (and (`self.bIsPressed`) (not (`self.bIsHolding`)))
            (if (>= (- (`KismetSystemLibrary.GetGameTimeInSeconds`) (`self.PressTime`)) (`self.ShortPressThreshold`))
              (`self.StartHold`))
            (elif (`self.bIsHolding`)
              (`self.TickHold` DeltaSeconds))))))))

(event `/Game/ElCortijo/Features/Interaction/BPI_Interactable.Interact`
  (params (Interactor :type "Actor Object Reference"))
  (bind _as_bp_first_person_character (`self.As BP First Person Character`))
  (bind _asbp_first_person_character (cast `/Game/FirstPerson/Blueprints/BP_FirstPersonCharacter` Interactor))
  (set `self.As BP First Person Character` _asbp_first_person_character)
  (bind _asplayer_controller (cast `PlayerController` (`Pawn.GetController` _asbp_first_person_character)))
  (set `self.As Player Controller` _asplayer_controller)
  (set `self.CameraOwner` (`ActorComponent.GetOwner` (`self.Camera`)))
  (if (`self.CanInteract`)
    (`/Engine/EditorBlueprintResources/StandardMacros.FlipFlop`
      (:`A`
        (`self.CreateResearchableObject` _as_bp_first_person_character)
        (`Controller.SetIgnoreLookInput` (`self.As Player Controller`) true)
        (`Controller.SetIgnoreMoveInput` (`self.As Player Controller`) true)
        (`PlayerController.SetViewTargetWithBlend` (`self.As Player Controller`) (`self.CameraOwner`) (`self.Blend Time`) "VTBlend_Linear" 0.0 false)
        (set `PlayerController.bShowMouseCursor` true (`self.As Player Controller`))
        (set `self.CanInteract` false)
        (`WidgetBlueprintLibrary.SetInputMode_GameAndUIEx` (`self.As Player Controller`) null "DoNotLock" false)
        (`KismetSystemLibrary.Delay` (`self.Blend Time`))
        (set `self.CanInteract` true)
        (set `self.PlayerInTable` true))
      (:`B`
        (`self.DestroyReserchableObject` _as_bp_first_person_character)
        (`PlayerController.SetViewTargetWithBlend` (`self.As Player Controller`) (`self.As BP First Person Character`) (`self.Blend Time`) "VTBlend_Linear" 0.0 false)
        (set `self.CanInteract` false)
        (`KismetSystemLibrary.Delay` (`self.Blend Time`))
        (set `self.CanInteract` true)
        (`Controller.SetIgnoreLookInput` (`self.As Player Controller`) false)
        (`Controller.SetIgnoreMoveInput` (`self.As Player Controller`) false)
        (set `PlayerController.bShowMouseCursor` false (`self.As Player Controller`))
        (`WidgetBlueprintLibrary.SetInputMode_GameOnly` (`self.As Player Controller`))
        (set `self.PlayerInTable` false)))))

(fn `CreateResearchableObject`
  (params (Interactor :type "/Game/FirstPerson/Blueprints/BP_FirstPersonCharacter Object Reference"))
  (bind _proofplacement (`self.ProofPlacement`))
  (bind (_name _mesh _type _previewrotator _scale _objectoffset _collidersize _canpickup _candrop _isresearched) (break `/Game/ElCortijo/Features/Interaction/Pickable/S_ItemData` (`/Game/ElCortijo/Features/Character/BP_InventoryComponent.CurrentItem` (`self.Inventory Slot`))))
  ; Check if item can be picked up
  (bind _output_get (set `self.Inventory Slot` (`/Game/FirstPerson/Blueprints/BP_FirstPersonCharacter.InventorySlot` Interactor)))
  (bind _canpickup_2 (`/Game/ElCortijo/Features/Character/BP_InventoryComponent.CanPickup` :`self` _output_get))
  (if (not _canpickup_2)
    ; Check typing
    (if (!= _type 0)
      ; Set correct position and spawn Actor
      (bind _returnvalue (`|SpawnActorFromClass` "/Game/ElCortijo/Features/Interaction/Pickable/BP_Pickable.BP_Pickable_C" (`KismetMathLibrary.MakeTransform` (`SceneComponent.K2_GetComponentLocation` _proofplacement) (`SceneComponent.K2_GetComponentRotation` _proofplacement) _scale) "AlwaysSpawn" "MultiplyWithRoot" null (make `/Game/ElCortijo/Features/Interaction/Pickable/S_ItemData` _name _mesh _type _previewrotator _scale _objectoffset _collidersize false false _isresearched) true null))
      ; Set collision channel to research
      (`PrimitiveComponent.SetCollisionResponseToChannel` (`/Game/ElCortijo/Features/Interaction/Pickable/BP_Pickable.Collision` _returnvalue) "ECC_GameTraceChannel2" "ECR_Block")
      ; Turn off physics
      (bind _output_get_2 (set `self.ResearchableObject` _returnvalue))
      (`PrimitiveComponent.SetSimulatePhysics` (`/Game/ElCortijo/Features/Interaction/Pickable/BP_Pickable.Collision` _output_get_2) false)
      ; Empty inventory
      (`/Game/ElCortijo/Features/Character/BP_InventoryComponent.ClearItem` (`self.Inventory Slot`))
      (`self.ResetRotationValues`)
      (return))))

(fn `DestroyReserchableObject`
  (params (Interactor :type "/Game/FirstPerson/Blueprints/BP_FirstPersonCharacter Object Reference"))
  (bind _researchableobject (`self.ResearchableObject`))
  (bind (_name _mesh _type _previewrotator _scale _objectoffset _collidersize _canpickup _candrop _isresearched) (break `/Game/ElCortijo/Features/Interaction/Pickable/S_ItemData` (`/Game/ElCortijo/Features/Interaction/Pickable/BP_Pickable.ItemData` _researchableobject)))
  (if (!= _researchableobject null)
    (`/Game/ElCortijo/Features/Character/BP_InventoryComponent.AddItem` (`/Game/FirstPerson/Blueprints/BP_FirstPersonCharacter.InventorySlot` Interactor) (make `/Game/ElCortijo/Features/Interaction/Pickable/S_ItemData` _name _mesh _type _previewrotator _scale _objectoffset _collidersize true true _isresearched))
    (`self.K2_DestroyActor` (`self.ResearchableObject`))
    (return)))

(fn `EndHold`
  (set `self.bIsHolding` false))

(fn `LeftClickPress`
  (bind _researchableobject (`self.ResearchableObject`))
  (bind (_name _mesh _type _previewrotator _scale _objectoffset _collidersize) (break `/Game/ElCortijo/Features/Interaction/Pickable/S_ItemData` (`/Game/ElCortijo/Features/Interaction/Pickable/BP_Pickable.ItemData` (`self.ResearchableObject`))))
  (bind (_name_2 _mesh_2 _type_2 _previewrotator_2 _scale_2 _objectoffset_2 _collidersize_2 _canpickup _candrop) (break `/Game/ElCortijo/Features/Interaction/Pickable/S_ItemData` (`/Game/ElCortijo/Features/Interaction/Pickable/BP_Pickable.ItemData` _researchableobject)))
  (bind (_bblockinghit _binitialoverlap _time _distance _location _impactpoint _normal _impactnormal _physmat _hitactor) (`GameplayStatics.BreakHitResult` (`PlayerController.GetHitResultUnderCursorByChannel` (`GameplayStatics.GetPlayerController` 0) "TraceTypeQuery4" true)))
  (if (!= (`self.ResearchableObject`) null)
    (if (`self.PlayerInTable`)
      (if (and (`KismetSystemLibrary.DoesImplementInterface` _hitactor "/Game/ElCortijo/Features/Interaction/BPI_Interactable.BPI_Interactable_C") (!= (`KismetSystemLibrary.GetDisplayName` _hitactor) (`KismetSystemLibrary.GetDisplayName` self)))
        (if (not (`.IsResearched_30_165A08BA435CE352260BC5ABFC98750A` (break `/Game/ElCortijo/Features/Interaction/Pickable/S_ItemData` (`/Game/ElCortijo/Features/Interaction/Pickable/BP_Pickable.ItemData` (`self.ResearchableObject`)))))
          (for _index (range (`self.HintAmount(temporal)`))
            (bind _output (`|GetArrayItem` (`self.HintPlacementsRef`) _index))
            (bind _returnvalue (`|SpawnActorFromClass` "/Game/ElCortijo/Features/Interaction/Pickable/BP_Pickable.BP_Pickable_C" (`KismetMathLibrary.MakeTransform` (`SceneComponent.K2_GetComponentLocation` _output) (`SceneComponent.K2_GetComponentRotation` _output) _scale) "AlwaysSpawn" "MultiplyWithRoot" null (make `/Game/ElCortijo/Features/Interaction/Pickable/S_ItemData` _name _mesh "NewEnumerator2" _previewrotator _scale _objectoffset _collidersize true true true) true null))
            ; Set collision channel to Interact
            (`PrimitiveComponent.SetCollisionResponseToChannel` (`/Game/ElCortijo/Features/Interaction/Pickable/BP_Pickable.Collision` _returnvalue) "ECC_GameTraceChannel1" "ECR_Block"))
          (set `/Game/ElCortijo/Features/Interaction/Pickable/BP_Pickable.ItemData` (make `/Game/ElCortijo/Features/Interaction/Pickable/S_ItemData` _name_2 _mesh_2 _type_2 _previewrotator_2 _scale_2 _objectoffset_2 _collidersize_2 _canpickup _candrop true) _researchableobject))))))

(fn `ResetRotationValues`
  (set `self.bIsPressed` false)
  (set `self.bIsHolding` false)
  (set `self.bPlayingFlip` false)
  (set `self.StartMousePos` (0.0 0.0))
  (set `self.PressTime` 0.0)
  (set `self.HoldStartLocalRotation` (struct))
  (set `self.CurrentOffsetPitch` 0.0)
  (set `self.CurrentOffsetRoll` 0.0)
  (set `self.FlipElapsed` 0.0)
  (set `self.FlipStartRot` (struct))
  (set `self.FlipTargetRot` (struct))
  (set `self.BaseLocalRotation` (struct))
  (set `self.FlipLocalRotation` (struct))
  (set `self.bIsSnaped` true)
  (set `self.ResetStartRot` (struct))
  (set `self.ResetTargetRot` (struct))
  (set `self.bIsFliped` false)
  (set `self.ShoudFlip` false))

(fn `SnapToNearestCanonicalRotation`
  (locals (CurrentRot :type "Rotator Structure" :default (struct)) (FlipDelta :type "Rotator Structure" :default (struct)) (DeltaBase :type "Rotator Structure" :default (struct)) (FlipBase :type "Rotator Structure" :default (struct)) (DistToBase :type "Float (double-precision)") (DistToFlip :type "Float (double-precision)"))
  (if (`KismetSystemLibrary.IsValid` (`self.ResearchableObject`))
    (set `self.BaseLocalRotation` (`self.K2_GetActorRotation` self))
    (set `local.CurrentRot` (`self.K2_GetActorRotation` (`self.ResearchableObject`)))
    (set `self.FlipLocalRotation` (`self.FlipTargetRot`))
    (bind _output_get (set `local.DeltaBase` (`KismetMathLibrary.ComposeRotators` (`local.CurrentRot`) (`KismetMathLibrary.NegateRotator` (`self.BaseLocalRotation`)))))
    (set `local.DistToBase` (+ (+ (`KismetMathLibrary.Abs` (.roll _output_get)) (`KismetMathLibrary.Abs` (.pitch _output_get))) (`KismetMathLibrary.Abs` (.yaw _output_get))))
    (bind _output_get_2 (set `local.FlipBase` (`KismetMathLibrary.ComposeRotators` (`local.CurrentRot`) (`KismetMathLibrary.NegateRotator` (`self.FlipLocalRotation`)))))
    (set `local.DistToFlip` (+ (+ (`KismetMathLibrary.Abs` (.roll _output_get_2)) (`KismetMathLibrary.Abs` (.pitch _output_get_2))) (`KismetMathLibrary.Abs` (.yaw _output_get_2))))
    (set `self.ResetStartRot` (`local.CurrentRot`))
    (if (<= (`local.DistToBase`) (`local.DistToFlip`))
      (set `self.ResetTargetRot` (`self.BaseLocalRotation`))
      (else
        (set `self.ResetTargetRot` (`self.FlipLocalRotation`))))))

(fn `StartFlip`
  (if (not (`self.bPlayingFlip`))
    (set `self.bPlayingFlip` true)
    (set `self.FlipElapsed` 0.0)
    (bind _output_get (set `self.FlipStartRot` (`self.K2_GetActorRotation` (`self.ResearchableObject`))))
    (if (`self.bIsFliped`)
      (bind _roll (.roll _output_get))
      (bind _pitch (.pitch _output_get))
      (bind _yaw (.yaw _output_get))
      (set `self.FlipTargetRot` (`KismetMathLibrary.MakeRotator` (+ _roll -180.0) _pitch _yaw))
      (else
        (set `self.FlipTargetRot` (`KismetMathLibrary.MakeRotator` (+ _roll 180.0) _pitch _yaw))))))

(fn `StartHold`
  (if (`self.bIsSnaped`)
    (set `self.bIsHolding` true)))

(fn `TickFlip`
  (params (DeltaSeconds :type "Float (double-precision)"))
  (bind _returnvalue (`KismetMathLibrary.FClamp` (/ (`self.FlipElapsed`) (`self.FlipDuration`))))
  (set `self.FlipElapsed` (+ (`self.FlipElapsed`) DeltaSeconds))
  (`self.K2_SetActorRelativeRotation` (`self.ResearchableObject`) (`KismetMathLibrary.RLerp` (`self.FlipStartRot`) (`self.FlipTargetRot`) (`|EaseFunction` "EaseInOut" _returnvalue 0.0 1.0)) false false)
  (if (>= _returnvalue 1.0)
    (set `self.bPlayingFlip` false)
    (`self.K2_SetActorRelativeRotation` (`self.ResearchableObject`) (`self.FlipTargetRot`) false false)
    (set `self.FlipElapsed` 0.0)
    (bind _output_get (set `self.bIsFliped` (not (`self.bIsFliped`))))
    (`KismetSystemLibrary.PrintString` (`KismetStringLibrary.Conv_BoolToString` _output_get))))

(fn `TickHold`
  (params (DelataSeconds :type "Float (double-precision)"))
  (locals (Drag :type "Vector2D Structure") (Dist :type "Float (double-precision)" :default 0.0) (DistNorm :type "Float (double-precision)" :default 0.0) (SpeedScale :type "Float (double-precision)") (RawDesiredRoll :type "Float (double-precision)") (RawDesiredPitch :type "Float (double-precision)") (DesiredRollOffset :type "Float (double-precision)" :default 0.0) (DesiredPitchOffset :type "Float (double-precision)" :default 0.0) (DeltaSeconds :type "Float (double-precision)"))
  (bind _maxangle (`self.MaxAngle`))
  (bind _maxangle_2 (`self.MaxAngle`))
  (bind (_locationx _locationy _returnvalue) (`PlayerController.GetMousePosition` (`GameplayStatics.GetPlayerController` 0)))
  (bind (_x _y) (`KismetMathLibrary.BreakVector2D` (`local.Drag`)))
  (set `local.DeltaSeconds` DelataSeconds)
  (if _returnvalue
    (set `local.Drag` (- (`KismetMathLibrary.MakeVector2D` _locationx _locationy) (`self.StartMousePos`)))
    (set `local.Dist` (`KismetMathLibrary.VSize2D` (`local.Drag`)))
    (set `local.DistNorm` (`KismetMathLibrary.FClamp` (/ (`local.Dist`) (`self.MaxDragDistance`))))
    (set `local.SpeedScale` (- 1.0 (`local.DistNorm`)))
    (set `local.RawDesiredRoll` (* (* _x (`self.BaseRotateSpeed`)) (`local.SpeedScale`)))
    (set `local.RawDesiredPitch` (* (* _y (`self.BaseRotateSpeed`)) (`local.SpeedScale`)))
    (set `local.DesiredRollOffset` (`KismetMathLibrary.FClamp` (`local.RawDesiredRoll`) (* _maxangle_2 -1.0) _maxangle_2))
    (set `local.DesiredPitchOffset` (`KismetMathLibrary.FClamp` (`local.RawDesiredPitch`) (* _maxangle -1.0) _maxangle))
    (set `self.CurrentOffsetRoll` (`KismetMathLibrary.FInterpTo` (`self.CurrentOffsetRoll`) (`local.DesiredRollOffset`) (`local.DeltaSeconds`) 12.0))
    (set `self.CurrentOffsetPitch` (`KismetMathLibrary.FInterpTo` (`self.CurrentOffsetPitch`) (`local.DesiredPitchOffset`) (`local.DeltaSeconds`) 12.0))
    (`self.K2_SetActorRotation` (`self.ResearchableObject`) (`KismetMathLibrary.MakeRotator` (+ (.roll (`self.HoldStartLocalRotation`)) (`self.CurrentOffsetRoll`)) (+ (.pitch (`self.HoldStartLocalRotation`)) (`self.CurrentOffsetPitch`)) (.yaw (`self.HoldStartLocalRotation`))) false)))

(fn `UserConstructionScript`)