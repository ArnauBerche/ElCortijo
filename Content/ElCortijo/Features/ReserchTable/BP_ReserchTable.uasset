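; Research table actor where the player places an inventory item to inspect it and produce hints.
; Interact alternates between blending to the table camera with the item spawned as a physics-free pickable, and returning the item and player control.
; Bound character mouse events drive inspection: right-click hold rotates the item by mouse delta.
; Left-click cursor-traces for an interactable, spawning hint pickables at placement points and marking the item researched to prevent repeats.
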(event `self.ReceiveBeginPlay`
  (bind _asbp_first_person_character (cast `/Game/FirstPerson/Blueprints/BP_FirstPersonCharacter` (`GameplayStatics.GetPlayerCharacter` 0)))
  (`|ExecutionSequence`
    (:`then_0`
      (`KismetArrayLibrary.Array_Add` (`self.HintPlacementsRef`) (`self.HintPlacement1`))
      (`KismetArrayLibrary.Array_Add` (`self.HintPlacementsRef`) (`self.HintPlacement2`))
      (`KismetArrayLibrary.Array_Add` (`self.HintPlacementsRef`) (`self.HintPlacement3`)))
    (:`then_1`
      (add `/Game/FirstPerson/Blueprints/BP_FirstPersonCharacter.OnLeftClick` _asbp_first_person_character (delegate `OnLeftClick_Handler`))
      (add `/Game/FirstPerson/Blueprints/BP_FirstPersonCharacter.OnRightClick` _asbp_first_person_character (delegate `OnRightClick_Handler`))
      (add `/Game/FirstPerson/Blueprints/BP_FirstPersonCharacter.OnRightClickHold` _asbp_first_person_character (delegate `OnRightClickHold_Handler`)))))

(event `OnLeftClick_Handler`
  (`self.Click`))

(event `OnRightClick_Handler`
  (`self.RotationInfo`))

(event `OnRightClickHold_Handler`
  (`self.Rotate`))

(event `self.ReceiveTick`
  (params (DeltaSeconds :type "Float (single-precision)")))

(event `/Game/ElCortijo/Features/Interaction/BPI_Interactable.Interact`
  (params (Interactor :type "Actor Object Reference"))
  (bind _as_bp_first_person_character (`self.As BP First Person Character`))
  (bind _asbp_first_person_character (cast `/Game/FirstPerson/Blueprints/BP_FirstPersonCharacter` Interactor))
  (set `self.As BP First Person Character` _asbp_first_person_character)
  (bind _asplayer_controller (cast `PlayerController` (`Pawn.GetController` _asbp_first_person_character)))
  (set `self.As Player Controller` _asplayer_controller)
  (set `self.CameraOwner` (`ActorComponent.GetOwner` (`self.Camera`)))
  (if (`self.CanInteract`)
    (`/Engine/EditorBlueprintResources/StandardMacros.FlipFlop`
      (:`A`
        (`self.CreateResearchableObject` _as_bp_first_person_character)
        (`Controller.SetIgnoreLookInput` (`self.As Player Controller`) true)
        (`Controller.SetIgnoreMoveInput` (`self.As Player Controller`) true)
        (`PlayerController.SetViewTargetWithBlend` (`self.As Player Controller`) (`self.CameraOwner`) (`self.Blend Time`) "VTBlend_Linear" 0.0 false)
        (set `PlayerController.bShowMouseCursor` true (`self.As Player Controller`))
        (set `self.CanInteract` false)
        (`KismetSystemLibrary.Delay` (`self.Blend Time`))
        (set `self.CanInteract` true)
        (set `self.PlayerInTable` true))
      (:`B`
        (`self.DestroyReserchableObject` _as_bp_first_person_character)
        (`PlayerController.SetViewTargetWithBlend` (`self.As Player Controller`) (`self.As BP First Person Character`) (`self.Blend Time`) "VTBlend_Linear" 0.0 false)
        (set `self.CanInteract` false)
        (`KismetSystemLibrary.Delay` (`self.Blend Time`))
        (set `self.CanInteract` true)
        (`Controller.SetIgnoreLookInput` (`self.As Player Controller`) false)
        (`Controller.SetIgnoreMoveInput` (`self.As Player Controller`) false)
        (set `PlayerController.bShowMouseCursor` false (`self.As Player Controller`))
        (`WidgetBlueprintLibrary.SetInputMode_GameOnly` (`self.As Player Controller`))
        (set `self.PlayerInTable` false)))))

(fn `Click`
  (bind _objeto_investigable (`self.Objeto Investigable`))
  (bind (_name _mesh _type _previewrotator _scale _objectoffset _collidersize) (break `/Game/ElCortijo/Features/Interaction/Pickable/S_ItemData` (`/Game/ElCortijo/Features/Interaction/Pickable/BP_Pickable.ItemData` (`self.Objeto Investigable`))))
  (bind (_name_2 _mesh_2 _type_2 _previewrotator_2 _scale_2 _objectoffset_2 _collidersize_2 _canpickup _candrop) (break `/Game/ElCortijo/Features/Interaction/Pickable/S_ItemData` (`/Game/ElCortijo/Features/Interaction/Pickable/BP_Pickable.ItemData` _objeto_investigable)))
  (bind (_bblockinghit _binitialoverlap _time _distance _location _impactpoint _normal _impactnormal _physmat _hitactor) (`GameplayStatics.BreakHitResult` (`PlayerController.GetHitResultUnderCursorByChannel` (`GameplayStatics.GetPlayerController` 0) "TraceTypeQuery4" true)))
  (if (!= (`self.Objeto Investigable`) null)
    (if (`self.PlayerInTable`)
      (if (and (`KismetSystemLibrary.DoesImplementInterface` _hitactor "/Game/ElCortijo/Features/Interaction/BPI_Interactable.BPI_Interactable_C") (!= (`KismetSystemLibrary.GetDisplayName` _hitactor) (`KismetSystemLibrary.GetDisplayName` self)))
        (if (not (`.IsResearched_30_165A08BA435CE352260BC5ABFC98750A` (break `/Game/ElCortijo/Features/Interaction/Pickable/S_ItemData` (`/Game/ElCortijo/Features/Interaction/Pickable/BP_Pickable.ItemData` (`self.Objeto Investigable`)))))
          (for _index (range (`self.HintAmount(temporal)`))
            (bind _output (`|GetArrayItem` (`self.HintPlacementsRef`) _index))
            (bind _returnvalue (`|SpawnActorFromClass` "/Game/ElCortijo/Features/Interaction/Pickable/BP_Pickable.BP_Pickable_C" (`KismetMathLibrary.MakeTransform` (`SceneComponent.K2_GetComponentLocation` _output) (`SceneComponent.K2_GetComponentRotation` _output) _scale) "AlwaysSpawn" "MultiplyWithRoot" null (make `/Game/ElCortijo/Features/Interaction/Pickable/S_ItemData` _name _mesh "NewEnumerator2" _previewrotator _scale _objectoffset _collidersize true true true) true null))
            ; Set collision channel to Interact
            (`PrimitiveComponent.SetCollisionResponseToChannel` (`/Game/ElCortijo/Features/Interaction/Pickable/BP_Pickable.Collision` _returnvalue) "ECC_GameTraceChannel1" "ECR_Block"))
          (set `/Game/ElCortijo/Features/Interaction/Pickable/BP_Pickable.ItemData` (make `/Game/ElCortijo/Features/Interaction/Pickable/S_ItemData` _name_2 _mesh_2 _type_2 _previewrotator_2 _scale_2 _objectoffset_2 _collidersize_2 _canpickup _candrop true) _objeto_investigable))))))

(fn `CreateResearchableObject`
  (params (Interactor :type "/Game/FirstPerson/Blueprints/BP_FirstPersonCharacter Object Reference"))
  (bind _proofplacement (`self.ProofPlacement`))
  (bind (_name _mesh _type _previewrotator _scale _objectoffset _collidersize _canpickup _candrop _isresearched) (break `/Game/ElCortijo/Features/Interaction/Pickable/S_ItemData` (`/Game/ElCortijo/Features/Interaction/Pickable/BP_Pickable.ItemData` (`/Game/ElCortijo/Features/Character/BP_InventoryComponent.CurrentItemActor` (`self.Inventory Slot`)))))
  ; Check if item can be picked up
  (bind _output_get (set `self.Inventory Slot` (`/Game/FirstPerson/Blueprints/BP_FirstPersonCharacter.InventorySlot` Interactor)))
  (bind _empty (`/Game/ElCortijo/Features/Character/BP_InventoryComponent.IsEmpty` _output_get))
  (if _empty
    ; Check typing
    (if (!= _type 0)
      ; Set correct position and spawn Actor
      (bind _returnvalue (`|SpawnActorFromClass` "/Game/ElCortijo/Features/Interaction/Pickable/BP_Pickable.BP_Pickable_C" (`KismetMathLibrary.MakeTransform` (`SceneComponent.K2_GetComponentLocation` _proofplacement) (`SceneComponent.K2_GetComponentRotation` _proofplacement) _scale) "AlwaysSpawn" "MultiplyWithRoot" null (make `/Game/ElCortijo/Features/Interaction/Pickable/S_ItemData` _name _mesh _type _previewrotator _scale _objectoffset _collidersize false false _isresearched) true null))
      ; Set collision channel to research
      (`PrimitiveComponent.SetCollisionResponseToChannel` (`/Game/ElCortijo/Features/Interaction/Pickable/BP_Pickable.Collision` _returnvalue) "ECC_GameTraceChannel2" "ECR_Block")
      ; Turn off physics
      (bind _output_get_2 (set `self.Objeto Investigable` _returnvalue))
      (`PrimitiveComponent.SetSimulatePhysics` (`/Game/ElCortijo/Features/Interaction/Pickable/BP_Pickable.Collision` _output_get_2) false)
      ; Empty inventory
      (`/Game/ElCortijo/Features/Character/BP_InventoryComponent.ClearItem` (`self.Inventory Slot`))
      (return))))

(fn `DestroyReserchableObject`
  (params (Interactor :type "/Game/FirstPerson/Blueprints/BP_FirstPersonCharacter Object Reference"))
  (bind _objeto_investigable (`self.Objeto Investigable`))
  (if (!= _objeto_investigable null)
    (`/Game/ElCortijo/Features/Character/BP_InventoryComponent.PickUpActor` (`/Game/FirstPerson/Blueprints/BP_FirstPersonCharacter.InventorySlot` Interactor) _objeto_investigable)
    (return)))

(fn `Rotate`
  (locals (NewLocalVar :type "Vector Structure"))
  (bind (_locationx _locationy) (`PlayerController.GetMousePosition` (`GameplayStatics.GetPlayerController` 0)))
  (if (!= (`self.Objeto Investigable`) null)
    (if (`self.PlayerInTable`)
      (`KismetSystemLibrary.PrintString` "Rotate")
      (`self.K2_AddActorLocalRotation` (`self.Objeto Investigable`) (`KismetMathLibrary.MakeRotator` (.x (- (`KismetMathLibrary.MakeVector` _locationx _locationy) (`self.StartMousePos`))) (.y (- (`KismetMathLibrary.MakeVector` _locationx _locationy) (`self.StartMousePos`))) (.z (- (`KismetMathLibrary.MakeVector` _locationx _locationy) (`self.StartMousePos`)))) false false)
      (`self.RotationInfo`))))

(fn `RotationInfo`
  (bind (_locationx _locationy) (`PlayerController.GetMousePosition` (`GameplayStatics.GetPlayerController` 0)))
  (`KismetSystemLibrary.PrintString` "GetInfo")
  (set `self.StartMousePos` (`KismetMathLibrary.MakeVector` _locationx _locationy)))

(fn `UserConstructionScript`)