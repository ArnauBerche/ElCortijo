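; BP_MusicaTension is a placed actor that drives tension music based on how close the player is to it.
; On BeginPlay it caches the first-person player character.
; While Enabled, each Tick maps player distance to the SM_4_Capas global audio parameter, raising it as the player approaches within a set range.
; The mapped value is also printed every frame as debug text.
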(event `self.ReceiveBeginPlay`
  (bind _asbp_first_person_character (cast `/Game/ElCortijo/Features/1_MainCharacter/Blueprints/BP_FirstPersonCharacter` (`GameplayStatics.GetPlayerCharacter` 0)))
  (set `self.PlayerChar` _asbp_first_person_character))

(event `self.ReceiveTick`
  (params (DeltaSeconds :type "Float (single-precision)"))
  (bind _returnvalue (`KismetMathLibrary.MapRangeClamped` (`self.GetDistanceTo` (`self.PlayerChar`) self) 2500.0 350.0 0.0 3.0))
  (if (`self.Enabled`)
    (`KismetSystemLibrary.PrintText` (`KismetTextLibrary.Conv_DoubleToText` _returnvalue "HalfToEven"))
    (`FMODBlueprintStatics.SetGlobalParameterByName` "SM_4_Capas" _returnvalue)))

(fn `UserConstructionScript`)