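; BP_Evidence is an evidence item that the player can take back from a research table or model board.
; On Interact while on a table, it calls PickUp with the player character, then casts the current table by its type and removes itself from that slot.
; It then clears its table state and turns off clickability, which SetClickable controls through the collision response to a custom trace channel.
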(event `self.ReceiveBeginPlay`
  (`parent.ReceiveBeginPlay`))

(event `/Game/ElCortijo/Features/Interaction/BPI_Interactable.Interact`
  (params (Interactor :type "Actor Object Reference"))
  (bind _currenttable (`self.CurrentTable`))
  (bind _slotindex (`self.SlotIndex`))
  (if (`self.bIsOnTable`)
    (`self.PickUp` (`GameplayStatics.GetPlayerCharacter` 0))
    (if (== (`/Game/ElCortijo/Features/Tables/BP_Table.TType` (`self.CurrentTable`)) 0)
      (bind _asbp_research_table (cast `/Game/ElCortijo/Features/ResearchTable/Blueprint/BP_ResearchTable` _currenttable))
      (`/Game/ElCortijo/Features/ResearchTable/Blueprint/BP_ResearchTable.RemoveEvidence` _asbp_research_table _slotindex)
      (else
        (bind _asbp_model_board (cast `/Game/ElCortijo/Features/ModelBoard/Blueprint/BP_ModelBoard` _currenttable))
        (`/Game/ElCortijo/Features/ModelBoard/Blueprint/BP_ModelBoard.RemoveEvidence` _asbp_model_board _slotindex)))
    (`self.SetClickable` false)
    (set `self.CurrentTable` null)
    (set `self.SlotIndex` 0)
    (set `self.bIsOnTable` false)))

(fn `SetClickable`
  (params (Enabled :type Boolean))
  (bind _collision (`self.Collision`))
  (if Enabled
    (`PrimitiveComponent.SetCollisionResponseToChannel` _collision "ECC_GameTraceChannel3" "ECR_Block")
    (else
      (`PrimitiveComponent.SetCollisionResponseToChannel` _collision "ECC_GameTraceChannel3" "ECR_Ignore"))))

(fn `UserConstructionScript`
  (`parent.UserConstructionScript`))