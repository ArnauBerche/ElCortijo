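; Telephone evidence prop, a child Blueprint that can be dragged onto the grid of a BP_ModelBoard when its table type allows it.
; Click lifts the mesh, and Tick moves the actor to the cursor hit in table space while updating the board's cell visor.
; Release snaps it into a valid cell that is empty or its own, updating grid and hint-slot bookkeeping, or returns it to its previous cell or slot.
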(event `self.ReceiveBeginPlay`
  (bind (_returnvalue_x _returnvalue_y _returnvalue_z) (`KismetMathLibrary.BreakVector` (`BoxComponent.GetScaledBoxExtent` (`self.Collision`))))
  (bind (_relativelocation_x _relativelocation_y _relativelocation_z) (`KismetMathLibrary.BreakVector` (`SceneComponent.RelativeLocation` (`self.Object`))))
  (set `self.EType` "NewEnumerator0")
  (set `self.Offset_0` _returnvalue_z)
  (bind _output_get (set `self.StartRLocation_0` _relativelocation_z))
  (set `self.UpRLocation_0` (+ _output_get 15.0))
  (`parent.ReceiveBeginPlay`))

(event `self.ReceiveTick`
  (params (DeltaSeconds :type "Float (single-precision)"))
  (`|ExecutionSequence`
    (:`then_0`
      (`parent.ReceiveTick` DeltaSeconds))
    (:`then_1`
      (if (`self.IsDragging_0`)
        (`self.K2_SetActorRelativeLocation` self (`KismetMathLibrary.MakeVector` (.x (`KismetMathLibrary.InverseTransformLocation` (`self.GetTransform` (`self.CurrentTable`)) (`.Location` (`GameplayStatics.BreakHitResult` (`PlayerController.GetHitResultUnderCursorByChannel` (`GameplayStatics.GetPlayerController` 0) "TraceTypeQuery4" true))))) (.y (`KismetMathLibrary.InverseTransformLocation` (`self.GetTransform` (`self.CurrentTable`)) (`.Location` (`GameplayStatics.BreakHitResult` (`PlayerController.GetHitResultUnderCursorByChannel` (`GameplayStatics.GetPlayerController` 0) "TraceTypeQuery4" true))))) (`self.Offset_0`)) false false)
        (bind _asbp_model_board (cast `/Game/ElCortijo/Features/ModelBoard/Blueprint/BP_ModelBoard` (`self.CurrentTable`)))
        (bind (_cell _iscellvalid) (`/Game/ElCortijo/Features/ModelBoard/Blueprint/BP_ModelBoard.Get Cell From Object` _asbp_model_board self))
        (`/Game/ElCortijo/Features/ModelBoard/Blueprint/BP_ModelBoard.SetVisor Pos` _asbp_model_board _cell _iscellvalid)))))

(event `self.Click`
  (params (Interactor :type "Actor Object Reference"))
  (if (== (`/Game/ElCortijo/Features/Tables/BP_Table.TType` (`self.CurrentTable`)) 1)
    (set `self.IsDragging_0` true)
    (`SceneComponent.K2_SetRelativeLocation` (`self.Object`) (`KismetMathLibrary.MakeVector` 0.0 0.0 (`self.UpRLocation_0`)) false false)))

(event `self.Release`
  (params (Interactor :type "Actor Object Reference"))
  (bind _bp_model_board_0 (`self.BP Model Board_0`))
  (bind _output_placement (break `/Game/ElCortijo/Features/ResearchTable/S_TablePlacements` (`|GetArrayItem` (`/Game/ElCortijo/Features/ModelBoard/Blueprint/BP_ModelBoard.HintPlacementsRef` _bp_model_board_0) (`self.SlotIndex`))))
  (if (== (`/Game/ElCortijo/Features/Tables/BP_Table.TType` (`self.CurrentTable`)) 1)
    (set `self.IsDragging_0` false)
    (`SceneComponent.K2_SetRelativeLocation` (`self.Object`) (`KismetMathLibrary.MakeVector` 0.0 0.0 (`self.StartRLocation_0`)) false false)
    (bind _asbp_model_board (cast `/Game/ElCortijo/Features/ModelBoard/Blueprint/BP_ModelBoard` (`self.CurrentTable`)))
    (set `self.BP Model Board_0` _asbp_model_board)
    (bind (_cell _iscellvalid) (`/Game/ElCortijo/Features/ModelBoard/Blueprint/BP_ModelBoard.Get Cell From Object` _asbp_model_board self))
    (bind _isempty (`/Game/ElCortijo/Features/ModelBoard/Blueprint/BP_ModelBoard.IsCellEmpty` _asbp_model_board _cell))
    (bind _hasself (`/Game/ElCortijo/Features/ModelBoard/Blueprint/BP_ModelBoard.CellHasObject` _asbp_model_board _cell self))
    (if (and (or _hasself _isempty) _iscellvalid)
      (`/Game/ElCortijo/Features/ModelBoard/Blueprint/BP_ModelBoard.Add ObjectToGrid` _asbp_model_board _cell self)
      (`/Game/ElCortijo/Features/ModelBoard/Blueprint/BP_ModelBoard.RemoveEvidenceINHP` _asbp_model_board (`self.SlotIndex`))
      (bind _relative_pos (`/Game/ElCortijo/Features/ModelBoard/Blueprint/BP_ModelBoard.Get Cell Relative Pos` _asbp_model_board _cell))
      (`self.K2_SetActorRelativeLocation` self (`KismetMathLibrary.MakeVector` (.x _relative_pos) (.y _relative_pos) (+ (.z _relative_pos) (`self.Offset_0`))) false false)
      (set `self.IsOnGrid_0` true)
      (if (!= (`self.StayCell_0`) (-1.0 -1.0))
        (`/Game/ElCortijo/Features/ModelBoard/Blueprint/BP_ModelBoard.Remove ObjectFromGrid` _asbp_model_board (`self.StayCell_0`))
        (set `self.StayCell_0` _cell)
        (else
          (set `self.StayCell_0` _cell)))
      (elif (`self.IsOnGrid_0`)
        (bind _relative_pos_2 (`/Game/ElCortijo/Features/ModelBoard/Blueprint/BP_ModelBoard.Get Cell Relative Pos` _asbp_model_board (`self.StayCell_0`)))
        (`self.K2_SetActorRelativeLocation` (`KismetMathLibrary.MakeVector` (.x _relative_pos_2) (.y _relative_pos_2) (+ (.z _relative_pos_2) (`self.Offset_0`))))
        (else
          (`self.K2_SetActorRelativeLocation` (+ (`SceneComponent.RelativeLocation` (`/Game/ElCortijo/Features/ModelBoard/Blueprint/BP_ModelBoard.EvidenceRelativeSlots` _bp_model_board_0)) (`SceneComponent.RelativeLocation` _output_placement))))))))

(fn `UserConstructionScript`
  (`parent.UserConstructionScript`))